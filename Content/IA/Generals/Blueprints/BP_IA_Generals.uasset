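; Base Blueprint for AI-controlled General enemies, configured by an IAType variant.
; On BeginPlay it has its generals AI controller switch to the behavior tree for that type.
; The construction script sets per-type explosion radius and walk speed, currently only for the First General.
; StartAttack locks translation while allowing rotation through CanMove, which swaps between Walking, Custom and disabled movement modes, and resets the player-hit flag.
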(event Custom|CanMove
  (params (canMove? :type Boolean) (canRotate? :type Boolean))
  (bind _charactermovement (Variables|Character|GetCharacterMovement))
  (if canMove?
    (Pawn|Components|CharacterMovement|SetMovementMode _charactermovement "MOVE_Walking" 0)
    (elif canRotate?
      (Pawn|Components|CharacterMovement|SetMovementMode _charactermovement "MOVE_Custom" 0)
      (else
        (Pawn|Components|CharacterMovement|DisableMovement _charactermovement)))))

(event Custom|StartAttack
  (if (not (Variables|Default|GetIsAttacking?))
    (CallFunction|CanMove false true)
    (Variables|Default|SetIsAttacking? true)
    (Variables|Utilities|SetHit%20Player%20? false)))

(event EventBeginPlay
  (Default|ChangeBehaviorTree (.AsIA%20Controller%20Generals (Utilities|Casting|CastToIA_Controller_Generals (AI|GetAIController self))) (Variables|Default|GetIA_Type)))

(fn ConstructionScript
  (switch Utilities|FlowControl|Switch|SwitchonIA_Types_Generals (Variables|Default|GetIA_Type)
    (:NewEnumerator0
      (Variables|Default|SetRadiusExplo 3e+02)
      (Variables|/Script/Engine.CharacterMovementComponent|SetMaxWalkSpeed (Variables|Character|GetCharacterMovement) 2e+02))))