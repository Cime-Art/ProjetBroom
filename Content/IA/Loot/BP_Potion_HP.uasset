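; BP_Potion_HP is a health potion pickup that bobs its sphere and applies healing to the player on overlap.
; A timeline started at BeginPlay drives the sphere's relative Z.
; On overlap, a BP_PlayerTest below max HP receives Heal through SetterHP, followed by a zero-HP SetterHP call if max is then reached.
; The potion is never destroyed or disabled in this graph.
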(event OnComponentBeginOverlap(Sphere)
  (params (OverlappedComponent :type Primitive%20Component%20Object%20Reference) (OtherActor :type Actor%20Object%20Reference) (OtherComp :type Primitive%20Component%20Object%20Reference) (OtherBodyIndex :type Integer) (bFromSweep :type Boolean) (SweepResult :type Hit%20Result%20Structure%20%28by%20ref%29))
  (bind _asbp_player_test (Utilities|Casting|CastToBP_PlayerTest OtherActor))
  (if (not (>= (.hpplayer (Variables|/Game/Blueprint/BP_PlayerTest.BP_PlayerTest_C|GetInfoPlayer _asbp_player_test)) (.maxhp (Variables|/Game/Blueprint/BP_PlayerTest.BP_PlayerTest_C|GetInfoPlayer _asbp_player_test))))
    ;[1 1 1] True
    (Default|SetterHP _asbp_player_test (Variables|Default|GetHeal) false 0.0)
    (if (>= (.hpplayer (Variables|/Game/Blueprint/BP_PlayerTest.BP_PlayerTest_C|GetInfoPlayer _asbp_player_test)) (.maxhp (Variables|/Game/Blueprint/BP_PlayerTest.BP_PlayerTest_C|GetInfoPlayer _asbp_player_test)))
      (Default|SetterHP _asbp_player_test 0.0 false 0.0))))

(event EventBeginPlay
  (bind _sphere (Variables|Default|GetSphere))
  (bind _relativelocation (Variables|/Script/Engine.SceneComponent|GetRelativeLocation _sphere))
  (bind _mouvement (Timeline|Mouvement%20Y Play)
    (:Update
      (Transformation|SetRelativeLocation _sphere (Math|Vector|MakeVector (.x _relativelocation) (.y _relativelocation) _mouvement) false false))))

(fn ConstructionScript)