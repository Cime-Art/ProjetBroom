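; Ranged AI projectile actor that launches toward the player when its ActivatePhysics event is called.
; The event rotates the actor from its Sphere toward the player mesh's spine_02 socket, adds and stores a ProjectileMovement component at runtime, then sets the Sphere to query-only collision.
; Aim is taken once at activation, as the node that assigns the player mesh as homing target is disconnected.
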(event Custom|ActivatePhysics
  (Transformation|SetActorRotation (Math|Rotator|FindLookatRotation (Transformation|GetWorldLocation (Variables|Default|GetSphere)) (Transformation|GetSocketLocation (Variables|/Script/Engine.Character|GetMesh (Game|GetPlayerCharacter 0)) "spine_02")))
  (bind _returnvalue (AddComponent|AddProjectileMovementComponent))
  (bind _output_get (Variables|Default|SetProjectile%20Ref _returnvalue))
  (Collision|SetCollisionEnabled (Variables|Default|GetSphere) "QueryOnly"))

(fn ConstructionScript)