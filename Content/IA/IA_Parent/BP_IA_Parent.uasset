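; BP_IA_Parent is a base AI character Blueprint that handles behavior tree assignment, attack start and movement locking.
; On BeginPlay it passes its IAType to its IA_Controller_ to switch the behavior tree.
; StartAttack ignores calls while already attacking, otherwise it sets attack state, clears HitPlayer and stops movement while allowing rotation.
; CanMove switches between Walking, a Custom mode for rotation-only, and fully disabled movement.
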(event Custom|CanMove
  (params (canMove? :type Boolean) (canRotate? :type Boolean))
  (bind _charactermovement (Variables|Character|GetCharacterMovement))
  (if canMove?
    (Pawn|Components|CharacterMovement|SetMovementMode _charactermovement "MOVE_Walking" 0)
    (elif canRotate?
      (Pawn|Components|CharacterMovement|SetMovementMode _charactermovement "MOVE_Custom" 0)
      (else
        (Pawn|Components|CharacterMovement|DisableMovement _charactermovement)))))

(event Custom|StartAttack
  (if (not (Variables|Default|GetIsAttacking?))
    (CallFunction|CanMove false true)
    (Variables|Default|SetIsAttacking? true)
    (Variables|Utilities|SetHit%20Player%20? false)))

(event EventBeginPlay
  (Default|ChangeBehaviorTree (.AsIA%20Controller%20 (Utilities|Casting|CastToIA_Controller_ (AI|GetAIController self))) (Variables|Default|GetIA_Type)))

(fn ConstructionScript)