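; BP_Random_Spawn is a box volume that plays random Wwise sounds at random positions inside it while the player character is present.
; Construction adds a box scaled by BoxExtents; begin play or overlap starts a random-delay timer, and leaving clears it.
; Each timer firing posts a random event from the Event array at a random point in the box, then re-arms itself.
; The debug marker spawn is disconnected.
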(event Custom|Sound_Trig
  (bind _event (Variables|Default|GetEvent))
  (bind _box (Variables|Default|GetBox))
  (bind _refdebug (Variables|Default|GetRefDebug))
  (Utilities|IsValid _refdebug
    (:Is%20Valid
      (Actor|DestroyActor _refdebug))
    (:Is%20Not%20Valid
      _))
  (Class|AkGameplayStatics|SpawnAkComponentatLocation (Utilities|Array|Get(acopy) _event (Math|Random|RandomIntegerinRange 0 (Utilities|Array|LastIndex _event))) (Math|Random|RandomPointinBoundingBox (Transformation|GetWorldLocation _box) (Components|Box|GetScaledBoxExtent _box)) "0, 0, 0" true)
  (CallFunction|Retrigger)
  (if (Variables|Default|GetDebug)
    _))

(event Custom|Retrigger
  (Utilities|Time|SetTimerbyFunctionName 0 "Sound_Trig" (Math|Random|RandomFloatinRange (Variables|Time|GetTime%20Min) (Variables|Time|GetTime%20Max))))

(event Collision|EventActorBeginOverlap
  (params (OtherActor :type Actor%20Object%20Reference))
  (if (== OtherActor (Game|GetPlayerCharacter 0))
    (Utilities|Time|SetTimerbyFunctionName 0 "Sound_Trig" (Math|Random|RandomFloatinRange (Variables|Time|GetTime%20Min) (Variables|Time|GetTime%20Max)))))

(event Collision|EventActorEndOverlap
  (params (OtherActor :type Actor%20Object%20Reference))
  (if (== (Game|GetPlayerCharacter 0) OtherActor)
    (Utilities|Time|ClearTimerbyFunctionName 0 "Sound_Trig")))

(event EventBeginPlay
  (for _array_element (Collision|GetOverlappingActors "/Game/Game_Dev/Blueprint/Player/BP_PlayerTest.BP_PlayerTest_C" :!class /Script/Engine.Actor)
    (if (== _array_element (Game|GetPlayerCharacter 0))
      (Utilities|Time|SetTimerbyFunctionName 0 "Sound_Trig" (Math|Random|RandomFloatinRange (Variables|Time|GetTime%20Min) (Variables|Time|GetTime%20Max))))))

(fn ConstructionScript
  (bind _returnvalue (AddComponent|AddBoxComponent false (Math|Transform|MakeTransform "0, 0, 0" "0, 0, 0" (Variables|Shapes|Getbox%20Extents))))
  (bind _output_get (Variables|Default|SetBox _returnvalue))
  (Variables|/Script/Engine.PrimitiveComponent|SetbGenerateOverlapEvents _output_get true))