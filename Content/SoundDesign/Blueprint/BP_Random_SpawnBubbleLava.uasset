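; Lava bubble sound emitter that plays random Wwise events at random points inside a box while the player is in it.
; The construction script builds the box, and begin play or player overlap starts a random-delay timer that is cleared on exit.
; Each timer firing spawns an Ak component and re-arms itself.
; An optional debug marker spawns at a separately rolled point, not the sound's location.
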(event Custom|Sound_Trig
  (bind _event (Variables|Default|GetEvent))
  (bind _box (Variables|Default|GetBox))
  (bind _returnvalue (Transformation|GetWorldLocation _box))
  (bind _returnvalue_2 (Components|Box|GetScaledBoxExtent _box))
  (bind _returnvalue_3 (Math|Random|RandomPointinBoundingBox _returnvalue _returnvalue_2))
  (Utilities|IsValid (Variables|Default|GetRefDebug)
    (:Is%20Valid
      (Actor|DestroyActor (Variables|Default|GetRefDebug)))
    (:Is%20Not%20Valid
      _))
  (Class|AkGameplayStatics|SpawnAkComponentatLocation (Utilities|Array|Get(acopy) _event (Math|Random|RandomIntegerinRange 0 (Utilities|Array|LastIndex _event))) _returnvalue_3 "0, 0, 0" true)
  (CallFunction|Retrigger)
  (if (Variables|Default|GetDebug)
    (bind _returnvalue_4 (Game|SpawnActorfromClass "/Game/SoundDesign/Blueprint/Bp_Pos_test.Bp_Pos_test_C" (Math|Conversions|ToTransform(Vector) _returnvalue_3) "Undefined" 0 0))
    (Variables|Default|SetRefDebug _returnvalue_4)))

(event Custom|Retrigger
  (Utilities|Time|SetTimerbyFunctionName 0 "Sound_Trig" (Math|Random|RandomFloatinRange (Variables|Time|GetTime%20Min) (Variables|Time|GetTime%20Max))))

(event Collision|EventActorBeginOverlap
  (params (OtherActor :type Actor%20Object%20Reference))
  (if (== OtherActor (Game|GetPlayerCharacter 0))
    (Utilities|Time|SetTimerbyFunctionName 0 "Sound_Trig" (Math|Random|RandomFloatinRange (Variables|Time|GetTime%20Min) (Variables|Time|GetTime%20Max)))))

(event Collision|EventActorEndOverlap
  (params (OtherActor :type Actor%20Object%20Reference))
  (if (== (Game|GetPlayerCharacter 0) OtherActor)
    (Utilities|Time|ClearTimerbyFunctionName 0 "Sound_Trig")))

(event EventBeginPlay
  (bind _box (Variables|Default|GetBox))
  (Collision|SetCollisionObjectType _box "ECC_GameTraceChannel2")
  (Collision|SetCollisionResponsetoChannel _box "ECC_Visibility" "ECR_Ignore")
  (Collision|SetCollisionResponsetoChannel _box "ECC_Camera" "ECR_Overlap")
  (for _array_element (Collision|GetOverlappingActors "/Game/Game_Dev/Blueprints/Player/BP_PlayerTest.BP_PlayerTest_C" :!class /Script/Engine.Actor)
    (if (== _array_element (Game|GetPlayerCharacter 0))
      (Utilities|Time|SetTimerbyFunctionName 0 "Sound_Trig" (Math|Random|RandomFloatinRange (Variables|Time|GetTime%20Min) (Variables|Time|GetTime%20Max))))))

(fn ConstructionScript
  (bind _returnvalue (AddComponent|AddBoxComponent false (Math|Transform|MakeTransform "0, 0, 0" "0, 0, 0" (Variables|Shapes|Getbox%20Extents))))
  (bind _output_get (Variables|Default|SetBox _returnvalue))
  (Variables|/Script/Engine.PrimitiveComponent|SetbGenerateOverlapEvents _output_get true))