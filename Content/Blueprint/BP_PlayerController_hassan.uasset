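; Player controller that handles menu widgets, inventory input and input-device detection.
; It shows the mouse cursor at start and sets a Gamepad flag from whether the last pressed key was a gamepad key.
; ChangeItemLeft and ChangeItemRight actions call the matching change functions on the inventory widget when it is valid.
; Custom events lazily create, cache and add the main menu, play (Jouer) and options widgets to the viewport.
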(event EventBeginPlay
  (Variables|Default|SetbShowMouseCursor true))

(event Input|KeyboardEvents|AnyKey
  (params (Key :type Key%20Structure :default "None"))
  (:Pressed
    (if (Class|KismetInputLibrary|KeyIsGamepadKey Key)
      (Variables|Default|SetGamepad? true)
      (else
        (Variables|Default|SetGamepad? false)))))

(event Custom|HUD-Option
  ;[1 1 1] HUD
  (Utilities|IsValid (Variables|Default|GetHUD%20Option)
    (:Is%20Valid
      _)
    (:Is%20Not%20Valid
      (bind _returnvalue (UserInterface|CreateWidget "/Game/Widget/WG_Option.WG_Option_C"))
      (bind _output_get (Variables|Default|SetHUD%20Option _returnvalue))))
  (UserInterface|Viewport|AddtoViewport _output_get 0))

(event Custom|HUD-MENU
  ;[1 1 1] HUD
  (Utilities|IsValid (Variables|Default|GetHUD%20MENU)
    (:Is%20Valid
      _)
    (:Is%20Not%20Valid
      (bind _returnvalue (UserInterface|CreateWidget "/Game/Widget/MainMenu.MainMenu_C"))
      (bind _output_get (Variables|Default|SetHUD%20MENU _returnvalue))))
  (UserInterface|Viewport|AddtoViewport _output_get 0))

(event Custom|HUD-Jouer
  ;[1 1 1] HUD
  (Utilities|IsValid (Variables|Default|GetHUD%20JOUER)
    (:Is%20Valid
      _)
    (:Is%20Not%20Valid
      (bind _returnvalue (UserInterface|CreateWidget "/Game/Widget/WG_Jouer.WG_Jouer_C"))
      (bind _output_get (Variables|Default|SetHUD%20JOUER _returnvalue))))
  (UserInterface|Viewport|AddtoViewport _output_get 0))

(event Input|ActionEvents|InputActionChangeItemLeft
  (params (Key :type Key%20Structure :default "None"))
  (bind _wg_inventaire (Variables|Default|GetWG_Inventaire))
  (:Pressed
    (Utilities|IsValid _wg_inventaire
      (:Is%20Valid
        (Default|ChangeLeft _wg_inventaire)))))

(event Input|ActionEvents|InputActionChangeItemRight
  (params (Key :type Key%20Structure :default "None"))
  (bind _wg_inventaire (Variables|Default|GetWG_Inventaire))
  (:Pressed
    (Utilities|IsValid _wg_inventaire
      (:Is%20Valid
        (Default|ChangeRight _wg_inventaire)))))

(fn ConstructionScript)