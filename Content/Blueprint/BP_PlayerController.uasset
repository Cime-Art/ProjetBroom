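; Player controller Blueprint that handles the inventory menu input and tracks whether the player is using a gamepad.
; On begin play it shows the mouse cursor in game-only input mode, and any key press updates the Gamepad flag.
; OpenInventaire toggles pause, creating or removing the WG_Inventaire widget; WidgetOpen acts inverted, with true meaning ready to open.
; ChangeItemLeft and ChangeItemRight forward item navigation to that widget while it exists.
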(event EventBeginPlay
  (Variables|Default|SetbShowMouseCursor true)
  (Input|SetInputModeGameOnly self))

(event Input|KeyboardEvents|AnyKey
  (params (Key :type Key%20Structure :default "None"))
  (:Pressed
    (if (Class|KismetInputLibrary|KeyIsGamepadKey Key)
      (Variables|Default|SetGamepad? true)
      (else
        (Variables|Default|SetGamepad? false)))))

(event Input|ActionEvents|InputActionOpenInventaire
  (params (Key :type Key%20Structure :default "None"))
  (:Pressed
    (if (Variables|Default|GetWidgetOpen)
      (Variables|Default|SetWidgetOpen false)
      (Game|SetGamePaused true)
      (Utilities|IsValid (Variables|Default|GetWG_Inventaire)
        (:Is%20Not%20Valid
          (bind _returnvalue (UserInterface|CreateWidget "/Game/Widget/WG_Inventaire.WG_Inventaire_C"))
          (bind _output_get (Variables|Default|SetWG_Inventaire _returnvalue))
          (UserInterface|Viewport|AddtoViewport _output_get 0)))
      (else
        (Game|SetGamePaused false)
        (Variables|Default|SetWidgetOpen true)
        (Default|RemoveWidget (Variables|Default|GetWG_Inventaire))
        (Variables|Default|SetWG_Inventaire 0)))))

(event Input|ActionEvents|InputActionChangeItemLeft
  (params (Key :type Key%20Structure :default "None"))
  (bind _wg_inventaire (Variables|Default|GetWG_Inventaire))
  (:Pressed
    (Utilities|IsValid _wg_inventaire
      (:Is%20Valid
        (Default|ChangeLeft _wg_inventaire)))))

(event Input|ActionEvents|InputActionChangeItemRight
  (params (Key :type Key%20Structure :default "None"))
  (bind _wg_inventaire (Variables|Default|GetWG_Inventaire))
  (:Pressed
    (Utilities|IsValid _wg_inventaire
      (:Is%20Valid
        (Default|ChangeRight _wg_inventaire)))))

(fn ConstructionScript)