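; BP_LibraryPlayer is a shared set of helper functions for fetching the game's core player-related objects as typed references.
; CastController and CastPlayer cast the index 0 player controller and pawn to BP_PlayerController and BP_PlayerTest, while CastGameInstance casts the game instance to BP_GameInstance.
; Each function returns the typed reference on success, with no handling for a failed cast.
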(fn CastController
  (bind _asbp_player_controller (Utilities|Casting|CastToBP_PlayerController (Game|GetPlayerController 0)))
  (return _asbp_player_controller))

(fn CastGameInstance
  (bind _asbp_game_instance (Utilities|Casting|CastToBP_GameInstance (Game|GetGameInstance)))
  (return _asbp_game_instance))

(fn CastPlayer
  (bind _asbp_player_test (Utilities|Casting|CastToBP_PlayerTest (Game|Player|GetPlayerPawn 0)))
  (return _asbp_player_test))