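; Collapsing bridge platform, apparently a test version, that falls apart after the player enters its trigger.
; A one-shot overlap waits a delay, then a timeline randomly jitters the skeletal mesh in X and Z as a warning shake.
; The collapse animation then plays while a second timeline's Destroy events disable five collision boxes in sequence.
; ResetAll stops both timelines, rewinds the animation, restores collision and re-arms the trigger.
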(event OnComponentBeginOverlap(Trigger)
  (params (OverlappedComponent :type Primitive%20Component%20Object%20Reference) (OtherActor :type Actor%20Object%20Reference) (OtherComp :type Primitive%20Component%20Object%20Reference) (OtherBodyIndex :type Integer) (bFromSweep :type Boolean) (SweepResult :type Hit%20Result%20Structure%20%28by%20ref%29))
  (Utilities|Casting|CastToBP_PlayerTest OtherActor)
  (Utilities|FlowControl|DoOnce false
    (:Completed
      (Utilities|FlowControl|Delay (Variables|Default|GetDelay))
      (CallFunction|BEGINSHAKE))))

(event Custom|BEGIN_SHAKE
  (bind _returnvalue (Math|Random|RandomFloatinRange -2.0 2.0))
  (bind _skeletalmesh (Variables|Default|GetSkeletalMesh))
  (Timeline|Timeline_1 PlayFromStart
    (:Update
      (Variables|Default|SetRandomX _returnvalue)
      (Variables|Default|SetRandomY _returnvalue)
      (Transformation|SetRelativeLocation _skeletalmesh (Math|Vector|MakeVector (Variables|Default|GetRandomX) (.y (Variables|/Script/Engine.SceneComponent|GetRelativeLocation _skeletalmesh)) (Variables|Default|GetRandomY)) false false))
    (:Finished
      (Audio|Components|Audio|Play (Variables|Default|GetSkeletalMesh) false)
      (Timeline|Timeline_0 PlayFromStart
        (:Destroy
          (Collision|SetCollisionEnabled (Utilities|Array|Get(acopy) (Variables|Default|GetTabBox) (Variables|Default|Getindex)) "NoCollision")
          (Math|Integer|IncrementInt (Variables|Default|Getindex)))))))

(event EventBeginPlay
  (|CallParentFunction) ; This node is disabled and will not be called.\nDrag off pins to build functionality.
)

(event Collision|EventActorBeginOverlap
  (params (OtherActor :type Actor%20Object%20Reference))
  (|CallParentFunction OtherActor) ; This node is disabled and will not be called.\nDrag off pins to build functionality.
)

(event EventTick
  (params (DeltaSeconds :type Float%20%28single-precision%29))
  (|CallParentFunction DeltaSeconds) ; This node is disabled and will not be called.\nDrag off pins to build functionality.
)

(event EventResetAll
  (bind _timeline_0 (Variables|Default|GetTimeline_0))
  (if (Audio|Components|Audio|IsPlaying (Variables|Default|GetTimeline_1))
    (Audio|Components|Audio|Stop (Variables|Default|GetTimeline_1)))
  (if (Audio|Components|Audio|IsPlaying _timeline_0)
    (Audio|Components|Audio|Stop _timeline_0))
  (Audio|Components|Audio|Stop (Variables|Default|GetSkeletalMesh))
  (Components|Animation|SetPosition (Variables|Default|GetSkeletalMesh) 0.0 true)
  (Variables|Default|Setindex 0)
  (for _array_element (Variables|Default|GetTabBox)
    (Collision|SetCollisionEnabled _array_element "QueryAndPhysics"))
  (Utilities|FlowControl|DoOnce false) ; enters at Reset
)

(fn ConstructionScript
  (|CallParentFunction)
  (Variables|Default|SetInitialScale (.y (Variables|/Script/Engine.BoxComponent|GetBoxExtent (Variables|Default|GetBox))))
  (Variables|Default|SetTabBox (Utilities|Array|MakeArray (Variables|Default|GetBox4) (Variables|Default|GetBox3) (Variables|Default|GetBox2) (Variables|Default|GetBox1) (Variables|Default|GetBox))))