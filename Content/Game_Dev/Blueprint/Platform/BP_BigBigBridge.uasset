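; Collapsing bridge platform that falls apart, once per reset, after the player overlaps its trigger and a delay elapses.
; BeginAnim plays five bridge-part animations together and starts the Destroy timeline.
; Each Destroy event on that timeline disables collision on the next of thirty boxes ordered in the construction script.
; ResetAll stops and rewinds the animations, restores collision through TabBox, clears the index and re-arms the trigger.
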(event OnComponentBeginOverlap(Trigger)
  (params (OverlappedComponent :type Primitive%20Component%20Object%20Reference) (OtherActor :type Actor%20Object%20Reference) (OtherComp :type Primitive%20Component%20Object%20Reference) (OtherBodyIndex :type Integer) (bFromSweep :type Boolean) (SweepResult :type Hit%20Result%20Structure%20%28by%20ref%29))
  ;[1 1 1] Begin
  (Utilities|Casting|CastToBP_PlayerTest OtherActor)
  (Utilities|FlowControl|DoOnce false
    (:Completed
      (Utilities|FlowControl|Delay (Variables|Default|GetDelay))
      (CallFunction|BeginAnim))))

(event Custom|Begin%20Anim
  ;[1 1 1] Destroy
  (Audio|Components|Audio|Play (Variables|Default|Get2_Pont_D) false)
  (Timeline|Destroy PlayFromStart
    (:Destroy
      (Collision|SetCollisionEnabled (Utilities|Array|Get(acopy) (Variables|Default|GetLeTabSale) (Variables|Default|Getindex)) "NoCollision")
      (Math|Integer|IncrementInt (Variables|Default|Getindex)))))

(event EventResetAll
  (bind _destroy (Variables|Default|GetDestroy))
  ;[1 1 1] Reset
  (if (Audio|Components|Audio|IsPlaying _destroy)
    (Audio|Components|Audio|Stop _destroy))
  (Audio|Components|Audio|Stop (Variables|Default|Get2_Pont_D))
  (Components|Animation|SetPosition (Variables|Default|Get2_Pont_D) 0.0 true)
  (Variables|Default|Setindex 0)
  (for _array_element (Variables|Default|GetTabBox)
    (Collision|SetCollisionEnabled _array_element "QueryAndPhysics"))
  ;[1 1 1] Begin
  (Utilities|FlowControl|DoOnce false) ; enters at Reset
)

(fn ConstructionScript
  (Variables|Default|SetLeTabSale (Utilities|Array|MakeArray (Variables|Default|GetBox1) (Variables|Default|GetBox2) (Variables|Default|GetBox3) (Variables|Default|GetBox4) (Variables|Default|GetBox5) (Variables|Default|GetBox6) (Variables|Default|GetBox7) (Variables|Default|GetBox8) (Variables|Default|GetBox9) (Variables|Default|GetBox10) (Variables|Default|GetBox11) (Variables|Default|GetBox12) (Variables|Default|GetBox13) (Variables|Default|GetBox14) (Variables|Default|GetBox15) (Variables|Default|GetBox16) (Variables|Default|GetBox17) (Variables|Default|GetBox18) (Variables|Default|GetBox19) (Variables|Default|GetBox20) (Variables|Default|GetBox21) (Variables|Default|GetBox22) (Variables|Default|GetBox23) (Variables|Default|GetBox24) (Variables|Default|GetBox25) (Variables|Default|GetBox26) (Variables|Default|GetBox27) (Variables|Default|GetBox28) (Variables|Default|GetBox29) (Variables|Default|GetBox30))))