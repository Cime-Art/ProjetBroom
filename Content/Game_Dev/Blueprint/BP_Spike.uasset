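; BP_Spike is a spike trap that rises when a character's capsule overlaps its box and damages characters on it.
; A timeline moves the configurable mesh vertically, and its event track toggles the damaging window.
; A map of overlapping characters to flags limits damage to one hit per cycle, with flags reset and the cycle replayed while occupied.
; The IsInfinite loop is vestigial: SpikeLoop only sets a flag, and its delay logic is disconnected.
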(event OnComponentBeginOverlap(Box)
  (params (OverlappedComponent :type Primitive%20Component%20Object%20Reference) (OtherActor :type Actor%20Object%20Reference) (OtherComp :type Primitive%20Component%20Object%20Reference) (OtherBodyIndex :type Integer) (bFromSweep :type Boolean) (SweepResult :type Hit%20Result%20Structure%20%28by%20ref%29))
  (bind _ascharacter (Utilities|Casting|CastToCharacter OtherActor))
  (Utilities|Casting|CastToCapsuleComponent OtherComp)
  (Utilities|Map|Add (Variables|Default|GetOverlapingActor) _ascharacter true)
  ;[1 1 1] Activate spike if first actor on it
  (if (not (Audio|Components|Audio|IsPlaying (Variables|Default|GetSpike)))
    (CallFunction|ActivateSpike)))

(event OnComponentEndOverlap(Box)
  (params (OverlappedComponent :type Primitive%20Component%20Object%20Reference) (OtherActor :type Actor%20Object%20Reference) (OtherComp :type Primitive%20Component%20Object%20Reference) (OtherBodyIndex :type Integer))
  ;[1 1 1] End Overlap - Remove Actor
  (bind _ascharacter (Utilities|Casting|CastToCharacter OtherActor))
  (Utilities|IsValid _ascharacter
    (:Is%20Valid
      (Utilities|Map|Remove (Variables|Default|GetOverlapingActor) _ascharacter))))

(event Custom|OverlapingActor=0
  ;[1 1 1] Resize
  (if (<= (Utilities|Array|Length (Collision|GetOverlappingActors (Variables|Default|GetBox) "/Script/Engine.Character" :!class /Script/Engine.PrimitiveComponent)) 0)
    _))

(event Custom|SpikeLoop
  (if (not (Variables|Default|GetAlredyActive))
    (Variables|Default|SetAlredyActive true)))

(event Custom|ActivateSpike
  (bind _overlapingactor (Variables|Default|GetOverlapingActor))
  (bind _staticmesh (Variables|Default|GetStaticMesh))
  (bind _relativelocation (Variables|/Script/Engine.SceneComponent|GetRelativeLocation _staticmesh))
  (bind _movement (Timeline|Spike PlayFromStart)
    (:Update
      ;[1 1 1] Déplacement des piques
      (Transformation|SetRelativeLocation _staticmesh (Math|Vector|MakeVector (.x _relativelocation) (.y _relativelocation) (Math|Float|MapRangeClamped _movement 0.0 1.0 -4e+01 (Variables|Default|GetHeight))) false false)
      (if (Variables|Default|GetSpickActive)
        (CallFunction|ApplyDamagetoAll)))
    (:Finished
      ;[1 1 1] Still one actor on spike at the end of timeline
      (if (> (Utilities|Map|Length (Variables|Default|GetOverlapingActor)) 0)
        (bind _keys (Utilities|Map|Keys _overlapingactor))
        (for _array_element _keys
          (Utilities|Map|Add _overlapingactor _array_element true))
        (CallFunction|ActivateSpike)))
    (:SetBoolActiveSpike
      (Variables|Default|SetSpickActive (not (Variables|Default|GetSpickActive))))))

(event Custom|ApplyDamageToAll
  (bind _overlapingactor (Variables|Default|GetOverlapingActor))
  ;[1 1 1] ApplyDamageToAll
  (bind _values (Utilities|Map|Values _overlapingactor))
  (bind _keys (Utilities|Map|Keys _overlapingactor))
  (for (_array_element _array_index) _keys
    (if (Utilities|Array|Get(acopy) _values _array_index)
      (Game|Damage|ApplyDamage _array_element (Variables|OpenVariables|GetDamage) 0 self)
      (Utilities|Map|Add (Variables|Default|GetOverlapingActor) _array_element false))))

(event EventTick
  (params (DeltaSeconds :type Float%20%28single-precision%29))
  ;[1 1 1] Debug
)

(event EventBeginPlay
  ;[1 1 1] Begin play
  (Components|Timeline|SetPlayRate (Variables|Default|GetSpike) (Variables|OpenVariables|GetPlayRate))
  (if (Variables|OpenVariables|GetIsInfinite)
    (CallFunction|SpikeLoop)))

(fn ConstructionScript
  (Components|StaticMesh|SetStaticMesh (Variables|Default|GetStaticMesh) (Variables|OpenVariables|GetMesh)))