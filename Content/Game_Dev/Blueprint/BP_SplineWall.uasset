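; Spline wall actor that tiles spline mesh segments along its spline in the construction script.
; TabMeshesScale maps meshes to lengths; each step places the first entry that fits before the spline end.
; When none fits, the map's last mesh closes the gap to the final point.
; Tangents are clamped to segment length; per-point and closed-loop variants are unconnected, and SelectMesh is an empty stub.
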(event EventBeginPlay)

(event Collision|EventActorBeginOverlap
  (params (OtherActor :type Actor%20Object%20Reference)))

(event EventTick
  (params (DeltaSeconds :type Float%20%28single-precision%29)))

(fn ConstructionScript
  (bind _tabmeshesscale (Variables|Default|GetTabMeshesScale))
  (bind _spline (Variables|Default|GetSpline))
  (bind _spline_2 (Variables|Default|GetSpline))
  (bind _returnvalue (Spline|GetNumberOfSplinePoints _spline))
  (bind _returnvalue_2 (- _returnvalue 1))
  (bind _keys (Utilities|Map|Keys _tabmeshesscale))
  (LocalVariables|SetTempMeshes _keys)
  (bind _values (Utilities|Map|Values _tabmeshesscale))
  (LocalVariables|SetTempDistance _values)
  (LocalVariables|SetSplineDist (Spline|GetSplineLength _spline_2))
  (while (and (< (LocalVariables|GetActualDist) (LocalVariables|GetSplineDist)) (LocalVariables|GetCanPutWall?))
    (LocalVariables|SetCanPutWall? false)
    (LocalVariables|SetStartLocation (Spline|GetLocationatDistanceAlongSpline _spline_2 (LocalVariables|GetActualDist) "Local"))
    (LocalVariables|SetStartTangent (Spline|GetTangentatDistanceAlongSpline _spline_2 (LocalVariables|GetActualDist) "Local"))
    (LocalVariables|SetIndex 0)
    (bind (_array_element _array_index) (Utilities|Array|ForEachLoopwithBreak (LocalVariables|GetTempDistance) :!label _label)
      (:LoopBody
        (LocalVariables|SetIndex _array_index)
        (if (< (+ _array_element (LocalVariables|GetActualDist)) (LocalVariables|GetSplineDist))
          (LocalVariables|SetActualDist (+ _array_element (LocalVariables|GetActualDist)))
          (LocalVariables|SetCanPutWall? true)
          (goto _label Break)))
      (:Completed
        (LocalVariables|SetEndLocation (Math|Vector|SelectVector (Spline|GetLocationatDistanceAlongSpline _spline (LocalVariables|GetActualDist) "Local") (Spline|GetLocationatSplinePoint _spline _returnvalue_2 "Local") (LocalVariables|GetCanPutWall?)))
        (LocalVariables|SetEndTangent (Math|Vector|SelectVector (Spline|GetTangentatDistanceAlongSpline _spline (LocalVariables|GetActualDist) "Local") (Spline|GetTangentatSplinePoint _spline _returnvalue_2 "Local") (LocalVariables|GetCanPutWall?)))
        (bind _returnvalue_3 (AddComponent|AddSplineMeshComponent false))
        (Components|StaticMesh|SetStaticMesh _returnvalue_3 (Utilities|Array|Get(acopy) (LocalVariables|GetTempMeshes) (LocalVariables|GetIndex)))
        (SplineMesh|SetStartandEnd _returnvalue_3 (LocalVariables|GetStartLocation) (Math|Vector|ClampVectorSize (LocalVariables|GetStartTangent) 0.0 (Utilities|Array|Get(acopy) (LocalVariables|GetTempDistance) (LocalVariables|GetIndex))) (LocalVariables|GetEndLocation) (Math|Vector|ClampVectorSize (LocalVariables|GetEndTangent) 0.0 (Utilities|Array|Get(acopy) (LocalVariables|GetTempDistance) (LocalVariables|GetIndex))) true :!class /Script/Engine.SplineMeshComponent)))))

(fn SelectMesh
  (params (Distances :type Array%20of%20Floats%20%28single-precision%29) (CurrentDist :type Float%20%28single-precision%29))
  (return 0))