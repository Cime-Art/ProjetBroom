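; Player controller that switches between gamepad and mouse input and drives the pause and player menus.
; Any key press updates the Gamepad flag and cursor visibility.
; Pause and inventory inputs create or close mutually exclusive widgets and toggle game pause, with WidgetOpen acting as an inverted open flag.
; Menu inputs cycle three wrapping tabs in WG_PlayerMenu and forward left/right item changes to its nested WG_Inventaire.
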(event EventBeginPlay
  (Variables|Default|SetbShowMouseCursor true)
  (Input|SetInputModeGameandUI self 0 "DoNotLock" false))

(event Input|KeyboardEvents|AnyKey
  (params (Key :type Key%20Structure :default "None"))
  (:Pressed
    (if (Class|KismetInputLibrary|KeyIsGamepadKey Key)
      (Variables|Default|SetGamepad? true)
      (Variables|Default|SetbShowMouseCursor false)
      (Class|PlayerController|SetMouseLocation)
      (else
        (Variables|Default|SetGamepad? false)
        (Variables|Default|SetbShowMouseCursor true)))))

(event Custom|Resume
  (Game|SetGamePaused false)
  (Widget|RemovefromParent (Variables|Default|GetWg_Pause))
  (Variables|Default|SetWg_Pause 0))

(event Custom|CloseInventory
  (Game|SetGamePaused false)
  (Variables|Default|SetWidgetOpen true)
  (Default|CloseMenu (Variables|Default|GetWG_Inventaire))
  (Variables|Default|SetWG_Inventaire 0))

(event Input|ActionEvents|InputActionOpenInventaire
  (params (Key :type Key%20Structure :default "None"))
  (:Pressed
    (Utilities|IsValid (Variables|Default|GetWg_Pause)
      (:Is%20Not%20Valid
        (if (Variables|Default|GetWidgetOpen)
          (Variables|Default|SetWidgetOpen false)
          (Game|SetGamePaused true)
          (Utilities|IsValid (Variables|Default|GetWG_Inventaire)
            (:Is%20Not%20Valid
              (bind _returnvalue (UserInterface|CreateWidget "/Game/Game_Dev/Widget/WG_PlayerMenu.WG_PlayerMenu_C"))
              (bind _output_get (Variables|Default|SetWG_Inventaire _returnvalue))
              (UserInterface|Viewport|AddtoViewport _output_get 0)))
          (else
            (Game|SetGamePaused false)
            (Variables|Default|SetWidgetOpen true)
            (Default|CloseMenu (Variables|Default|GetWG_Inventaire))
            (Variables|Default|SetWG_Inventaire 0)))))))

(event Input|ActionEvents|InputActionPauseMenu
  (params (Key :type Key%20Structure :default "None"))
  (:Pressed
    (Utilities|IsValid (Variables|Default|GetWG_Inventaire)
      (:Is%20Not%20Valid
        (Utilities|IsValid (Variables|Default|GetWg_Pause)
          (:Is%20Valid
            (Game|SetGamePaused false)
            (Widget|RemovefromParent (Variables|Default|GetWg_Pause))
            (Variables|Default|SetWg_Pause 0))
          (:Is%20Not%20Valid
            (Development|PrintString "Hello")
            (Game|SetGamePaused true)
            (bind _returnvalue (UserInterface|CreateWidget "/Game/Game_Dev/Widget/WG_PauseMenu.WG_PauseMenu_C"))
            (bind _output_get (Variables|Default|SetWg_Pause _returnvalue))
            (UserInterface|Viewport|AddtoViewport _output_get 0)))))))

(event Input|ActionEvents|InputActionUIReturn
  (params (Key :type Key%20Structure :default "None"))
  (:Pressed
    (Utilities|IsValid (Variables|Default|GetWG_Inventaire)
      (:Is%20Valid
        (CallFunction|CloseInventory)))))

(event Input|ActionEvents|InputActionUIChangeItemLeft
  (params (Key :type Key%20Structure :default "None"))
  (bind _wg_inventaire (Variables|Default|GetWG_Inventaire))
  (:Pressed
    (Utilities|IsValid _wg_inventaire
      (:Is%20Valid
        (bind _aswg_inventaire (Utilities|Casting|CastToWG_Inventaire (Class|PanelWidget|GetChildat (Variables|/Game/Game_Dev/Widget/WG_PlayerMenu.WG_PlayerMenu_C|GetWidgetChild _wg_inventaire))))
        (Default|ChangeLeft _aswg_inventaire)))))

(event Input|ActionEvents|InputActionUIChangeItemRight
  (params (Key :type Key%20Structure :default "None"))
  (bind _wg_inventaire (Variables|Default|GetWG_Inventaire))
  (:Pressed
    (Utilities|IsValid _wg_inventaire
      (:Is%20Valid
        (bind _aswg_inventaire (Utilities|Casting|CastToWG_Inventaire (Class|PanelWidget|GetChildat (Variables|/Game/Game_Dev/Widget/WG_PlayerMenu.WG_PlayerMenu_C|GetWidgetChild _wg_inventaire))))
        (Default|ChangeRight _aswg_inventaire)))))

(event Input|ActionEvents|InputActionUIChangeMenuLeft
  (params (Key :type Key%20Structure :default "None"))
  (bind _wg_inventaire (Variables|Default|GetWG_Inventaire))
  (:Pressed
    (Utilities|IsValid _wg_inventaire
      (:Is%20Valid
        (Variables|/Game/Game_Dev/Widget/WG_PlayerMenu.WG_PlayerMenu_C|SetIndexMenu _wg_inventaire (Math|Integer|SelectInt 2 (- (Variables|/Game/Game_Dev/Widget/WG_PlayerMenu.WG_PlayerMenu_C|GetIndexMenu _wg_inventaire) 1) (== (Variables|/Game/Game_Dev/Widget/WG_PlayerMenu.WG_PlayerMenu_C|GetIndexMenu _wg_inventaire) 0)))
        (Default|ChangeMenu _wg_inventaire)))))

(event Input|ActionEvents|InputActionUiChangeMenuRight
  (params (Key :type Key%20Structure :default "None"))
  (bind _wg_inventaire (Variables|Default|GetWG_Inventaire))
  (:Pressed
    (Utilities|IsValid _wg_inventaire
      (:Is%20Valid
        (Variables|/Game/Game_Dev/Widget/WG_PlayerMenu.WG_PlayerMenu_C|SetIndexMenu _wg_inventaire (Math|Integer|SelectInt 0 (+ (Variables|/Game/Game_Dev/Widget/WG_PlayerMenu.WG_PlayerMenu_C|GetIndexMenu _wg_inventaire) 1) (== (Variables|/Game/Game_Dev/Widget/WG_PlayerMenu.WG_PlayerMenu_C|GetIndexMenu _wg_inventaire) 2)))
        (Default|ChangeMenu _wg_inventaire)))))

(fn ConstructionScript)