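; Lava platform that shakes, then rises toward a configurable height, with its mesh set by the construction script.
; With DontLoop on, a player overlapping the box triggers it once until reset.
; The Shake timeline jitters the mesh in XY, then after a delay MovingPlatform drives its height, stopping near the top.
; ResetAll cancels a pending rise, recenters the mesh, rewinds both timelines and re-arms the trigger.
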(event OnComponentBeginOverlap(Box)
  (params (OverlappedComponent :type Primitive%20Component%20Object%20Reference) (OtherActor :type Actor%20Object%20Reference) (OtherComp :type Primitive%20Component%20Object%20Reference) (OtherBodyIndex :type Integer) (bFromSweep :type Boolean) (SweepResult :type Hit%20Result%20Structure%20%28by%20ref%29))
  (bind _returnvalue (Math|Random|RandomFloatinRange -2.0 2.0))
  (Utilities|Casting|CastToBP_PlayerTest OtherActor)
  (if (Variables|OpenVariable|GetDontLoop)
    (Utilities|FlowControl|DoOnce false
      (:Completed
        (Timeline|Shake PlayFromStart
          (:Update
            (Variables|Default|SetRandomX _returnvalue)
            (Variables|Default|SetRandomY _returnvalue)
            (Transformation|SetRelativeLocation (Variables|Default|GetStaticMesh) (Math|Vector|MakeVector (Variables|Default|GetRandomX) (Variables|Default|GetRandomY) (Math|Float|MapRangeClamped (stale _movingz) 0.0 1.0 0.0 (Variables|OpenVariable|GetmaxHeight))) false false :!label _label)
            (if (and (>= (stale _movingz) 0.99) (Variables|OpenVariable|GetDontLoop))
              (Audio|Components|Audio|Stop (Variables|Default|GetMovingPlatform))))
          (:Finished
            (Variables|Default|SetReset false)
            (Utilities|FlowControl|Delay (Variables|OpenVariable|GetDelayBeforeUp))
            (if (not (Variables|Default|GetReset))
              (bind _movingz (Timeline|MovingPlatform PlayFromStart)
                (:Update
                  (goto _label))
                (:Finished
                  (CallFunction|ResetAll))))))))))

(event Custom|ResetAll
  (bind _returnvalue (Math|Random|RandomFloatinRange -2.0 2.0))
  (bind _shake (Variables|Default|GetShake))
  (Variables|Default|SetReset true)
  (Audio|Components|Audio|Stop _shake)
  (Transformation|SetRelativeLocation (Variables|Default|GetStaticMesh) "0, 0, 0" false false)
  (Components|Timeline|SetPlaybackPosition _shake 0.0 false true)
  (Components|Timeline|SetPlaybackPosition (Variables|Default|GetMovingPlatform) 0.0 false true)
  (Utilities|FlowControl|DoOnce false) ; enters at Reset
)

(event EventBeginPlay
  (bind _shake (Variables|Default|GetShake))
  (Components|Timeline|SetPlayRate (Variables|Default|GetShake) (Variables|OpenVariable|GetShaking%20Time))
  (Components|Timeline|SetPlayRate (Variables|Default|GetMovingPlatform) (Variables|OpenVariable|GetSpeed))
  (if (Variables|OpenVariable|GetDontLoop)
    (Components|Timeline|SetLooping _shake false)
    (Audio|Components|Audio|Stop _shake)))

(fn ConstructionScript
  (Components|StaticMesh|SetStaticMesh (Variables|Default|GetStaticMesh) (Variables|OpenVariable|GetMesh)))