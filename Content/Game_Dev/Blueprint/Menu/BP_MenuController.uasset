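; Menu controller that routes UI input actions for the main menu and options screen.
; It sets Game and UI input mode, flags gamepad key presses, and lets a skip action load the menu through RefWidget.
; Options inputs switch left or right, open the apply popup and confirm settings.
; Return closes an open popup and refocuses the first switch or slider, otherwise it replaces the options widget with a new WG_MainMenu.
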(event Custom|ReturnOption
  ;[1 1 1] Switch Menu + Input For UI
  ;;[1 1 1] ReturnOption
  (Widget|RemovefromParent (Variables|Default|GetWg_MenuOption))
  (bind _output_get (Variables|Default|SetWg_MenuOption 0))
  (Development|PrintString (Utilities|GetDisplayName _output_get))
  (bind _returnvalue (UserInterface|CreateWidget "/Game/Game_Dev/Widget/WG_MainMenu.WG_MainMenu_C"))
  (UserInterface|Viewport|AddtoViewport _returnvalue 0))

(event EventBeginPlay
  (Input|SetInputModeGameandUI (Game|GetPlayerController 0) 0 "DoNotLock" true))

(event Input|ActionEvents|InputActionUIBtnA
  (params (Key :type Key%20Structure :default "None"))
  (bind _wg_menuoption (Variables|Default|GetWg_MenuOption))
  (bind _validapply (Variables|/Game/Game_Dev/Widget/WG_MenuOption.WG_MenuOption_C|GetValidApply _wg_menuoption))
  ;[1 1 1] Switch Menu + Input For UI
  (:Pressed
    (Utilities|IsValid _validapply
      (:Is%20Valid
        (Default|ApplySettings _wg_menuoption)
        (Widget|RemovefromParent _validapply)))))

(event Input|ActionEvents|InputActionUISkippMainMenu
  (params (Key :type Key%20Structure :default "None"))
  (:Pressed
    (Utilities|IsValid (Variables|Default|GetRefWidget)
      (:Is%20Valid
        (Default|LoadMenu (Variables|Default|GetRefWidget))
        (Variables|Default|SetRefWidget 0)))))

(event Input|ActionEvents|InputActionUIReturn
  (params (Key :type Key%20Structure :default "None"))
  (bind _wg_menuoption (Variables|Default|GetWg_MenuOption))
  (bind _wg_menuoption_2 (Variables|Default|GetWg_MenuOption))
  (bind _returnvalue (Widget|GetOwningPlayer _wg_menuoption))
  (bind _scrollbox_param (Variables|/Game/Game_Dev/Widget/WG_MenuOption.WG_MenuOption_C|GetScrollBox_Param _wg_menuoption_2))
  (bind _returnvalue_2 (Class|PanelWidget|GetChildat _scrollbox_param))
  ;[1 1 1] Switch Menu + Input For UI
  ;;[1 1 1] ReturnOption
  (:Pressed
    (Utilities|IsValid _wg_menuoption_2
      (:Is%20Valid
        (Utilities|IsValid (Variables|/Game/Game_Dev/Widget/WG_MenuOption.WG_MenuOption_C|GetValidApply _wg_menuoption_2)
          (:Is%20Valid
            (Widget|RemovefromParent (Variables|/Game/Game_Dev/Widget/WG_MenuOption.WG_MenuOption_C|GetValidApply _wg_menuoption_2))
            (Variables|/Game/Game_Dev/Widget/WG_MenuOption.WG_MenuOption_C|SetValidApply _wg_menuoption_2 0)
            (bind _aswg_switch_option (Utilities|Casting|CastToWG_SwitchOption _returnvalue_2)
              (:then
                (Class|Widget|SetUserFocus (Variables|/Game/Game_Dev/Widget/WG_SwitchOption.WG_SwitchOption_C|GetButton_Left _aswg_switch_option) _returnvalue))
              (:CastFailed
                (bind _aswg_slider (Utilities|Casting|CastToWG_Slider _returnvalue_2))
                (Class|Widget|SetUserFocus (Variables|/Game/Game_Dev/Widget/WG_Slider.WG_Slider_C|GetSlider_Param _aswg_slider) _returnvalue))))
          (:Is%20Not%20Valid
            (CallFunction|ReturnOption)))))))

(event Input|ActionEvents|InputActionUIButtonApply
  (params (Key :type Key%20Structure :default "None"))
  (bind _wg_menuoption (Variables|Default|GetWg_MenuOption))
  ;[1 1 1] Switch Menu + Input For UI
  (:Pressed
    (Utilities|IsValid _wg_menuoption
      (:Is%20Valid
        (Utilities|IsValid (Variables|/Game/Game_Dev/Widget/WG_MenuOption.WG_MenuOption_C|GetValidApply _wg_menuoption)
          (:Is%20Not%20Valid
            (Default|OpenPopUpApply _wg_menuoption)))))))

(event Input|ActionEvents|InputActionUISwitchMenuOptionLeft
  (params (Key :type Key%20Structure :default "None"))
  (bind _wg_menuoption (Variables|Default|GetWg_MenuOption))
  ;[1 1 1] Switch Menu + Input For UI
  (:Pressed
    (Utilities|IsValid _wg_menuoption
      (:Is%20Valid
        (Utilities|IsValid (Variables|/Game/Game_Dev/Widget/WG_MenuOption.WG_MenuOption_C|GetValidApply _wg_menuoption)
          (:Is%20Not%20Valid
            (Default|ChangeLeft _wg_menuoption)))))))

(event Input|ActionEvents|InputActionUISwitchMenuOptionRight
  (params (Key :type Key%20Structure :default "None"))
  (bind _wg_menuoption (Variables|Default|GetWg_MenuOption))
  ;[1 1 1] Switch Menu + Input For UI
  (:Pressed
    (Utilities|IsValid _wg_menuoption
      (:Is%20Valid
        (Utilities|IsValid (Variables|/Game/Game_Dev/Widget/WG_MenuOption.WG_MenuOption_C|GetValidApply _wg_menuoption)
          (:Is%20Not%20Valid
            (Default|ChangeRight _wg_menuoption)))))))

(event Input|KeyboardEvents|AnyKey
  (params (Key :type Key%20Structure :default "None"))
  (:Pressed
    (Variables|Default|SetGamepad? (Class|KismetInputLibrary|KeyIsGamepadKey Key))))

(fn ConstructionScript)