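; Chest actor that opens and throws out loot when BP_PlayerTest overlaps its box.
; The OpenChest timeline rotates the lid on roll, then a DoOnce spawns one Bp_Loot and the NS_Chest Niagara effect.
; A second timeline sweeps the loot along Y from the chest and along absolute world Z, scaled by MovingY and MovingZ.
; BeginPlay sets a timeline play rate from the Loot variable.
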(event OnComponentBeginOverlap(Box)
  (params (OverlappedComponent :type Primitive%20Component%20Object%20Reference) (OtherActor :type Actor%20Object%20Reference) (OtherComp :type Primitive%20Component%20Object%20Reference) (OtherBodyIndex :type Integer) (bFromSweep :type Boolean) (SweepResult :type Hit%20Result%20Structure%20%28by%20ref%29))
  (bind _returnvalue (Transformation|GetActorTransform))
  (bind _returnvalue_2 (Transformation|GetActorLocation))
  (Utilities|Casting|CastToBP_PlayerTest OtherActor)
  (bind _rotation (Timeline|OpenChest Play)
    (:Update
      (Transformation|SetRelativeRotation (Variables|Default|GetCoffre_Couvercle_coffe) (Math|Rotator|MakeRotator (Math|Float|MapRangeClamped _rotation 0.0 1.0 0.0 (Variables|Default|GetRotation%20coffre)) 0.0 0.0) false false))
    (:Finished
      (Utilities|FlowControl|DoOnce false
        (:Completed
          (bind _returnvalue_3 (Game|SpawnActorfromClass "/Game/Game_Dev/Blueprint/GameplayScript/chest/Bp_Loot.Bp_Loot_C" (Math|Transform|MakeTransform (Transformation|GetActorLocation) "0, 0, 0" "1,1,1") "AdjustIfPossibleButAlwaysSpawn" 0 0))
          (Niagara|SpawnSystematLocation "/Game/Game_Dev/Blueprint/GameplayScript/chest/NS_Chest.NS_Chest" (.location _returnvalue) (.rotation _returnvalue) (.scale _returnvalue))
          (bind (_direction _lootz _newtrack_2) (Timeline|Timeline_0 PlayFromStart)
            (:Update
              (Transformation|SetActorLocation _returnvalue_3 (Math|Vector|MakeVector (.x _returnvalue_2) (+ (Math|Float|MapRangeClamped _newtrack_2 0.0 2.0 0.0 (Variables|Default|GetMoving%20Y)) (.y _returnvalue_2)) (Math|Float|MapRangeClamped _lootz 0.0 2.0 0.0 (Variables|Default|GetMovingZ))) true false))))))))

(event EventBeginPlay
  (Components|Timeline|SetPlayRate (Variables|Default|GetTimeline_0) (Variables|Default|GetLoot%20)))

(fn ConstructionScript)