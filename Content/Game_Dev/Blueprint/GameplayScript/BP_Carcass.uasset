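; BP_Carcass is a tutorial prop, a chained skeletal-mesh carcass that reacts as tutorial steps are passed.
; StepPass runs each indexed step once: a physics shove on a chain bone, then temporary immobilisation and acid material swaps, each followed by a tutorial preview widget.
; The final step opens the linked BPDoor.
; Separate TakeHit and self-repeating ResetForce events handle impact forces; a delayed constraint destruction is left unconnected.
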(event Custom|StepPass
  (params (Index :type Integer))
  (bind _skeletalmesh (Variables|Default|GetSkeletalMesh))
  (switch int Index
    (:0
      (Utilities|FlowControl|DoOnce false
        (:Completed
          (Class|PrimitiveComponent|AddForceatLocation (Variables|Default|GetSkeletalMesh) (Math|Vector|MakeVector 5e+04 5e+04 0.0) "0, 0, 0" "chaine29_skn")
          (Utilities|FlowControl|Delay 1.5)
          (bind _returnvalue (UserInterface|CreateWidget "/Game/Game_Dev/Blueprint/Widget/Tuto/HUD_Tuto_Preview.HUD_Tuto_Preview_C" 0 "NewEnumerator1"))
          (UserInterface|Viewport|AddtoViewport _returnvalue 0))))
    (:1
      (Utilities|FlowControl|DoOnce false
        (:Completed
          (Variables|Default|SetMat_Carcass (Utilities|Array|Get(acopy) (Rendering|Material|GetMaterials (Variables|Default|GetSkeletalMesh)) 1))
          (Rendering|Material|SetMaterial _skeletalmesh 1 "/Game/Game_Dev/Material/M_SpellImmo_Inst.M_SpellImmo_Inst")
          (Utilities|FlowControl|Delay 1.5)
          (Rendering|Material|SetMaterial _skeletalmesh 1 (Variables|Default|GetMat_Carcass))
          (bind _returnvalue_2 (UserInterface|CreateWidget "/Game/Game_Dev/Blueprint/Widget/Tuto/HUD_Tuto_Preview.HUD_Tuto_Preview_C" 0 "NewEnumerator3"))
          (UserInterface|Viewport|AddtoViewport _returnvalue_2 0))))
    (:2
      (Utilities|FlowControl|DoOnce false
        (:Completed
          (Rendering|Material|SetMaterial (Variables|Default|GetSkeletalMesh) 1 "/Game/Game_ART/TEMP/Material/Mat_Block/Acide_Inst.Acide_Inst")
          (Utilities|FlowControl|Delay 1.5)
          (Rendering|Material|SetMaterial (Variables|Default|GetSkeletalMesh) 1 (Variables|Default|GetMat_Carcass))
          (bind _returnvalue_3 (UserInterface|CreateWidget "/Game/Game_Dev/Blueprint/Widget/Tuto/HUD_Tuto_Preview.HUD_Tuto_Preview_C" 0 "NewEnumerator4"))
          (UserInterface|Viewport|AddtoViewport _returnvalue_3 0))))
    (:3
      (Utilities|FlowControl|DoOnce false
        (:Completed
          (Default|OpenDoor (Variables|Default|GetBP_Door)))))))

(event Custom|ResetForce
  (Utilities|FlowControl|DoOnce false) ; enters at Reset
)

(event Custom|TakeHit
  (params (Impact :type Vector))
  (Utilities|IsValid (Variables|Default|GetPhysicsConstraint)
    (:Is%20Valid
      (Utilities|FlowControl|DoOnce false
        (:Completed
          (Physics|AddForce (Variables|Default|GetSkeletalMesh) (* Impact -3e+03) "chaine29_skn" false)
          (Utilities|FlowControl|Delay 3.0)
          (CallFunction|ResetForce))))))

(event EventBeginPlay)

(fn ConstructionScript)