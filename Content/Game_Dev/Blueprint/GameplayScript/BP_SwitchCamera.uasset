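; BP_SwitchCamera is a trigger volume that blends the view to its assigned camera actor while the player is inside.
; Box begin overlap stores that camera on BP_PlayerTest and blends to it; end overlap clears it and blends back only if no other switch volume still overlaps.
; Tick feeds the player's overlap state to the camera's PlayerIn, and construction applies the configured field of view.
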(event OnComponentBeginOverlap(Box)
  (params (OverlappedComponent :type Primitive%20Component%20Object%20Reference) (OtherActor :type Actor%20Object%20Reference) (OtherComp :type Primitive%20Component%20Object%20Reference) (OtherBodyIndex :type Integer) (bFromSweep :type Boolean) (SweepResult :type Hit%20Result%20Structure%20%28by%20ref%29))
  (bind _asbp_player_test (Utilities|Casting|CastToBP_PlayerTest OtherActor))
  (bind _output_get (Variables|/Game/Game_Dev/Blueprint/Player/BP_PlayerTest.BP_PlayerTest_C|SetCameraSwitch _asbp_player_test (Variables|Default|GetCameraActor)))
  (Game|Player|SetViewTargetwithBlend (Game|GetPlayerController 0) _output_get (Variables|Default|GetBeginBlend) "VTBlend_Linear" 0.0 true))

(event OnComponentEndOverlap(Box)
  (params (OverlappedComponent :type Primitive%20Component%20Object%20Reference) (OtherActor :type Actor%20Object%20Reference) (OtherComp :type Primitive%20Component%20Object%20Reference) (OtherBodyIndex :type Integer))
  (bind _asbp_player_test (Utilities|Casting|CastToBP_PlayerTest OtherActor))
  (if (not (Collision|IsOverlappingActor _asbp_player_test (Utilities|Array|Get(acopy) (Collision|GetOverlappingActors (Variables|/Script/Engine.Character|GetCapsuleComponent _asbp_player_test) "BP_SwitchCamera_C" :!class /Script/Engine.PrimitiveComponent)) :!class /Script/Engine.Actor))
    (Variables|/Game/Game_Dev/Blueprint/Player/BP_PlayerTest.BP_PlayerTest_C|SetCameraSwitch _asbp_player_test 0)
    (Game|Player|SetViewTargetwithBlend (Game|GetPlayerController 0) _asbp_player_test (Variables|Default|GetEndBlend) "VTBlend_Linear" 0.0 true)))

(event EventTick
  (params (DeltaSeconds :type Float%20%28single-precision%29))
  (Variables|/Game/Game_Dev/Blueprint/GameplayScript/BP_CameraSpline.BP_CameraSpline_C|SetPlayerIn (Variables|Default|GetCameraActor) (Collision|IsOverlappingActor (Variables|Default|GetBox) (CallFunction|CastPlayer) :!class /Script/Engine.PrimitiveComponent)))

(fn ConstructionScript
  (Camera|SetFieldOfView (Variables|/Script/Engine.CameraActor|GetCameraComponent (Variables|Default|GetCameraActor)) (Variables|Default|GetField%20of%20View)))