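; Death trigger volume that handles the player falling or entering it and makes trash mob AIs fall.
; Player overlap runs through a DoOnce, reset on end overlap, that pauses the game and shows the Respawn widget with tips if lives remain, otherwise the Continue widget.
; Trash mobs entering the box call their Fall event instead.
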(event OnComponentBeginOverlap(Box)
  (params (OverlappedComponent :type Primitive%20Component%20Object%20Reference) (OtherActor :type Actor%20Object%20Reference) (OtherComp :type Primitive%20Component%20Object%20Reference) (OtherBodyIndex :type Integer) (bFromSweep :type Boolean) (SweepResult :type Hit%20Result%20Structure%20%28by%20ref%29))
  (Utilities|Casting|CastToBP_PlayerTest OtherActor
    (:then
      (Utilities|FlowControl|DoOnce false
        (:Completed
          (Game|SetGamePaused true)
          (if (> (.currentlife (Variables|/Game/Game_Dev/Blueprint/Player/BP_PlayerTest.BP_PlayerTest_C|GetInfoPlayer (CallFunction|CastPlayer))) 0)
            (Variables|Default|GetRespawn
              (:then
                (Variables|Default|SetRespawn 0))
              (:else
                _))
            (bind _returnvalue (UserInterface|CreateWidget "/Game/Game_Dev/Blueprint/Widget/Respawn/WG_Respawn.WG_Respawn_C" 0 (Variables|OpenVariable|GetTips) (Variables|OpenVariable|GetSpecialTips?) (Variables|OpenVariable|GetSpecialTip)))
            (bind _output_get (Variables|Default|SetRespawn _returnvalue))
            (UserInterface|Viewport|AddtoViewport _output_get 0)
            (else
              (Variables|Default|GetContinue
                (:then
                  (Variables|Default|SetContinue 0))
                (:else
                  _))
              (bind _returnvalue_2 (UserInterface|CreateWidget "/Game/Game_Dev/Blueprint/Widget/Respawn/WG_Continue.WG_Continue_C"))
              (bind _output_get_2 (Variables|Default|SetContinue _returnvalue_2))
              (UserInterface|Viewport|AddtoViewport _output_get_2 0))))))
    (:CastFailed
      (bind _asbp_ia_trash_mob (Utilities|Casting|CastToBP_IA_TrashMob OtherActor))
      (Default|Fall _asbp_ia_trash_mob))))

(event OnComponentEndOverlap(Box)
  (params (OverlappedComponent :type Primitive%20Component%20Object%20Reference) (OtherActor :type Actor%20Object%20Reference) (OtherComp :type Primitive%20Component%20Object%20Reference) (OtherBodyIndex :type Integer))
  (Utilities|Casting|CastToBP_PlayerTest OtherActor)
  (CallFunction|ResetDoOnce))

(event Custom|ResetDoOnce
  (Utilities|FlowControl|DoOnce false) ; enters at Reset
)

(fn ConstructionScript)