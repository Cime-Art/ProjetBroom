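; Camera rail actor that moves a camera along a spline to follow the player while its PlayerIn flag is set.
; Each tick it turns the camera to look at the player and eases it toward the spline point closest to them.
; The easing is a lerp from the current position with delta seconds as alpha, giving a lagging follow.
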(event EventTick
  (params (DeltaSeconds :type Float%20%28single-precision%29))
  (bind _cameracomponent (Variables|CameraActor|GetCameraComponent))
  (bind _cameracomponent_2 (Variables|CameraActor|GetCameraComponent))
  (if (Variables|Default|GetPlayerIn)
    (Transformation|SetWorldRotation _cameracomponent_2 (Math|Rotator|FindLookatRotation (Transformation|GetWorldLocation _cameracomponent_2) (Transformation|GetActorLocation (CallFunction|CastPlayer))) false false)
    (Transformation|SetWorldLocation _cameracomponent (Math|Vector|Lerp(Vector) (Transformation|GetWorldLocation _cameracomponent) (Spline|FindLocationClosesttoWorldLocation (Variables|Default|GetSpline) (Transformation|GetActorLocation (CallFunction|CastPlayer)) "World") (Utilities|Time|GetWorldDeltaSeconds)) false false)))

(fn ConstructionScript)