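; BP_PlayerAttack is an animation notify state that applies the player's melee damage during an attack animation.
; Each notify tick sphere-traces on Visibility between the mesh's RightHand and HandR sockets, looking for BP_IA_TrashMob hits.
; A mob missing from BP_PlayerTest's ListeEnemy is added and takes fixed damage, so listed mobs are not hit again.
; The list is not cleared here.
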(fn ReceivedNotifyTick
  (params (MeshComp :type Skeletal%20Mesh%20Component%20Object%20Reference) (Animation :type Anim%20Sequence%20Base%20Object%20Reference) (FrameDeltaTime :type Float%20%28single-precision%29))
  (bind _returnvalue (Game|GetPlayerCharacter MeshComp))
  (bind _asbp_player_test (Utilities|Casting|CastToBP_PlayerTest _returnvalue))
  (bind _listeenemy (Variables|/Game/Game_Dev/Blueprint/BP_PlayerTest.BP_PlayerTest_C|GetListeEnemy _asbp_player_test))
  (bind _outhits (Collision|MultiSphereTraceByChannel MeshComp (Transformation|GetSocketLocation MeshComp "RightHand") (Transformation|GetSocketLocation MeshComp "HandR") 4e+01 "TraceTypeQuery1" false 0 "None"))
  (bind _array_element (Utilities|Array|ForEachLoopwithBreak _outhits)
    (:LoopBody
      (bind _asbp_ia_trash_mob (Utilities|Casting|CastToBP_IA_TrashMob (.HitActor (Collision|BreakHitResult _array_element))))
      (if (not (Utilities|Array|ContainsItem _listeenemy _asbp_ia_trash_mob))
        (Utilities|Array|Add _listeenemy _asbp_ia_trash_mob)
        (Default|TakeDamage _asbp_ia_trash_mob 35.0)
        (return true)))))