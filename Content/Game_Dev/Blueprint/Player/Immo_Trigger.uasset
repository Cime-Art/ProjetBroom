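; Short-lived cone trigger actor that detects trash mobs and carcasses for what appears to be the player's "Immo" ability.
; Overlapping BP_IA_TrashMob actors are added uniquely to the player's IATrashmobImmo array and removed on end overlap, while overlapping BP_Carcass actors receive StepPass(1).
; The actor destroys itself 0.1 seconds after BeginPlay and clears the player's array when destroyed.
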(event OnComponentBeginOverlap(Cone_Trigger)
  (params (OverlappedComponent :type Primitive%20Component%20Object%20Reference) (OtherActor :type Actor%20Object%20Reference) (OtherComp :type Primitive%20Component%20Object%20Reference) (OtherBodyIndex :type Integer) (bFromSweep :type Boolean) (SweepResult :type Hit%20Result%20Structure%20%28by%20ref%29))
  (bind _asbp_ia_trash_mob (Utilities|Casting|CastToBP_IA_TrashMob OtherActor)
    (:then
      (Utilities|Array|AddUnique (Variables|/Game/Game_Dev/Blueprint/Player/BP_PlayerTest.BP_PlayerTest_C|GetIA_Trashmob_Immo (CallFunction|CastPlayer)) _asbp_ia_trash_mob))
    (:CastFailed
      (bind _asbp_carcass (Utilities|Casting|CastToBP_Carcass OtherActor))
      (Default|StepPass _asbp_carcass 1))))

(event OnComponentEndOverlap(Cone_Trigger)
  (params (OverlappedComponent :type Primitive%20Component%20Object%20Reference) (OtherActor :type Actor%20Object%20Reference) (OtherComp :type Primitive%20Component%20Object%20Reference) (OtherBodyIndex :type Integer))
  (bind _asbp_player_test (CallFunction|CastPlayer))
  (bind _ia_trashmob_immo (Variables|/Game/Game_Dev/Blueprint/Player/BP_PlayerTest.BP_PlayerTest_C|GetIA_Trashmob_Immo _asbp_player_test))
  (bind _asbp_ia_trash_mob (Utilities|Casting|CastToBP_IA_TrashMob OtherActor))
  (Utilities|Array|RemoveIndex _ia_trashmob_immo (Utilities|Array|FindItem _ia_trashmob_immo _asbp_ia_trash_mob)))

(event EventDestroyed
  (Utilities|Array|Clear (Variables|/Game/Game_Dev/Blueprint/Player/BP_PlayerTest.BP_PlayerTest_C|GetIA_Trashmob_Immo (CallFunction|CastPlayer))))

(event EventBeginPlay
  (Utilities|FlowControl|Delay 0.1)
  (Actor|DestroyActor))

(fn ConstructionScript)