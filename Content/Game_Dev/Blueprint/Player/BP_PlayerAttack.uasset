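; BP_PlayerAttack is an animation notify state that deals melee damage to trash mob enemies during the player's attack animation.
; Each tick it sphere-traces between two right-hand sockets on the mesh and filters hits to BP_IA_TrashMob.
; Mobs not yet in player 0's IATrashmobAttacSystem array are added and take fixed damage, preventing repeat hits while listed.
; The tick returns after the first new mob damaged.
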(fn ReceivedNotifyTick
  (params (MeshComp :type Skeletal%20Mesh%20Component%20Object%20Reference) (Animation :type Anim%20Sequence%20Base%20Object%20Reference) (FrameDeltaTime :type Float%20%28single-precision%29))
  (bind _returnvalue (Game|GetPlayerCharacter MeshComp))
  (bind _asbp_player_test (Utilities|Casting|CastToBP_PlayerTest _returnvalue))
  (bind _ia_trashmob_attac_system (Variables|/Game/Game_Dev/Blueprint/Player/BP_PlayerTest.BP_PlayerTest_C|GetIA_Trashmob_Attac_System _asbp_player_test))
  (bind _outhits (Collision|MultiSphereTraceByChannel MeshComp (Transformation|GetSocketLocation MeshComp "RightHand") (Transformation|GetSocketLocation MeshComp "HandR") 4e+01 "TraceTypeQuery1" false 0 "None"))
  (bind _array_element (Utilities|Array|ForEachLoopwithBreak _outhits)
    (:LoopBody
      (Utilities|FlowControl|Sequence
        (:then_0
          (bind _asbp_ia_trash_mob (Utilities|Casting|CastToBP_IA_TrashMob (.HitActor (Collision|BreakHitResult _array_element))))
          (if (not (Utilities|Array|ContainsItem _ia_trashmob_attac_system _asbp_ia_trash_mob))
            (Utilities|Array|Add _ia_trashmob_attac_system _asbp_ia_trash_mob)
            (Game|Damage|ApplyDamage _asbp_ia_trash_mob 5e+01 0 0)
            (return true)))))))