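; BP_LightSystem is a light actor whose intensity can vary continuously and randomly between a minimum and maximum.
; Its construction script adds a point, spot or rect light component according to the Lights selection.
; The restart event plays a timeline that lerps intensity toward a random target, then picks another and calls itself.
; BeginPlay sets the play rate and first target, but does not trigger that loop.
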(event Custom|restart
  (bind _newtrack_0 (Timeline|Intensity PlayFromStart)
    (:Update
      (Rendering|Components|Light|SetIntensity (Variables|Default|GetCurrentLight) (Math|Float|Lerp (Variables|Default|GetOldIntensity) (Variables|Default|GetFuturIntensity) _newtrack_0)))
    (:Finished
      (Variables|Default|SetFuturIntensity (Math|Random|RandomFloatinRange (Variables|Default|GetMinIntensity) (Variables|Default|GetMaxIntensity)))
      (Variables|Default|SetOldIntensity (Variables|/Script/Engine.LightComponentBase|GetIntensity (Variables|Default|GetCurrentLight)))
      (CallFunction|Restart))))

(event EventBeginPlay
  (Components|Timeline|SetPlayRate (Variables|Default|GetIntensity) (Variables|Default|GetPlayRate))
  (Variables|Default|SetOldIntensity (Variables|/Script/Engine.LightComponentBase|GetIntensity (Variables|Default|GetCurrentLight)))
  (Variables|Default|SetFuturIntensity (Math|Random|RandomFloatinRange (Variables|Default|GetMinIntensity) (Variables|Default|GetMaxIntensity))))

(fn ConstructionScript
  (switch Utilities|FlowControl|Switch|SwitchonEnum_Lights (Variables|Default|GetLights)
    (:NewEnumerator0
      (bind _returnvalue (AddComponent|AddPointLightComponent false))
      (Variables|Default|SetCurrentLight _returnvalue))
    (:NewEnumerator1
      (bind _returnvalue_2 (AddComponent|AddSpotLightComponent false))
      (Variables|Default|SetCurrentLight _returnvalue_2))
    (:NewEnumerator2
      (bind _returnvalue_3 (AddComponent|AddRectLightComponent false))
      (Variables|Default|SetCurrentLight _returnvalue_3))))