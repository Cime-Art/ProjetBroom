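; Boiler trap that shoots a Niagara flame and deals massive damage to BP_PlayerTest through a sphere trace along the emitter's up vector.
; In cyclic mode, timelines shake the grill, then drive its rotation, fire emissive and toggled damage window, before waiting through the Delay array in rotation.
; IsInfinite instead keeps the grill open and flame on, with a timeline running the trace.
; The construction script sets grill visibility.
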(event Custom|Flames
  (bind _meshgrill (Variables|Default|GetMeshGrill))
  (bind _niagara (Variables|Default|GetNiagara))
  (bind _meshgrill_2 (Variables|Default|GetMeshGrill))
  (bind _returnvalue (Transformation|GetWorldLocation _niagara))
  (bind _relativerotation (Variables|/Script/Engine.SceneComponent|GetRelativeRotation _meshgrill))
  (bind _relativerotation_2 (Variables|/Script/Engine.SceneComponent|GetRelativeRotation _meshgrill_2))
  (Class|AkGameObject|PostAssociatedAkEvent (Variables|Default|GetAk_BoilerAction))
  (Timeline|ShakeGrill PlayFromStart
    (:Update
      (bind _output_get (Variables|Default|SetRandomX (Math|Random|RandomFloatinRange -2.5 2.5)))
      (Transformation|SetRelativeRotation _meshgrill (Math|Rotator|MakeRotator (.roll _relativerotation) (.pitch _relativerotation) (+ (Variables|Default|GetRandomX) _output_get)) false false))
    (:Finished
      (Components|Activation|SetActive (Variables|Default|GetNiagara) true true)
      (bind (_direction _emissivefire _rotationgrill) (Timeline|NiagaraSystem PlayFromStart)
        (:Update
          (Rendering|Material|SetScalarParameterValueonMaterials (Variables|Default|GetStaticMesh) "EmissiveFire" _emissivefire)
          ;[1 1 1] Detect Damage
          (Transformation|SetRelativeRotation _meshgrill_2 (Math|Rotator|MakeRotator (.roll _relativerotation_2) (.pitch _relativerotation_2) _rotationgrill) false false)
          (if (Variables|Default|GetDetectDamage?)
            (bind _outhit (Collision|SphereTraceByChannel _returnvalue (+ _returnvalue (* (Math|Vector|GetUpVector _niagara) (Variables|OpenVariables|GetDist))) 2e+01 "TraceTypeQuery1" false 0 "ForOneFrame"))
            (bind _asbp_player_test (Utilities|Casting|CastToBP_PlayerTest (.hitactor _outhit)))
            (Default|SetterHP _asbp_player_test 1e+03 false)))
        (:Finished
          (Components|Activation|SetActive (Variables|Default|GetNiagara) false false)
          (Utilities|FlowControl|Delay (Utilities|Array|Get(acopy) (Variables|OpenVariables|GetDelay) (Variables|Default|GetCount)))
          (Variables|Default|SetCount (Math|Integer|SelectInt 0 (+ (Variables|Default|GetCount) 1) (> (+ (Variables|Default|GetCount) 1) (Utilities|Array|LastIndex (Variables|OpenVariables|GetDelay)))))
          (CallFunction|Flames))
        (:SetBoolTrack
          (bind _isa (Utilities|FlowControl|FlipFlop)
            (:A
              _)
            (:B
              _))
          (Variables|Default|SetDetectDamage? _isa))))))

(event Custom|Infinite
  (bind _niagara (Variables|Default|GetNiagara))
  (bind _returnvalue (Transformation|GetWorldLocation _niagara))
  (Transformation|SetRelativeRotation (Variables|Default|GetMeshGrill) (Math|Rotator|MakeRotator 0.0 0.0 185.0) false false)
  (Components|Activation|SetActive (Variables|Default|GetNiagara) true true)
  (Variables|Default|SetDetectDamage? true)
  (Rendering|Material|SetScalarParameterValueonMaterials (Variables|Default|GetStaticMesh) "EmissiveFire" 1.0)
  (Timeline|InfiniteLoop Play
    (:Update
      (bind _outhit (Collision|SphereTraceByChannel _returnvalue (+ _returnvalue (* (Math|Vector|GetUpVector _niagara) (Variables|OpenVariables|GetDist))) 2e+01 "TraceTypeQuery1" false 0 "ForOneFrame"))
      (bind _asbp_player_test (Utilities|Casting|CastToBP_PlayerTest (.hitactor _outhit)))
      (Default|SetterHP _asbp_player_test 1e+03 false))))

(event EventBeginPlay
  (Utilities|FlowControl|Sequence
    (:then_0
      (if (Variables|OpenVariables|GetIsInfinite)
        (CallFunction|Infinite)
        (else
          (CallFunction|Flames))))
    (:then_1
      (Class|AkGameObject|PostAssociatedAkEvent (Variables|Default|GetAk_FireLoop)))))

(fn ConstructionScript
  (bind _meshgrill (Variables|Default|GetMeshGrill))
  (if (Variables|OpenVariables|GetGrillIsVisible)
    (Rendering|SetVisibility _meshgrill true false)
    (else
      (Rendering|SetVisibility _meshgrill false false))))