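; BP_Push is a looping pusher trap that launches the player along its mesh's forward vector with an upward boost.
; Chained timelines shake the mesh on X as a warning, extend it to a distance-based offset, then retract it.
; Each cycle waits, then advances through a struct array that sets push speed and wait time, wrapping at the end.
; Tick checks the box for player overlap whenever the trap is not reloading.
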(event Custom|EventPush
  (bind _staticmesh (Variables|Default|GetStaticMesh))
  (bind _relativelocation (Variables|/Script/Engine.SceneComponent|GetRelativeLocation _staticmesh))
  (Components|Timeline|SetPlayRate (Variables|Default|GetPush) (.playrate (Utilities|Array|Get(acopy) (Variables|Default|GetTabStruct) (Variables|Default|GetIndex))))
  (Components|Timeline|SetPlayRate (Variables|Default|GetShakes) (/ 1.0 (Variables|Default|GetPlayRateShakes)))
  (Timeline|Shakes PlayFromStart
    (:Update
      (Transformation|SetRelativeLocation _staticmesh (Math|Vector|MakeVector (Math|Random|RandomFloatinRange -1e+01 1e+01) (.y _relativelocation) (.z _relativelocation)) false false))
    (:Finished
      (Variables|Default|SetReloading? false)
      (bind _ratio (Timeline|Push PlayFromStart)
        (:Update
          ;[1 1 1] StartPosition => finishPosition
          (Transformation|SetRelativeLocation (Variables|Default|GetStaticMesh) (Math|Vector|Lerp(Vector) "0, 0, 0" (Variables|Default|GetFinishLocation) _ratio) false false))
        (:Finished
          (Variables|Default|SetReloading? true)
          (bind _ratio_2 (Timeline|Reload PlayFromStart)
            (:Update
              ;[1 1 1] FinishPosition => StartPosition
              (Transformation|SetRelativeLocation (Variables|Default|GetStaticMesh) (Math|Vector|Lerp(Vector) "0, 0, 0" (Variables|Default|GetFinishLocation) _ratio_2) false false))
            (:Finished
              ;[1 1 1] Delay+NextIndex
              (Utilities|FlowControl|Delay (.waittime (Utilities|Array|Get(acopy) (Variables|Default|GetTabStruct) (Variables|Default|GetIndex))))
              (Variables|Default|SetIndex (Math|Integer|SelectInt 0 (+ (Variables|Default|GetIndex) 1) (> (+ (Variables|Default|GetIndex) 1) (Utilities|Array|LastIndex (Variables|Default|GetTabStruct)))))
              (CallFunction|EventPush))))))))

(event EventBeginPlay
  (Variables|Default|SetFinishLocation (* "1.000000, 0, 0" (Variables|Default|GetDistance)))
  (CallFunction|EventPush))

(event EventTick
  (params (DeltaSeconds :type Float%20%28single-precision%29))
  (bind _staticmesh (Variables|Default|GetStaticMesh))
  (bind _power (Variables|Default|Getpower))
  (bind _returnvalue (Math|Vector|GetForwardVector _staticmesh))
  (bind _returnvalue_2 (* _returnvalue _power))
  ;[1 1 1] DetectOverlap
  (if (not (Variables|Default|GetReloading?))
    (if (Collision|IsOverlappingActor (Variables|Default|GetBox) (CallFunction|CastPlayer) :!class /Script/Engine.PrimitiveComponent)
      (Character|LaunchCharacter (CallFunction|CastPlayer) (Math|Vector|MakeVector (.x _returnvalue_2) (.y _returnvalue_2) 5e+02) true true))))

(fn ConstructionScript)