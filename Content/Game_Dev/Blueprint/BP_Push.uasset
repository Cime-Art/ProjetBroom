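; BP_Push is a pusher obstacle that launches the player character.
; A timeline, with no Play input wired, maps its curve to world Y with sweep, pauses at a first-stop time, then resumes at another speed.
; Timeline events reset the stop flag and standard speed.
; Mesh hits launch BP_PlayerTest along the impact normal, only after that stop and while it overlaps the Box.
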(event OnComponentHit(StaticMesh)
  (params (HitComponent :type Primitive%20Component%20Object%20Reference) (OtherActor :type Actor%20Object%20Reference) (OtherComp :type Primitive%20Component%20Object%20Reference) (NormalImpulse :type Vector :default "0, 0, 0") (Hit :type Hit%20Result%20Structure%20%28by%20ref%29))
  ;[1 1 1] Push Si FIRST STOP ET OVERLAP WITH BOX
  (bind _asbp_player_test (Utilities|Casting|CastToBP_PlayerTest OtherActor))
  (if (and (Variables|Default|GetFirstStopPass) (Collision|IsOverlappingActor (Variables|Default|GetBox) _asbp_player_test :!class /Script/Engine.PrimitiveComponent))
    (Character|LaunchCharacter _asbp_player_test (* (.impactnormal Hit) (Variables|Default|GetPushForce)) true true)))

(event EventBeginPlay
  ;[1 1 1] gerer vitesse
  (Components|Timeline|SetPlayRate (Variables|Default|GetTimeline_0) (Variables|Default|GetSpeedStandardOfThePusher)))

(fn ConstructionScript)