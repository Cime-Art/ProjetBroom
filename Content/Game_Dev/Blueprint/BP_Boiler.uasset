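; BP_Boiler is a boiler actor that repeatedly fires a flame Niagara effect on a timed cycle.
; On BeginPlay it plays the Niagara system from the start, waits after it finishes, then calls itself again.
; The wait comes from a Delay array, stepped through by a counter that wraps to zero, producing a looping pattern of intervals between bursts.
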(event Custom|Flames
  (Timeline|NiagaraSystem PlayFromStart
    (:Finished
      (Utilities|FlowControl|Delay (Utilities|Array|Get(acopy) (Variables|OpenVariables|GetDelay) (Variables|Default|GetCount)))
      (Variables|Default|SetCount (Math|Integer|SelectInt 0 (+ (Variables|Default|GetCount) 1) (> (+ (Variables|Default|GetCount) 1) (Utilities|Array|LastIndex (Variables|OpenVariables|GetDelay)))))
      (CallFunction|Flames))))

(event EventBeginPlay
  (CallFunction|Flames))

(fn ConstructionScript)