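; BP_MovingPlatform_Spline is a moving platform actor that carries multiple static meshes along a looping path on a spline.
; The construction script spawns a component for each TabMeshes entry, using its mesh, scale and normalized Space position.
; Each Tick advances every Space by delta time over Speed, making Speed the lap duration, and resets it to zero at the end.
; Only location follows the spline, without sweeping.
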(event EventTick
  (params (DeltaSeconds :type Float%20%28single-precision%29))
  (bind _spline (Variables|Default|GetSpline))
  (bind _tabmeshes (Variables|Default|GetTabMeshes))
  (for (_array_element _array_index) _tabmeshes
    (Utilities|Array|SetArrayElem _tabmeshes _array_index (Utilities|Struct|MakeStruct_MeshesSpaces (.Mesh (Utilities|Struct|BreakStruct_MeshesSpaces _array_element)) (Math|Float|SelectFloat 0.0 (+ (.Space (Utilities|Struct|BreakStruct_MeshesSpaces _array_element)) (* (Utilities|Time|GetWorldDeltaSeconds) (/ 1.0 (Variables|Default|GetSpeed)))) (>= (+ (.Space (Utilities|Struct|BreakStruct_MeshesSpaces _array_element)) (* (Utilities|Time|GetWorldDeltaSeconds) (/ 1.0 (Variables|Default|GetSpeed)))) 1.0)) (.Scale (Utilities|Struct|BreakStruct_MeshesSpaces _array_element))))
    (Transformation|SetWorldLocation (Utilities|Array|Get(acopy) (Variables|Default|GetMeshesComp) _array_index) (Spline|GetLocationatDistanceAlongSpline _spline (* (Spline|GetSplineLength _spline) (.Space (Utilities|Struct|BreakStruct_MeshesSpaces _array_element))) "World") false false)))

(fn ConstructionScript
  (bind _spline (Variables|Default|GetSpline))
  (for _array_element (Variables|Default|GetTabMeshes)
    (bind _returnvalue (AddComponent|AddStaticMeshComponent false (Math|Transform|MakeTransform "0, 0, 0" "0, 0, 0" (.scale _array_element))))
    (Components|StaticMesh|SetStaticMesh _returnvalue (.mesh _array_element))
    (Transformation|SetWorldLocation _returnvalue (Spline|GetLocationatDistanceAlongSpline _spline (* (.space _array_element) (Spline|GetSplineLength _spline)) "World") false false)
    (Utilities|Array|Add (Variables|Default|GetMeshesComp) _returnvalue)))