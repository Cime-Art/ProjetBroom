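; Spline-following actor, named for acid sound, that keeps its Sphere at the point on its spline nearest the player.
; Each Tick it stores and prints the actor-to-player distance, then moves the Sphere to the closest world-space spline location.
; The distance is only printed here, and no audio logic appears in the graphs.
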(event Custom|Get%20distance%20to%20player
  (bind _output_get (Variables|Default|SetDistance%20To%20Player (Transformation|GetDistanceTo (CallFunction|CastPlayer))))
  (Development|PrintString (Utilities|String|ToString(Float) _output_get)))

(event Custom|Move%20Sphere
  (Transformation|SetWorldLocation (Variables|Default|GetSphere) (Spline|FindLocationClosesttoWorldLocation (Variables|Default|GetSpline) (Transformation|GetActorLocation (CallFunction|CastPlayer)) "World") false false))

(event EventBeginPlay)

(event Collision|EventActorBeginOverlap
  (params (OtherActor :type Actor%20Object%20Reference)))

(event EventTick
  (params (DeltaSeconds :type Float%20%28single-precision%29))
  (CallFunction|GetDistancetoPlayer)
  (CallFunction|MoveSphere))

(fn ConstructionScript)