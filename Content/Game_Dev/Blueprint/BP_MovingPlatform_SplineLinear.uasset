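; Moving platform that travels back and forth along a spline at constant speed.
; Tick advances a normalized Space value at a rate of 1/Temps, so Temps is the one-way travel time, and the Descente flag reverses direction at either end.
; Space times spline length sets the mesh's world location without sweep or rotation.
; The construction script applies the chosen Mesh and previews its starting position on the spline.
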(event EventTick
  (params (DeltaSeconds :type Float%20%28single-precision%29))
  (bind _spline (Variables|Default|GetSpline))
  (bind _temps (Variables|OpenVariable|GetTemps))
  (bind _returnvalue (/ 1.0 _temps))
  (bind _returnvalue_2 (* DeltaSeconds _returnvalue))
  (Utilities|FlowControl|Sequence
    (:then_0
      (if (and (>= (Variables|Default|GetSpace) 1.0) (not (Variables|Default|Getdescente)))
        (Variables|Default|Setdescente true)
        (elif (and (<= (Variables|Default|GetSpace) 0.0) (Variables|Default|Getdescente))
          (Variables|Default|Setdescente false))))
    (:then_1
      (if (Variables|Default|Getdescente)
        (Variables|Default|SetSpace (- (Variables|Default|GetSpace) _returnvalue_2))
        (else
          (Variables|Default|SetSpace (+ _returnvalue_2 (Variables|Default|GetSpace))))))
    (:then_2
      (Transformation|SetWorldLocation (Variables|Default|GetStaticMesh) (Spline|GetLocationatDistanceAlongSpline _spline (* (Spline|GetSplineLength _spline) (Variables|Default|GetSpace)) "World") false false))))

(fn ConstructionScript
  (bind _spline (Variables|Default|GetSpline))
  (Components|StaticMesh|SetStaticMesh (Variables|Default|GetStaticMesh) (Variables|OpenVariable|GetMesh))
  (Transformation|SetWorldLocation (Variables|Default|GetStaticMesh) (Spline|GetLocationatDistanceAlongSpline _spline (* (Spline|GetSplineLength _spline) (Variables|Default|GetSpace)) "World") false false))