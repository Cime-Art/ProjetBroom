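; Enemy character Blueprint for the AI trash mob, with a life bar widget and an optional dissolve-and-Niagara spawn that blocks actions and damage.
; Perception of the player alerts its Arena and sets Blackboard flags and walk speed.
; Attack, hit and death events gate movement and message the AnimInstance, while stuns also update the Blackboard.
; Handles puddle immunity, stun-free spike damage, recursive poison ticks, timed immobilization with material swap, and fall death.
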(event OnTargetPerceptionUpdated(AIPerception)
  (params (Actor :type Actor%20Object%20Reference) (Stimulus :type AI%20Stimulus%20Structure))
  ;[1 1 1] Seen?
  (Utilities|Casting|CastToBP_PlayerTest Actor)
  (if (not (Variables|Default|Getisdead))
    (if (not (ScalableFloat|GetValueasBool (AI|GetBlackboard 0) (Utilities|Name|MakeLiteralName "Seen?")))
      (Utilities|IsValid (Variables|OpenVariable|GetArena)
        (:Is%20Valid
          (Default|SetSeen (Variables|OpenVariable|GetArena)))
        (:Is%20Not%20Valid
          _))
      (AI|Components|Blackboard|SetValueasBool (AI|GetBlackboard 0) (Utilities|Name|MakeLiteralName "Seen?") true)
      (Variables|/Script/Engine.CharacterMovementComponent|SetMaxWalkSpeed (Variables|Character|GetCharacterMovement) (Variables|OpenVariable|GetSpeed)))))

(event Custom|StartBigAttack
  ;[1 1 1] BigAttack
  (if (Math|Boolean|ANDBoolean (not (Variables|Default|GetIsHit?)) (not (Variables|Default|Getisdead)) (not (Variables|Default|GetIsBigAttacking?)) (not (Variables|Default|GetSpawned?)))
    (CallFunction|CanMove false true)
    (Class|INTAnimBpIA|BigAttack(Message) (Components|SkeletalMesh|GetAnimInstance (Variables|Character|GetMesh)))
    (Variables|Default|SetIsBigAttacking? true)
    (Variables|Utilities|SetHit%20Player%20? false)))

(event Custom|TakeDamage
  (params (Degats :type Float%20%28single-precision%29) (IsTraps :type Boolean))
  ;[1 1 1] Mort
  (if (not (or (Variables|Default|Getisdead) (Variables|Default|GetSpawned?)))
    (Rendering|SetVisibility (Variables|Default|GetWidget) true false)
    (bind _output_get (Variables|Default|SetCurrentHp (- (Variables|Default|GetCurrentHp) Degats)))
    (if (<= _output_get 0.0)
      (Class|Pawn|DetachfromControllerPendingDestroy)
      (Collision|SetCollisionProfileName (Variables|Collision|GetCapsuleComponent) "NoCollision" true :!class /Script/Engine.PrimitiveComponent)
      (CallFunction|CanMove false false)
      (Variables|Default|Setisdead true)
      (Class|INTAnimBpIA|Death(Message) (Components|SkeletalMesh|GetAnimInstance (Variables|Character|GetMesh)))
      (Utilities|FlowControl|DoOnce false
        (:Completed
          (Default|RemoveMobs (Variables|OpenVariable|GetArena))))
      (elif (not (or (Variables|Default|GetIsHit?) IsTraps))
        (Variables|Default|SetIsHit? true)
        (bind _output_get_2 (Variables|Default|SetStunned? true))
        (AI|Components|Blackboard|SetValueasBool (AI|GetBlackboard 0) (Utilities|Name|MakeLiteralName "Stunned?") _output_get_2)
        (CallFunction|CanMove false false)
        (Class|INTAnimBpIA|GetHit(Message) (Components|SkeletalMesh|GetAnimInstance (Variables|Character|GetMesh)))))))

(event Custom|EndHit
  ;[1 1 1] EndHit
  (Variables|Default|SetIsAttacking? false)
  (Variables|Default|SetIsBigAttacking? false)
  (Variables|Default|SetIsHit? false)
  (if (not (Variables|Default|GetStunned?))
    (CallFunction|CanMove true true)
    (bind _output_get (Variables|Default|SetStunned? false))
    (AI|Components|Blackboard|SetValueasBool (AI|GetBlackboard 0) (Utilities|Name|MakeLiteralName "Stunned?") _output_get)))

(event Custom|Fall
  ;[1 1 1] Mort
  ;;[1 1 1] Chute
  (if (not (Variables|Default|Getisdead))
    (Variables|Default|SetCurrentHp 0.0)
    (Class|Pawn|DetachfromControllerPendingDestroy)
    (CallFunction|CanMove false false)
    (Variables|Default|Setisdead true)
    (Actor|DestroyActor)))

(event Custom|CanMove
  (params (canMove? :type Boolean) (canRotate? :type Boolean))
  (bind _charactermovement (Variables|Character|GetCharacterMovement))
  ;[1 1 1] Can Move
  (if canMove?
    (Pawn|Components|CharacterMovement|SetMovementMode _charactermovement "MOVE_Walking" 0)
    (elif canRotate?
      (Pawn|Components|CharacterMovement|SetMovementMode _charactermovement "MOVE_Custom" 0)
      (else
        (Pawn|Components|CharacterMovement|DisableMovement _charactermovement)))))

(event Custom|IsImmo
  (params (TimeImmo :type Float%20%28single-precision%29) (Damage :type Float%20%28single-precision%29))
  (bind _mesh (Variables|Character|GetMesh))
  ;[1 1 1] Immobilisation
  (if (not (or (Variables|Default|Getisdead) (Variables|Default|GetSpawned?)))
    (Variables|Default|SetMaterialBody (Rendering|Material|GetMaterial _mesh 0))
    (Rendering|Material|SetMaterial _mesh 0 "/Game/Game_Dev/Material/M_SpellImmo_Inst.M_SpellImmo_Inst")
    (bind _output_get (Variables|Default|SetStunned? true))
    (AI|Components|Blackboard|SetValueasBool (AI|GetBlackboard 0) (Utilities|Name|MakeLiteralName "Stunned?") _output_get)
    (CallFunction|CanMove false false)
    (Utilities|FlowControl|Delay TimeImmo)
    (if (not (Variables|Default|Getisdead))
      (bind _output_get_2 (Variables|Default|SetStunned? false))
      (CallFunction|CanMove true true)
      (Rendering|Material|SetMaterial (Variables|Character|GetMesh) 0 (Variables|Default|GetMaterialBody))
      (AI|Components|Blackboard|SetValueasBool (AI|GetBlackboard 0) (Utilities|Name|MakeLiteralName "Stunned?") _output_get_2))))

(event Custom|StartAttack
  ;[1 1 1] StartAttack
  (if (Math|Boolean|ANDBoolean (not (Variables|Default|GetIsHit?)) (not (Variables|Default|Getisdead)) (not (Variables|Default|GetIsAttacking?)) (not (Variables|Default|GetSpawned?)))
    (CallFunction|CanMove false false)
    (Class|INTAnimBpIA|Attack(Message) (Components|SkeletalMesh|GetAnimInstance (Variables|Character|GetMesh)))
    (Variables|Default|SetIsAttacking? true)
    (Variables|Utilities|SetHit%20Player%20? false)))

(event Custom|PoisonDamage
  (params (Degats :type Float%20%28single-precision%29) (Count :type Integer))
  ;[1 1 1] Poison Damage
  (if (not (or (Variables|Default|Getisdead) (Variables|Default|GetSpawned?)))
    (if (> Count 0)
      (bind _result (Math|Integer|DecrementInt Count)
        (:%20%20
          (Game|Damage|ApplyDamage self Degats 0 0)
          (if (<= (Variables|Default|GetCurrentHp) 0.0)
            (Class|Pawn|DetachfromControllerPendingDestroy)
            (CallFunction|CanMove false false)
            (Variables|Default|Setisdead true)
            (Class|INTAnimBpIA|Death(Message) (Components|SkeletalMesh|GetAnimInstance (Variables|Character|GetMesh)))
            (else
              (Utilities|FlowControl|Delay 1.0)
              (CallFunction|PoisonDamage Degats _result))))))))

(event Custom|Set%20Seen
  ;[1 1 1] Seen?
  (AI|Components|Blackboard|SetValueasBool (AI|GetBlackboard 0) (Utilities|Name|MakeLiteralName "Seen?") true)
  (Variables|/Script/Engine.CharacterMovementComponent|SetMaxWalkSpeed (Variables|Character|GetCharacterMovement) (Variables|OpenVariable|GetSpeed)))

(event Game|Damage|EventAnyDamage
  (params (Damage :type Float%20%28single-precision%29) (DamageType :type Damage%20Type%20Object%20Reference) (InstigatedBy :type Controller%20Object%20Reference) (DamageCauser :type Actor%20Object%20Reference))
  (bind _returnvalue (Utilities|GetClass DamageCauser))
  ;[1 1 1] Mort
  (if (not (== _returnvalue "/Game/Game_Dev/Blueprint/IA/Trashmob/Blueprints/BP_Puddle.BP_Puddle_C"))
    (CallFunction|TakeDamage Damage (== _returnvalue "/Game/Game_Dev/Blueprint/Trap/BP_Spike.BP_Spike_C"))))

(event EventBeginPlay
  (bind _niagara (Variables|Default|GetNiagara))
  ;[1 1 1] Widget Barre de vie
  (Variables|/Game/Game_Dev/Blueprint/Widget/LifesBar/WG_EnemyLife.WG_EnemyLife_C|SetTrashmob_ref (.AsWG%20Enemy%20Life (Utilities|Casting|CastToWG_EnemyLife (UserInterface|GetUserWidgetObject (Variables|Default|GetWidget)))) self)
  (if (Variables|Default|GetSpawned?)
    (CallFunction|CanMove false false)
    (Class|NiagaraComponent|SetAsset _niagara (Variables|OpenVariable|GetNiagaraSystem))
    (Niagara|ResetSystem _niagara)
    (bind _newtrack_0 (Timeline|Dissolve PlayFromStart)
      (:Update
        (Rendering|Material|SetScalarParameterValueonMaterials (Variables|Character|GetMesh) "Dissolve" _newtrack_0))
      (:Finished
        (CallFunction|CanMove true true)
        (Variables|Default|SetSpawned? false)
        (if (Variables|Default|GetSpawnSeen)
          (CallFunction|SetSeen))))
    (else
      (Components|Activation|SetActive (Variables|Default|GetNiagara) false false))))

(fn ConstructionScript)