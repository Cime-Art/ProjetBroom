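; Alambic trash mob enemy, a child Blueprint that attacks by dropping a puddle.
; On BeginPlay it switches its trashmob AI controller to the Alambic behavior tree.
; When not hit, dead or already attacking, StartAttack locks movement and rotation, notifies the anim instance and flags the attack.
; It then spawns a puddle actor at its own location, passing along its damage value.
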(event Custom|AttackAlambic
  (Game|SpawnActorfromClass "/Game/Game_Dev/Blueprint/IA/Trashmob/Blueprints/BP_Puddle.BP_Puddle_C" (Math|Transform|MakeTransform (Transformation|GetActorLocation) "0, 0, 0" "1,1,1") "Undefined" 0 (Variables|Default|GetDamage) 0))

(event EventBeginPlay
  (|CallParentFunction)
  (Default|ChangeBehaviorTree (.AsIA%20Controller%20Trashmob (Utilities|Casting|CastToIA_Controller_Trashmob (AI|GetAIController self))) "/Game/Game_Dev/Blueprint/IA/Trashmob/BehaviorTree_Blackboard/BT_IA_Alambic.BT_IA_Alambic"))

(event Collision|EventActorBeginOverlap
  (params (OtherActor :type Actor%20Object%20Reference)))

(event EventTick
  (params (DeltaSeconds :type Float%20%28single-precision%29))
  (|CallParentFunction DeltaSeconds) ; This node is disabled and will not be called.\nDrag off pins to build functionality.
)

(event EventStartAttack
  (if (Math|Boolean|ANDBoolean (not (Variables|Default|GetIsHit?)) (not (Variables|Default|Getisdead)) (not (Variables|Default|GetIsAttacking?)))
    (CallFunction|CanMove false false)
    (Class|INTAnimBpIA|Attack(Message) (Components|SkeletalMesh|GetAnimInstance (Variables|Character|GetMesh)))
    (Variables|Default|SetIsAttacking? true)
    (CallFunction|AttackAlambic)))

(fn ConstructionScript
  (|CallParentFunction))