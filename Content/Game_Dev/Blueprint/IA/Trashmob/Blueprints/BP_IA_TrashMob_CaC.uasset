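; Melee trash mob enemy that switches its AI controller to the BT_IA_CAC behavior tree on BeginPlay.
; Construction attaches a weapon component and randomly adds socketed gear from StuffToAdd, with a random small or big shield.
; If Spawned, a timeline drives the gear's Dissolve parameter.
; IsImmo stuns living, non-Spawned mobs for a given time via blackboard, movement lock and material swap, reverting unless dead.
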(event EventBeginPlay
  (|CallParentFunction)
  (Default|ChangeBehaviorTree (.AsIA%20Controller%20Trashmob (Utilities|Casting|CastToIA_Controller_Trashmob (AI|GetAIController self))) "/Game/Game_Dev/Blueprint/IA/Trashmob/BehaviorTree_Blackboard/BT_IA_CAC.BT_IA_CAC")
  (if (Variables|Default|GetSpawned?)
    (bind _newtrack_0 (Timeline|Timeline_0 PlayFromStart)
      (:Update
        (for _array_element (Variables|Default|GetStuff)
          (Rendering|Material|SetScalarParameterValueonMaterials _array_element "Dissolve" _newtrack_0))))))

(event Collision|EventActorBeginOverlap
  (params (OtherActor :type Actor%20Object%20Reference)))

(event EventTick
  (params (DeltaSeconds :type Float%20%28single-precision%29))
  (|CallParentFunction DeltaSeconds) ; This node is disabled and will not be called.\nDrag off pins to build functionality.
)

(event EventIsImmo
  (params (TimeImmo :type Float%20%28single-precision%29) (Damage :type Float%20%28single-precision%29))
  (bind _mesh (Variables|Character|GetMesh))
  (if (not (or (Variables|Default|Getisdead) (Variables|Default|GetSpawned?)))
    (Variables|Default|SetMaterialBody (Rendering|Material|GetMaterial _mesh 0))
    (for _array_element (Variables|Default|GetStuff)
      (Utilities|Array|Add (Variables|Default|GetStuffMaterial) (Rendering|Material|GetMaterial _array_element 0)))
    (Rendering|Material|SetMaterial _mesh 0 "/Game/Game_Dev/Material/M_SpellImmo_Inst.M_SpellImmo_Inst")
    (for _array_element_2 (Variables|Default|GetStuff)
      (Rendering|Material|SetMaterial _array_element_2 0 "/Game/Game_Dev/Material/M_SpellImmo_Inst.M_SpellImmo_Inst"))
    (Variables|Default|SetStunned? true)
    (AI|Components|Blackboard|SetValueasBool (AI|GetBlackboard 0) (Utilities|Name|MakeLiteralName "Stunned?") true)
    (CallFunction|CanMove false false)
    (Utilities|FlowControl|Delay TimeImmo)
    (if (not (Variables|Default|Getisdead))
      (Variables|Default|SetStunned? false)
      (CallFunction|CanMove true true)
      (Rendering|Material|SetMaterial (Variables|Character|GetMesh) 0 (Variables|Default|GetMaterialBody))
      (for (_array_element_3 _array_index) (Variables|Default|GetStuff)
        (Rendering|Material|SetMaterial _array_element_3 0 (Utilities|Array|Get(acopy) (Variables|Default|GetStuffMaterial) _array_index)))
      (AI|Components|Blackboard|SetValueasBool (AI|GetBlackboard 0) (Utilities|Name|MakeLiteralName "Stunned?") false))))

(fn ConstructionScript
  (bind _returnvalue (Math|Random|RandomFloat))
  (bind _stufftoadd (Variables|Default|GetStuffToAdd))
  (|CallParentFunction)
  (Utilities|Array|Clear (Variables|Default|GetStuff))
  (bind _returnvalue_2 (AddComponent|AddStaticMeshComponent false))
  (Transformation|AttachComponentToComponent _returnvalue_2 (Variables|Character|GetMesh) "Weapon" "KeepRelative" "KeepRelative" "KeepRelative" true)
  (Collision|SetCollisionEnabled _returnvalue_2 "NoCollision")
  (Utilities|Array|AddUnique (Variables|Default|GetStuff) _returnvalue_2)
  (bind _keys (Utilities|Map|Keys _stufftoadd))
  ;[1 1 1] Stuff
  (bind _values (Utilities|Map|Values _stufftoadd))
  (for (_array_element _array_index) _values
    (if (<= _returnvalue 0.5)
      (bind _returnvalue_3 (AddComponent|AddStaticMeshComponent false))
      (Components|StaticMesh|SetStaticMesh _returnvalue_3 (select (Utilities|Name|Equal(Name) (Utilities|Array|Get(acopy) _keys _array_index) "Shield") (select (<= _returnvalue 0.5) "/Game/Game_ART/Graph/Objects/Jail/Weapons_Skeleton/mesh_little_shield.mesh_little_shield" "/Game/Game_ART/Graph/Objects/Jail/Weapons_Skeleton/mesh_big_shield.mesh_big_shield") _array_element))
      (Utilities|Array|AddUnique (Variables|Default|GetStuff) _returnvalue_3)
      (Transformation|AttachComponentToComponent _returnvalue_3 (Variables|Character|GetMesh) (Utilities|Array|Get(acopy) _keys _array_index) "KeepRelative" "KeepRelative" "KeepRelative" true)
      (Collision|SetCollisionEnabled _returnvalue_3 "NoCollision"))))