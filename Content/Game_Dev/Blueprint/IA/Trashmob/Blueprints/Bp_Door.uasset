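; Door actor for the trashmob AI area that starts open, with collision off and its Y and Z scale shrunk to zero.
; Close_Door plays the Material timeline to grow the mesh back to its saved scale, and OpenDoor reverses it.
; When the timeline finishes, the Lock flag decides collision: enabled after closing, disabled after opening.
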(event Custom|Close_Door
  (bind _door (Variables|Default|GetDoor))
  (Variables|Default|SetLock false)
  (bind _scaling (Timeline|Material PlayFromStart)
    (:Update
      (Transformation|SetRelativeScale3D _door (Math|Vector|MakeVector (.x (Variables|/Script/Engine.SceneComponent|GetRelativeScale3D _door)) (Math|Float|MapRangeClamped _scaling 0.0 1.0 0.0 (Variables|Default|GetPreview%20Y)) (Math|Float|MapRangeClamped _scaling 0.0 1.0 0.0 (Variables|Default|GetPreview%20Z)))))
    (:Finished
      (if (Variables|Default|GetLock)
        (Collision|SetCollisionEnabled (Variables|Default|GetDoor) "NoCollision")
        (else
          (Collision|SetCollisionEnabled (Variables|Default|GetDoor) "QueryAndPhysics"))))))

(event Custom|Open%20Door
  (bind _door (Variables|Default|GetDoor))
  (Variables|Default|SetLock true)
  (bind _scaling (Timeline|Material ReverseFromEnd)
    (:Update
      (Transformation|SetRelativeScale3D _door (Math|Vector|MakeVector (.x (Variables|/Script/Engine.SceneComponent|GetRelativeScale3D _door)) (Math|Float|MapRangeClamped _scaling 0.0 1.0 0.0 (Variables|Default|GetPreview%20Y)) (Math|Float|MapRangeClamped _scaling 0.0 1.0 0.0 (Variables|Default|GetPreview%20Z)))))
    (:Finished
      (if (Variables|Default|GetLock)
        (Collision|SetCollisionEnabled (Variables|Default|GetDoor) "NoCollision")
        (else
          (Collision|SetCollisionEnabled (Variables|Default|GetDoor) "QueryAndPhysics"))))))

(event EventBeginPlay
  (bind _door (Variables|Default|GetDoor))
  (bind _relativescale3d (Variables|/Script/Engine.SceneComponent|GetRelativeScale3D _door))
  (Collision|SetCollisionEnabled _door "NoCollision")
  (Variables|Default|SetPreview%20Y (.y _relativescale3d))
  (Variables|Default|SetPreview%20Z (.z _relativescale3d))
  (Transformation|SetRelativeScale3D _door (Math|Vector|MakeVector (.x _relativescale3d) 0.0 0.0)))

(fn ConstructionScript)