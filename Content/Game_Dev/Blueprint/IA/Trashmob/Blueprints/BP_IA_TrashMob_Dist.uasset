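; Ranged trash mob enemy that switches its AI controller to the BT_IA_Dist behavior tree on BeginPlay.
; The construction script attaches collisionless hood, gloves, boots and crossbow meshes to skeletal sockets.
; If spawned, a timeline drives their Dissolve material parameter, posting a Wwise idle event inside that update loop when the Seen? blackboard key is true.
; Tick sets the Fuite (flee) flag while the player is close.
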(event EventBeginPlay
  (|CallParentFunction)
  (Default|ChangeBehaviorTree (.AsIA%20Controller%20Trashmob (Utilities|Casting|CastToIA_Controller_Trashmob (AI|GetAIController self))) "/Game/Game_Dev/Blueprint/IA/Trashmob/BehaviorTree_Blackboard/BT_IA_Dist.BT_IA_Dist")
  (if (Variables|Default|GetSpawned?)
    (bind _newtrack_0 (Timeline|Timeline_0 PlayFromStart)
      (:Update
        (for _array_element (Variables|Default|GetStuff)
          (Rendering|Material|SetScalarParameterValueonMaterials _array_element "Dissolve" _newtrack_0)
          (if (ScalableFloat|GetValueasBool (AI|GetBlackboard 0) (Utilities|Name|MakeLiteralName "Seen?"))
            (Class|AkGameplayStatics|PostEvent "/Game/WwiseAudio/Events/Default_Work_Unit/Mob/SkeletonDist/Event_SkDist_Idle.Event_SkDist_Idle" self)))))))

(event EventTick
  (params (DeltaSeconds :type Float%20%28single-precision%29))
  (|CallParentFunction DeltaSeconds)
  (if (<= (Transformation|GetDistanceTo (Game|GetPlayerCharacter 0)) 4.5e+02)
    (Variables|Default|SetFuite? true)
    (else
      (Variables|Default|SetFuite? false))))

(event Collision|EventActorBeginOverlap
  (params (OtherActor :type Actor%20Object%20Reference)))

(fn ConstructionScript
  (|CallParentFunction)
  ;[1 1 1] Stuff
  (for _index (range 0 (Variables|Default|GetNbAsset))
    (bind _returnvalue (AddComponent|AddStaticMeshComponent false))
    (Components|StaticMesh|SetStaticMesh _returnvalue (Utilities|Select :Index _index :Option%200 "/Game/Game_ART/Graph/Objects/Jail/Stuff_Skeleton/SM_Hood.SM_Hood" :Option%201 "/Game/Game_ART/Graph/Objects/Jail/Stuff_Skeleton/SM_Glove.SM_Glove" :Option%202 "/Game/Game_ART/Graph/Objects/Jail/Stuff_Skeleton/SM_Glove.SM_Glove" :Option%203 "/Game/Game_ART/Graph/Objects/Jail/Stuff_Skeleton/SM_Boot_L.SM_Boot_L" :Option%204 "/Game/Game_ART/Graph/Objects/Jail/Stuff_Skeleton/SM_Boot_R_01.SM_Boot_R_01" :Option%205 "/Game/Game_ART/Graph/Objects/Jail/Weapons_Skeleton/mesh_crossbow.mesh_crossbow"))
    (Utilities|Array|AddUnique (Variables|Default|GetStuff) _returnvalue)
    (Collision|SetCollisionEnabled _returnvalue "NoCollision")
    (Transformation|AttachComponentToComponent _returnvalue (Variables|Character|GetMesh) (Utilities|Select :Index _index :Option%200 "Hat" :Option%201 "Left_Glove" :Option%202 "Right_Glove" :Option%203 "L_Boot" :Option%204 "R_Boot" :Option%205 "Weapon_Crossbow") "KeepRelative" "KeepRelative" "KeepRelative" true)))