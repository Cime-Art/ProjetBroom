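; BP_Arena is a combat arena volume that locks the player in with linked doors until no trash mobs remain inside.
; The construction script creates a sphere or box collision.
; On the first player overlap it counts BP_IA_TrashMob actors and closes the doors if any exist; capsule exits decrement the count, reopening them at zero.
; SetSeen alerts contained mobs by restoring their walk speed, setting the "Seen?" blackboard key and refreshing the count.
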(event OnComponentBeginOverlap(Collision)
  (params (OverlappedComponent :type Primitive%20Component%20Object%20Reference) (OtherActor :type Actor%20Object%20Reference) (OtherComp :type Primitive%20Component%20Object%20Reference) (OtherBodyIndex :type Integer) (bFromSweep :type Boolean) (SweepResult :type Hit%20Result%20Structure%20%28by%20ref%29))
  (Utilities|Casting|CastToBP_PlayerTest OtherActor)
  (Variables|Default|SetNbMobs (Utilities|Array|Length (Collision|GetOverlappingActors (Variables|Default|GetCollision) "/Game/Game_Dev/Blueprint/IA/Trashmob/Blueprints/BP_IA_TrashMob.BP_IA_TrashMob_C" :!class /Script/Engine.PrimitiveComponent)))
  (Utilities|FlowControl|DoOnce false
    (:Completed
      (if (> (Variables|Default|GetNbMobs) 0)
        (for _array_element (Variables|Default|GetBp_Door)
          (Default|CloseDoor _array_element))))))

(event OnComponentEndOverlap(Collision)
  (params (OverlappedComponent :type Primitive%20Component%20Object%20Reference) (OtherActor :type Actor%20Object%20Reference) (OtherComp :type Primitive%20Component%20Object%20Reference) (OtherBodyIndex :type Integer))
  (Utilities|Casting|CastToBP_IA_TrashMob OtherActor)
  (Utilities|Casting|CastToCapsuleComponent OtherComp)
  (Math|Integer|DecrementInt (Variables|Default|GetNbMobs)
    (:%20%20
      (if (== (Variables|Default|GetNbMobs) 0)
        (for _array_element (Variables|Default|GetBp_Door)
          (Default|OpenDoor _array_element))))))

(event Custom|SetSeen
  (bind _collision (Variables|Default|GetCollision))
  (bind _overlappingactors (Collision|GetOverlappingActors _collision "/Game/Game_Dev/Blueprint/IA/Trashmob/Blueprints/BP_IA_TrashMob.BP_IA_TrashMob_C" :!class /Script/Engine.PrimitiveComponent))
  (for _array_element _overlappingactors
    (bind _asbp_ia_trash_mob (Utilities|Casting|CastToBP_IA_TrashMob _array_element))
    (Utilities|IsValid (AI|GetBlackboard _array_element)
      (:Is%20Valid
        (Variables|/Script/Engine.CharacterMovementComponent|SetMaxWalkSpeed (Variables|/Script/Engine.Character|GetCharacterMovement _asbp_ia_trash_mob) (Variables|/Game/Game_Dev/Blueprint/IA/Trashmob/Blueprints/BP_IA_TrashMob.BP_IA_TrashMob_C|GetSpeed _asbp_ia_trash_mob))
        (AI|Components|Blackboard|SetValueasBool (AI|GetBlackboard _array_element) (Utilities|Name|MakeLiteralName "Seen?") true))))
  (Variables|Default|SetNbMobs (Utilities|Array|Length _overlappingactors)))

(fn ConstructionScript
  (if (Variables|OpenVariable|GetSphere?)
    (bind _returnvalue (AddComponent|AddSphereComponent false (Math|Transform|MakeTransform "0, 0, 0" "0, 0, 0" "10.000000,10.000000,10.000000")))
    (Variables|Default|SetCollision _returnvalue)
    (else
      (bind _returnvalue_2 (AddComponent|AddBoxComponent false (Math|Transform|MakeTransform "0, 0, 0" "0, 0, 0" "10.000000,10.000000,10.000000")))
      (Variables|Default|SetCollision _returnvalue_2))))