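; Fireball projectile actor that damages the player character on contact.
; ActivatePhysics adds and stores a projectile movement component at runtime, then sets the FireBall component to query-only collision that overlaps Pawns.
; On overlap with BP_PlayerTest, a DoOnce gate applies the Damage value a single time and destroys the fireball.
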(event OnComponentBeginOverlap(FireBall)
  (params (OverlappedComponent :type Primitive%20Component%20Object%20Reference) (OtherActor :type Actor%20Object%20Reference) (OtherComp :type Primitive%20Component%20Object%20Reference) (OtherBodyIndex :type Integer) (bFromSweep :type Boolean) (SweepResult :type Hit%20Result%20Structure%20%28by%20ref%29))
  (bind _asbp_player_test (Utilities|Casting|CastToBP_PlayerTest OtherActor))
  (Utilities|FlowControl|DoOnce false
    (:Completed
      (Game|Damage|ApplyDamage _asbp_player_test (Variables|Default|GetDamage) 0 0)
      (Actor|DestroyActor self))))

(event Custom|ActivatePhysics
  (bind _fireball (Variables|Default|GetFireBall))
  (bind _returnvalue (AddComponent|AddProjectileMovementComponent))
  (Variables|Default|SetProjectile%20Ref _returnvalue)
  (Collision|SetCollisionEnabled _fireball "QueryOnly")
  (Collision|SetCollisionResponsetoChannel _fireball "ECC_Pawn" "ECR_Overlap"))

(fn ConstructionScript)