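; General enemy AI character with three variants (Tete De Feu, Entier, Fusion), each getting its own anim blueprint and walk speed at construction.
; On BeginPlay it has its AI controller switch to that variant's behavior tree and fills its HP.
; Three guarded attacks lock movement but allow rotation, then message the anim instance.
; A stun freezes it for three seconds through a blackboard flag, recovering unless dead.
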(event Custom|StartAttack_1
  (if (not (Variables|Default|GetIsAttacking_1))
    (CallFunction|CanMove false true)
    (Class|INTAnimBpIA|AttackGeneral1(Message) (Components|SkeletalMesh|GetAnimInstance (Variables|Character|GetMesh)))
    (Variables|Default|SetIsAttacking_1 true)
    (Variables|Utilities|SetHit%20Player%20?_0 false)))

(event Custom|Stunned
  (Variables|Default|SetStunned?_0 true)
  (AI|Components|Blackboard|SetValueasBool (AI|GetBlackboard 0) (Utilities|Name|MakeLiteralName "Stunned_General") true)
  (CallFunction|CanMove false false)
  (Utilities|FlowControl|Delay 3.0)
  (if (not (Variables|Default|Getisdead))
    (Variables|Default|SetStunned?_0 false)
    (CallFunction|CanMove true true)
    (AI|Components|Blackboard|SetValueasBool (AI|GetBlackboard 0) (Utilities|Name|MakeLiteralName "Stunned_General") false)))

(event Custom|CanMove
  (params (canMove? :type Boolean) (canRotate? :type Boolean))
  (bind _charactermovement (Variables|Character|GetCharacterMovement))
  (Variables|Default|SetCanMoveGeneral canMove?)
  (Variables|Default|SetCanRotateGeneral canRotate?)
  (if canMove?
    (Pawn|Components|CharacterMovement|SetMovementMode _charactermovement "MOVE_Walking" 0)
    (elif canRotate?
      (Pawn|Components|CharacterMovement|SetMovementMode _charactermovement "MOVE_Custom" 0)
      (else
        (Pawn|Components|CharacterMovement|DisableMovement _charactermovement)))))

(event Custom|StartAttack_2
  (if (not (Variables|Default|GetIsAttacking_2))
    (CallFunction|CanMove false true)
    (Class|INTAnimBpIA|AttackGeneral2(Message) (Components|SkeletalMesh|GetAnimInstance (Variables|Character|GetMesh)))
    (Variables|Default|SetIsAttacking_2 true)
    (Variables|Utilities|SetHit%20Player%20?_0 false)))

(event Custom|StartAttack_3
  (if (not (Variables|Default|GetIsAttacking_3))
    (CallFunction|CanMove false true)
    (Class|INTAnimBpIA|AttackGeneral3(Message) (Components|SkeletalMesh|GetAnimInstance (Variables|Character|GetMesh)))
    (Variables|Default|SetIsAttacking_3 true)
    (Variables|Utilities|SetHit%20Player%20?_0 false)))

(event EventBeginPlay
  (|CallParentFunction)
  (Default|ChangeBehaviorTree (.AsIA%20Controller%20Generals (Utilities|Casting|CastToIA_Controller_Generals (AI|GetAIController self))) (Variables|Default|GetIA_Type_Generals))
  (Variables|Default|SetCurrentHp (Variables|Default|GetMaxHp)))

(fn ConstructionScript
  (switch Utilities|FlowControl|Switch|SwitchonIA_Types_Generals (Variables|Default|GetIA_Type_Generals)
    (:NewEnumerator0
      (Variables|Default|SetRadiusExplo 3e+02)
      (Variables|/Script/Engine.CharacterMovementComponent|SetMaxWalkSpeed (Variables|Character|GetCharacterMovement) 5e+02)
      (Class|SkeletalMeshComponent|SetAnimClass (Variables|Character|GetMesh) "/Game/Game_Dev/Blueprint/IA/Generals/AnimBP_TeteDeFeu.AnimBP_TeteDeFeu_C"))
    (:NewEnumerator1
      (Variables|Default|SetRadiusExplo 3e+02)
      (Variables|/Script/Engine.CharacterMovementComponent|SetMaxWalkSpeed (Variables|Character|GetCharacterMovement) 2e+02)
      (Class|SkeletalMeshComponent|SetAnimClass (Variables|Character|GetMesh) "/Game/Game_Dev/Blueprint/IA/Generals/AnimBP_FullBody.AnimBP_FullBody_C"))
    (:NewEnumerator2
      (Variables|Default|SetRadiusExplo 3e+02)
      (Variables|/Script/Engine.CharacterMovementComponent|SetMaxWalkSpeed (Variables|Character|GetCharacterMovement) 2e+02)
      (Class|SkeletalMeshComponent|SetAnimClass (Variables|Character|GetMesh) "/Game/Game_Dev/Blueprint/IA/Generals/AnimBP_Fusion.AnimBP_Fusion_C"))))