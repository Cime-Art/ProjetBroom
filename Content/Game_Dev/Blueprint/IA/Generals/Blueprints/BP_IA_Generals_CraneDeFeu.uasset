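; AI Blueprint for the Crâne de Feu (fire skull) general, an enemy with health-triggered fire waves.
; On BeginPlay it switches the generals controller's behavior tree and writes the map centre to the blackboard.
; Tick checks health, setting the FireWave blackboard flag once at each quarter-health threshold.
; Capsule hits during Attack1 damage the player through a DoOnce, re-armed by a hit outside the attack.
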(event OnComponentHit(CapsuleComponent)
  (params (HitComponent :type Primitive%20Component%20Object%20Reference) (OtherActor :type Actor%20Object%20Reference) (OtherComp :type Primitive%20Component%20Object%20Reference) (NormalImpulse :type Vector :default "0, 0, 0") (Hit :type Hit%20Result%20Structure%20%28by%20ref%29))
  (if (Variables|Default|GetIsAttacking_1)
    (Utilities|FlowControl|DoOnce false :!label _label
      (:Completed
        (bind _asbp_player_test (Utilities|Casting|CastToBP_PlayerTest OtherActor))
        (Game|Damage|ApplyDamage _asbp_player_test 35.0 0 0)))
    (else
      (goto _label Reset))))

(event Custom|Condition%20Fire%20Wave
  (bind _maxhp (Variables|Default|GetMaxHp))
  (bind _currenthp (Variables|Default|GetCurrentHp))
  ;[1 1 1] Condition Fire Wave
  (Utilities|FlowControl|Sequence
    (:then_0
      (if (<= _currenthp (* _maxhp 0.75))
        (Utilities|FlowControl|DoOnce false
          (:Completed
            (bind _output_get (Variables|Default|SetFireWave true :!label _label))
            (AI|Components|Blackboard|SetValueasBool (AI|GetBlackboard 0) (Utilities|Name|MakeLiteralName "FireWave") _output_get)))))
    (:then_1
      (if (<= _currenthp (* _maxhp 0.5))
        (Utilities|FlowControl|DoOnce false
          (:Completed
            (goto _label)))))
    (:then_2
      (if (<= _currenthp (* _maxhp 0.25))
        (Utilities|FlowControl|DoOnce false
          (:Completed
            (goto _label)))))))

(event EventBeginPlay
  (|CallParentFunction)
  (Default|ChangeBehaviorTree (.AsIA%20Controller%20Generals (Utilities|Casting|CastToIA_Controller_Generals (AI|GetAIController self))) "NewEnumerator0")
  (AI|Components|Blackboard|SetValueasVector (AI|GetBlackboard 0) (Utilities|Name|MakeLiteralName "CentreMap") (Variables|Default|GetCentreMap)))

(event EventTick
  (params (DeltaSeconds :type Float%20%28single-precision%29))
  (|CallParentFunction DeltaSeconds)
  (CallFunction|ConditionFireWave))

(fn ConstructionScript
  (|CallParentFunction))