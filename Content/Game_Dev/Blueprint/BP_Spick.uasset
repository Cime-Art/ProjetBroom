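; BP_Spick is a spike trap that raises and lowers a configurable mesh to damage the player.
; The Spike timeline drives the mesh height, either looping with waits cycled from a Delay array or playing when BP_PlayerTest enters the Box.
; Timeline event tracks toggle the active state and reset a DoOnce.
; While active, Tick checks mesh overlap with the player and applies damage through that DoOnce, limiting repeat hits.
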(event OnComponentBeginOverlap(Box)
  (params (OverlappedComponent :type Primitive%20Component%20Object%20Reference) (OtherActor :type Actor%20Object%20Reference) (OtherComp :type Primitive%20Component%20Object%20Reference) (OtherBodyIndex :type Integer) (bFromSweep :type Boolean) (SweepResult :type Hit%20Result%20Structure%20%28by%20ref%29))
  (bind _staticmesh (Variables|Default|GetStaticMesh))
  (bind _relativelocation (Variables|/Script/Engine.SceneComponent|GetRelativeLocation _staticmesh))
  (Utilities|Casting|CastToBP_PlayerTest OtherActor)
  (if (not (Variables|OpenVariables|GetIsInfinite))
    (bind _movement (Timeline|Spike PlayFromStart)
      (:Update
        ;[1 1 1] Déplacement des piques
        (Transformation|SetRelativeLocation _staticmesh (Math|Vector|MakeVector (.x _relativelocation) (.y _relativelocation) (Math|Float|MapRangeClamped _movement 0.0 1.0 -4e+01 (Variables|Default|GetHeight))) false false))
      (:Finished
        (if (Variables|OpenVariables|GetIsInfinite)
          ;[1 1 1] Delay
          (Utilities|FlowControl|Delay (Utilities|Array|Get(acopy) (Variables|OpenVariables|GetDelay) (Variables|Default|GetCount)))
          (Variables|Default|SetCount (Math|Integer|SelectInt 0 (+ (Variables|Default|GetCount) 1) (> (+ (Variables|Default|GetCount) 1) (Utilities|Array|LastIndex (Variables|OpenVariables|GetDelay)))))
          (CallFunction|SpickLoop)
          (else
            (CallFunction|ResetTimeline))))
      (:SetBoolActiveSpike
        ;[1 1 1] SetSpikeActive
        (bind _isa (Utilities|FlowControl|FlipFlop)
          (:A
            _)
          (:B
            _))
        (Variables|Default|SetSpickActive _isa))
      (:ResetDoonce
        ;[1 1 1] Detecte si le player prend des dégats
        (Utilities|FlowControl|DoOnce false) ; enters at Reset
      ))))

(event Custom|ResetTimeline
  (bind _staticmesh (Variables|Default|GetStaticMesh))
  (bind _relativelocation (Variables|/Script/Engine.SceneComponent|GetRelativeLocation _staticmesh))
  (bind _movement (Timeline|Spike SetNewTime)
    (:Update
      ;[1 1 1] Déplacement des piques
      (Transformation|SetRelativeLocation _staticmesh (Math|Vector|MakeVector (.x _relativelocation) (.y _relativelocation) (Math|Float|MapRangeClamped _movement 0.0 1.0 -4e+01 (Variables|Default|GetHeight))) false false))
    (:Finished
      (if (Variables|OpenVariables|GetIsInfinite)
        ;[1 1 1] Delay
        (Utilities|FlowControl|Delay (Utilities|Array|Get(acopy) (Variables|OpenVariables|GetDelay) (Variables|Default|GetCount)))
        (Variables|Default|SetCount (Math|Integer|SelectInt 0 (+ (Variables|Default|GetCount) 1) (> (+ (Variables|Default|GetCount) 1) (Utilities|Array|LastIndex (Variables|OpenVariables|GetDelay)))))
        (CallFunction|SpickLoop)
        (else
          (CallFunction|ResetTimeline))))
    (:SetBoolActiveSpike
      ;[1 1 1] SetSpikeActive
      (bind _isa (Utilities|FlowControl|FlipFlop)
        (:A
          _)
        (:B
          _))
      (Variables|Default|SetSpickActive _isa))
    (:ResetDoonce
      ;[1 1 1] Detecte si le player prend des dégats
      (Utilities|FlowControl|DoOnce false) ; enters at Reset
    )))

(event Custom|SpickLoop
  (bind _staticmesh (Variables|Default|GetStaticMesh))
  (bind _relativelocation (Variables|/Script/Engine.SceneComponent|GetRelativeLocation _staticmesh))
  (bind _movement (Timeline|Spike PlayFromStart)
    (:Update
      ;[1 1 1] Déplacement des piques
      (Transformation|SetRelativeLocation _staticmesh (Math|Vector|MakeVector (.x _relativelocation) (.y _relativelocation) (Math|Float|MapRangeClamped _movement 0.0 1.0 -4e+01 (Variables|Default|GetHeight))) false false))
    (:Finished
      (if (Variables|OpenVariables|GetIsInfinite)
        ;[1 1 1] Delay
        (Utilities|FlowControl|Delay (Utilities|Array|Get(acopy) (Variables|OpenVariables|GetDelay) (Variables|Default|GetCount)))
        (Variables|Default|SetCount (Math|Integer|SelectInt 0 (+ (Variables|Default|GetCount) 1) (> (+ (Variables|Default|GetCount) 1) (Utilities|Array|LastIndex (Variables|OpenVariables|GetDelay)))))
        (CallFunction|SpickLoop)
        (else
          (CallFunction|ResetTimeline))))
    (:SetBoolActiveSpike
      ;[1 1 1] SetSpikeActive
      (bind _isa (Utilities|FlowControl|FlipFlop)
        (:A
          _)
        (:B
          _))
      (Variables|Default|SetSpickActive _isa))
    (:ResetDoonce
      ;[1 1 1] Detecte si le player prend des dégats
      (Utilities|FlowControl|DoOnce false) ; enters at Reset
    )))

(event EventTick
  (params (DeltaSeconds :type Float%20%28single-precision%29))
  (bind _returnvalue (Game|GetPlayerCharacter 0))
  (bind _asbp_player_test (Utilities|Casting|CastToBP_PlayerTest _returnvalue))
  ;[1 1 1] Detecte si le player prend des dégats
  (if (Variables|Default|GetSpickActive)
    (if (Collision|IsOverlappingActor (Variables|Default|GetStaticMesh) _asbp_player_test :!class /Script/Engine.PrimitiveComponent)
      (Utilities|FlowControl|DoOnce false
        (:Completed
          (Default|SetterHP _asbp_player_test (Variables|OpenVariables|GetDamage) false))))))

(event EventBeginPlay
  (Components|Timeline|SetPlayRate (Variables|Default|GetSpike) (Variables|OpenVariables|GetPlayRate))
  (if (Variables|OpenVariables|GetIsInfinite)
    (CallFunction|SpickLoop)))

(fn ConstructionScript
  (Components|StaticMesh|SetStaticMesh (Variables|Default|GetStaticMesh) (Variables|OpenVariables|GetMesh)))