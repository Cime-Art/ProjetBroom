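; BP_LibraryPlayer is a Blueprint helper library that gives typed access to the local player's core objects.
; CastController casts player controller 0 to BP_PlayerController, falls back to BP_MenuController on failure, and returns both references through a shared output.
; CastGameInstance and CastPlayer return the game instance as BP_GameInstance and pawn 0 as BP_PlayerTest.
; A failed final cast in any function ends it without reaching the return.
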(fn CastController
  (bind _returnvalue (Game|GetPlayerController 0))
  (bind _asbp_player_controller (Utilities|Casting|CastToBP_PlayerController _returnvalue)
    (:then
      _)
    (:CastFailed
      (bind _asbp_menu_controller (Utilities|Casting|CastToBP_MenuController _returnvalue))))
  (return _asbp_player_controller _asbp_menu_controller))

(fn CastGameInstance
  (bind _asbp_game_instance (Utilities|Casting|CastToBP_GameInstance (Game|GetGameInstance)))
  (return _asbp_game_instance))

(fn CastPlayer
  (bind _asbp_player_test (Utilities|Casting|CastToBP_PlayerTest (Game|Player|GetPlayerPawn 0)))
  (return _asbp_player_test))