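; BP_SwitchLevel is a level-transition trigger with two overlap volumes that respond to BP_PlayerTest.
; The BorderPop volume plays the Border timeline at a configurable speed to slide the HUD's top and bottom borders, reversing it on exit.
; The ChangeLevel volume plays the AllScreen timeline to slide the HUD's middle panel horizontally.
; When that finishes, it waits briefly, sets SwitchLevel on the game instance and opens the named level.
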(event OnComponentBeginOverlap(BorderPop)
  (params (OverlappedComponent :type Primitive%20Component%20Object%20Reference) (OtherActor :type Actor%20Object%20Reference) (OtherComp :type Primitive%20Component%20Object%20Reference) (OtherBodyIndex :type Integer) (bFromSweep :type Boolean) (SweepResult :type Hit%20Result%20Structure%20%28by%20ref%29))
  (bind _asbp_player_test (CallFunction|CastPlayer))
  (bind _wg_hud (Variables|/Game/Game_Dev/Blueprint/BP_PlayerTest.BP_PlayerTest_C|GetWG_HUD _asbp_player_test))
  (Utilities|Casting|CastToBP_PlayerTest OtherActor)
  (bind (_direction _topborder _botborder) (Timeline|Border Play)
    (:Update
      (Class|Widget|SetRenderTranslation (Variables|/Game/Game_Dev/Widget/WG_Hud.WG_Hud_C|GetBotBorder_1 _wg_hud) (Math|Vector2D|MakeVector2D 0.0 _botborder))
      (Class|Widget|SetRenderTranslation (Variables|/Game/Game_Dev/Widget/WG_Hud.WG_Hud_C|GetTopBorder _wg_hud) (Math|Vector2D|MakeVector2D 0.0 _topborder)))))

(event OnComponentEndOverlap(BorderPop)
  (params (OverlappedComponent :type Primitive%20Component%20Object%20Reference) (OtherActor :type Actor%20Object%20Reference) (OtherComp :type Primitive%20Component%20Object%20Reference) (OtherBodyIndex :type Integer))
  (bind _asbp_player_test (CallFunction|CastPlayer))
  (bind _wg_hud (Variables|/Game/Game_Dev/Blueprint/BP_PlayerTest.BP_PlayerTest_C|GetWG_HUD _asbp_player_test))
  (Utilities|Casting|CastToBP_PlayerTest OtherActor)
  (bind (_direction _topborder _botborder) (Timeline|Border Reverse)
    (:Update
      (Class|Widget|SetRenderTranslation (Variables|/Game/Game_Dev/Widget/WG_Hud.WG_Hud_C|GetBotBorder_1 _wg_hud) (Math|Vector2D|MakeVector2D 0.0 _botborder))
      (Class|Widget|SetRenderTranslation (Variables|/Game/Game_Dev/Widget/WG_Hud.WG_Hud_C|GetTopBorder _wg_hud) (Math|Vector2D|MakeVector2D 0.0 _topborder)))))

(event OnComponentBeginOverlap(ChangeLevel)
  (params (OverlappedComponent :type Primitive%20Component%20Object%20Reference) (OtherActor :type Actor%20Object%20Reference) (OtherComp :type Primitive%20Component%20Object%20Reference) (OtherBodyIndex :type Integer) (bFromSweep :type Boolean) (SweepResult :type Hit%20Result%20Structure%20%28by%20ref%29))
  (Utilities|Casting|CastToBP_PlayerTest OtherActor)
  (bind _newtrack_0 (Timeline|AllScreen Play)
    (:Update
      (Class|Widget|SetRenderTranslation (Variables|/Game/Game_Dev/Widget/WG_Hud.WG_Hud_C|GetMiddle (Variables|/Game/Game_Dev/Blueprint/BP_PlayerTest.BP_PlayerTest_C|GetWG_HUD (CallFunction|CastPlayer))) (Math|Vector2D|MakeVector2D _newtrack_0 0.0)))
    (:Finished
      (Utilities|FlowControl|Delay 1.0)
      (Variables|/Game/Game_Dev/Blueprint/BP_GameInstance.BP_GameInstance_C|SetSwitchLevel (CallFunction|CastGameInstance) true)
      (Game|OpenLevel(byName) (Variables|Default|GetLevel)))))

(event EventBeginPlay
  (Components|Timeline|SetPlayRate (Variables|Default|GetBorder) (Variables|Default|GetBorderPopSpeed)))

(fn ConstructionScript)