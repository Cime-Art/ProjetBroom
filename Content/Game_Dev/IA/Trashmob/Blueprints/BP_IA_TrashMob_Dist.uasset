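; Ranged ("Dist") trash mob AI character that flags itself to flee when the player gets close.
; On BeginPlay it switches its IA_Controller_Trashmob to the BT_IA_Dist behavior tree.
; Each Tick it sets the Fuite (flee) flag from a distance check against the player character.
; An old widget-facing-camera rotation remains as unconnected, unused logic.
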(event EventBeginPlay
  (|CallParentFunction)
  (Default|ChangeBehaviorTree (.AsIA%20Controller%20Trashmob (Utilities|Casting|CastToIA_Controller_Trashmob (AI|GetAIController self))) "/Game/Game_Dev/IA/Trashmob/BehaviorTree_Blackboard/BT_IA_Dist.BT_IA_Dist"))

(event EventTick
  (params (DeltaSeconds :type Float%20%28single-precision%29))
  (|CallParentFunction DeltaSeconds)
  (if (<= (Transformation|GetDistanceTo (Game|GetPlayerCharacter 0)) 4.5e+02)
    (Variables|Default|SetFuite? true)
    (else
      (Variables|Default|SetFuite? false))))

(event Collision|EventActorBeginOverlap
  (params (OtherActor :type Actor%20Object%20Reference)))

(fn ConstructionScript
  (|CallParentFunction))