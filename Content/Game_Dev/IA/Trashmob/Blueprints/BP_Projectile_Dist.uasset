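; BP_Projectile_Dist is an arrow projectile, apparently for ranged trash mobs, that damages the player.
; ActivatePhysics aims it at a random player skeleton socket, adds a projectile movement component at runtime and enables query-only collision.
; Its first overlap consumes a DoOnce; if that is the player, it applies damage, sticks to the mesh and destroys itself after a delay.
; A homing-target assignment exists but is unwired.
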(event OnComponentBeginOverlap(Arrow)
  (params (OverlappedComponent :type Primitive%20Component%20Object%20Reference) (OtherActor :type Actor%20Object%20Reference) (OtherComp :type Primitive%20Component%20Object%20Reference) (OtherBodyIndex :type Integer) (bFromSweep :type Boolean) (SweepResult :type Hit%20Result%20Structure%20%28by%20ref%29))
  (Utilities|FlowControl|DoOnce false
    (:Completed
      (bind _asbp_player_test (Utilities|Casting|CastToBP_PlayerTest OtherActor))
      (Default|SetterHP _asbp_player_test (Variables|Default|GetDamage) false)
      (Transformation|AttachComponentToComponent (Variables|/Script/Engine.Character|GetMesh _asbp_player_test) "None" "KeepWorld" "KeepWorld" "KeepWorld" true)
      (Components|DestroyComponent (Variables|Default|GetProjectile%20Ref))
      (Utilities|FlowControl|Delay 1e+01)
      (Actor|DestroyActor))))

(event Custom|ActivatePhysics
  (Transformation|SetActorRotation (Math|Rotator|FindLookatRotation (Transformation|GetWorldLocation (Variables|Default|GetArrow)) (Transformation|GetSocketLocation (Variables|/Script/Engine.Character|GetMesh (Game|GetPlayerCharacter 0)) (Utilities|Select :Index (Math|Random|RandomIntegerinRange 0 6) :Option%200 "Hips" :Option%201 "Spine2" :Option%202 "RightLeg" :Option%203 "Spine1" :Option%204 "Spine" :Option%205 "Head" :Option%206 "Neck"))))
  (bind _returnvalue (AddComponent|AddProjectileMovementComponent))
  (bind _output_get (Variables|Default|SetProjectile%20Ref _returnvalue))
  (Collision|SetCollisionEnabled (Variables|Default|GetArrow) "QueryOnly"))

(fn ConstructionScript)