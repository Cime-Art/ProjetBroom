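; BP_puddle is a short-lived damage puddle in the Trashmob AI folder that hurts whatever is around it.
; On BeginPlay it starts a looping timer and destroys itself after a few seconds.
; Each timer tick applies radial damage from the Damage variable at the actor's location and spawns a Niagara burst there.
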(event Custom|TickDamage
  (Game|Damage|ApplyRadialDamage (Math|Conversions|ToFloat(Integer) (Variables|Default|GetDamage)) (Transformation|GetActorLocation) 2e+02 0 0 self 0 false "ECC_Visibility")
  (Niagara|SpawnSystematLocation "/Game/Game_Dev/IA/Trashmob/Blueprints/NS_Burst.NS_Burst" (Transformation|GetActorLocation)))

(event EventBeginPlay
  (Utilities|FlowControl|Sequence
    (:then_0
      (Utilities|FlowControl|Delay 5.0)
      (Actor|DestroyActor))
    (:then_1
      (Utilities|Time|SetTimerbyEvent (delegate Custom|TickDamage) 0.2 true))))

(event Collision|EventActorBeginOverlap
  (params (OtherActor :type Actor%20Object%20Reference)))

(fn ConstructionScript)