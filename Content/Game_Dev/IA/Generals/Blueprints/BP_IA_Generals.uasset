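; Enemy General AI character in three variants, each getting its walk speed and anim blueprint in construction and passing its type to the controller to pick a behavior tree.
; Three guarded attacks lock movement but allow rotation via Custom movement mode and message the AnimInstance; EndHit clears flags and restores movement unless stunned.
; Damage ignores puddles, shows the life widget and triggers hit reactions except from spikes; death detaches the controller.
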(event Custom|StartAttack_1
  (if (not (Variables|Default|GetIsAttacking_1))
    (CallFunction|CanMove false true)
    (Class|INTAnimBpIA|AttackGeneral1(Message) (Components|SkeletalMesh|GetAnimInstance (Variables|Character|GetMesh)))
    (Variables|Default|SetIsAttacking_1 true)
    (Variables|Utilities|SetHit%20Player%20? false)))

(event Custom|TakeDamage
  (params (Degats :type Float%20%28single-precision%29) (IsTraps :type Boolean))
  ;[1 1 1] Mort
  (if (not (Variables|Default|Getisdead))
    (Rendering|SetVisibility (Variables|Default|GetWidget) true false)
    (bind _output_get (Variables|Default|SetCurrentHp (- (Variables|Default|GetCurrentHp) Degats)))
    (if (<= _output_get 0.0)
      (Class|Pawn|DetachfromControllerPendingDestroy)
      (CallFunction|CanMove false false)
      (Variables|Default|Setisdead true)
      (Class|INTAnimBpIA|Death(Message) (Components|SkeletalMesh|GetAnimInstance (Variables|Character|GetMesh)))
      (elif (not (or (Variables|Default|GetIsHit?) IsTraps))
        (Variables|Default|SetIsHit? true)
        (Class|INTAnimBpIA|GetHit(Message) (Components|SkeletalMesh|GetAnimInstance (Variables|Character|GetMesh)))))))

(event Custom|EndHit
  ;[1 1 1] EndHit
  (Variables|Default|SetIsAttacking_1 false)
  (Variables|Default|SetIsAttacking_2 false)
  (Variables|Default|SetIsAttacking_3 false)
  (Variables|Default|SetIsHit? false)
  (if (not (Variables|Default|GetStunned?))
    (CallFunction|CanMove true true)))

(event Custom|CanMove
  (params (canMove? :type Boolean) (canRotate? :type Boolean))
  (bind _charactermovement (Variables|Character|GetCharacterMovement))
  (if canMove?
    (Pawn|Components|CharacterMovement|SetMovementMode _charactermovement "MOVE_Walking" 0)
    (elif canRotate?
      (Pawn|Components|CharacterMovement|SetMovementMode _charactermovement "MOVE_Custom" 0)
      (else
        (Pawn|Components|CharacterMovement|DisableMovement _charactermovement)))))

(event Custom|StartAttack_2
  (if (not (Variables|Default|GetIsAttacking_2))
    (CallFunction|CanMove false true)
    (Class|INTAnimBpIA|AttackGeneral2(Message) (Components|SkeletalMesh|GetAnimInstance (Variables|Character|GetMesh)))
    (Variables|Default|SetIsAttacking_2 true)
    (Variables|Utilities|SetHit%20Player%20? false)))

(event Custom|StartAttack_3
  (if (not (Variables|Default|GetIsAttacking_3))
    (CallFunction|CanMove false true)
    (Class|INTAnimBpIA|AttackGeneral3(Message) (Components|SkeletalMesh|GetAnimInstance (Variables|Character|GetMesh)))
    (Variables|Default|SetIsAttacking_3 true)
    (Variables|Utilities|SetHit%20Player%20? false)))

(event Game|Damage|EventAnyDamage
  (params (Damage :type Float%20%28single-precision%29) (DamageType :type Damage%20Type%20Object%20Reference) (InstigatedBy :type Controller%20Object%20Reference) (DamageCauser :type Actor%20Object%20Reference))
  (bind _returnvalue (Utilities|GetClass DamageCauser))
  ;[1 1 1] Mort
  (if (not (== _returnvalue "/Game/Game_Dev/IA/Trashmob/Blueprints/BP_puddle.BP_Puddle_C"))
    (CallFunction|TakeDamage Damage (== _returnvalue "/Game/Game_Dev/Blueprint/Trap/BP_Spike.BP_Spike_C"))))

(event EventBeginPlay
  (Default|ChangeBehaviorTree (.AsIA%20Controller%20Generals (Utilities|Casting|CastToIA_Controller_Generals (AI|GetAIController self))) (Variables|Default|GetIA_Type_Generals))
  (Variables|/Game/Game_Dev/Widget/WG_GeneralLife.WG_GeneralLife_C|SetGenrals_ref (.AsWG%20General%20Life (Utilities|Casting|CastToWG_GeneralLife (UserInterface|GetUserWidgetObject (Variables|Default|GetWidget)))) self))

(fn ConstructionScript
  (switch Utilities|FlowControl|Switch|SwitchonIA_Types_Generals (Variables|Default|GetIA_Type_Generals)
    (:NewEnumerator0
      (Variables|Default|SetRadiusExplo 3e+02)
      (Variables|/Script/Engine.CharacterMovementComponent|SetMaxWalkSpeed (Variables|Character|GetCharacterMovement) 5e+02)
      (Class|SkeletalMeshComponent|SetAnimClass (Variables|Character|GetMesh) "/Game/Game_Dev/IA/Generals/AnimBP_TeteDeFeu.AnimBP_TeteDeFeu_C"))
    (:NewEnumerator1
      (Variables|Default|SetRadiusExplo 3e+02)
      (Variables|/Script/Engine.CharacterMovementComponent|SetMaxWalkSpeed (Variables|Character|GetCharacterMovement) 2e+02)
      (Class|SkeletalMeshComponent|SetAnimClass (Variables|Character|GetMesh) "/Game/Game_Dev/IA/Generals/AnimBP_FullBody.AnimBP_FullBody_C"))
    (:NewEnumerator2
      (Variables|Default|SetRadiusExplo 3e+02)
      (Variables|/Script/Engine.CharacterMovementComponent|SetMaxWalkSpeed (Variables|Character|GetCharacterMovement) 2e+02)
      (Class|SkeletalMeshComponent|SetAnimClass (Variables|Character|GetMesh) "/Game/Game_Dev/IA/Generals/AnimBP_Fusion.AnimBP_Fusion_C"))))