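; Jail door trap actor whose Door component starts hidden and moves vertically to close or open on demand.
; CloseDoor shows the door and plays the Movement timeline, which drives its relative Z; OpenDoor plays the same timeline in reverse.
; A Close flag lets the shared Finished handler hide the door only after opening, and both events post the BoneWall Wwise sound.
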(event EventOpenDoor
  (bind _door (Variables|Default|GetDoor))
  (bind _relativelocation (Variables|/Script/Engine.SceneComponent|GetRelativeLocation _door))
  (Variables|Default|SetClose false)
  ;[1 1 1] Sound Tavu
  (Class|AkGameplayStatics|PostEvent "/Game/WwiseAudio/Events/Default_Work_Unit/Level/Hell/Event_BoneWall.Event_BoneWall" self)
  (bind _z (Timeline|Movement ReverseFromEnd)
    (:Update
      (Transformation|SetRelativeLocation _door (Math|Vector|MakeVector (.x _relativelocation) (.y _relativelocation) _z) false false))
    (:Finished
      (if (not (Variables|Default|GetClose))
        (Rendering|SetVisibility (Variables|Default|GetDoor) false false)))))

(event EventCloseDoor
  (bind _door (Variables|Default|GetDoor))
  (bind _relativelocation (Variables|/Script/Engine.SceneComponent|GetRelativeLocation _door))
  (Rendering|SetVisibility (Variables|Default|GetDoor) true false)
  (Variables|Default|SetClose true)
  ;[1 1 1] Sound Tavu
  (Class|AkGameplayStatics|PostEvent "/Game/WwiseAudio/Events/Default_Work_Unit/Level/Hell/Event_BoneWall.Event_BoneWall" self)
  (bind _z (Timeline|Movement PlayFromStart)
    (:Update
      (Transformation|SetRelativeLocation _door (Math|Vector|MakeVector (.x _relativelocation) (.y _relativelocation) _z) false false))
    (:Finished
      (if (not (Variables|Default|GetClose))
        (Rendering|SetVisibility (Variables|Default|GetDoor) false false)))))

(event EventBeginPlay
  (Rendering|SetVisibility (Variables|Default|GetDoor) false false))

(fn ConstructionScript)