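; Spike trap that damages characters standing in its box, either triggered by their capsule overlap or looping infinitely.
; A timeline raises the mesh and toggles the damage window, with a Wwise sound posted on overlap activation.
; A map of overlapping characters to bools limits damage to one hit per cycle, re-arming and replaying while occupied.
; Infinite mode starts on BeginPlay and cycles through an array of delays between strikes.
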(event OnComponentBeginOverlap(Box)
  (params (OverlappedComponent :type Primitive%20Component%20Object%20Reference) (OtherActor :type Actor%20Object%20Reference) (OtherComp :type Primitive%20Component%20Object%20Reference) (OtherBodyIndex :type Integer) (bFromSweep :type Boolean) (SweepResult :type Hit%20Result%20Structure%20%28by%20ref%29))
  (bind _ascharacter (Utilities|Casting|CastToCharacter OtherActor))
  (Utilities|Casting|CastToCapsuleComponent OtherComp)
  (Utilities|Map|Add (Variables|Default|GetOverlapingActor) _ascharacter true)
  ;[1 1 1] Activate spike if first actor on it
  (if (not (Audio|Components|Audio|IsPlaying (Variables|Default|GetSpike)))
    (CallFunction|ActivateSpike)
    (Class|AkGameplayStatics|PostEvent "/Game/WwiseAudio/Events/Default_Work_Unit/Level/Hell/Event_SpikeTrap.Event_SpikeTrap" self)))

(event OnComponentEndOverlap(Box)
  (params (OverlappedComponent :type Primitive%20Component%20Object%20Reference) (OtherActor :type Actor%20Object%20Reference) (OtherComp :type Primitive%20Component%20Object%20Reference) (OtherBodyIndex :type Integer))
  ;[1 1 1] End Overlap - Remove Actor
  (bind _ascharacter (Utilities|Casting|CastToCharacter OtherActor))
  (Utilities|IsValid _ascharacter
    (:Is%20Valid
      (Utilities|Map|Remove (Variables|Default|GetOverlapingActor) _ascharacter))))

(event Custom|ActivateSpike
  (bind _staticmesh (Variables|Default|GetStaticMesh))
  (bind _relativelocation (Variables|/Script/Engine.SceneComponent|GetRelativeLocation _staticmesh))
  (bind _movement (Timeline|Spike PlayFromStart)
    (:Update
      ;[1 1 1] Déplacement des piques
      (Transformation|SetRelativeLocation _staticmesh (Math|Vector|MakeVector (.x _relativelocation) (.y _relativelocation) (Math|Float|MapRangeClamped _movement 0.0 1.0 -4e+01 (Variables|Default|GetHeight))) false false)
      (if (and (Variables|Default|GetSpickActive) (not (Variables|OpenVariables|GetIsInfinite)))
        (CallFunction|ApplyDamagetoAll :!label _label)
        (elif (Math|Boolean|ANDBoolean (Variables|Default|GetSpickActive) (Variables|OpenVariables|GetIsInfinite) (> (Utilities|Map|Length (Variables|Default|GetOverlapingActor)) 0))
          (goto _label))))
    (:Finished
      (CallFunction|ResetSpike)
      (if (Variables|OpenVariables|GetIsInfinite)
        (CallFunction|InfiniteSpikeLoopDelay)))
    (:SetBoolActiveSpike
      (Variables|Default|SetSpickActive (not (Variables|Default|GetSpickActive))))))

(event Custom|ApplyDamageToAll
  (bind _overlapingactor (Variables|Default|GetOverlapingActor))
  ;[1 1 1] ApplyDamageToAll
  (bind _values (Utilities|Map|Values _overlapingactor))
  (bind _keys (Utilities|Map|Keys _overlapingactor))
  (for (_array_element _array_index) _keys
    (if (Utilities|Array|Get(acopy) _values _array_index)
      (Game|Damage|ApplyDamage _array_element (Variables|OpenVariables|GetDamage) 0 self)
      (Utilities|Map|Add (Variables|Default|GetOverlapingActor) _array_element false))))

(event Custom|BeginLoop)

(event Custom|ResetSpike
  (bind _overlapingactor (Variables|Default|GetOverlapingActor))
  ;[1 1 1] Still one actor on spike at the end of timeline
  (if (> (Utilities|Map|Length (Variables|Default|GetOverlapingActor)) 0)
    (bind _keys (Utilities|Map|Keys _overlapingactor))
    (for _array_element _keys
      (Utilities|Map|Add _overlapingactor _array_element true))
    (CallFunction|ActivateSpike)))

(event Custom|InfiniteSpikeLoopDelay
  ;[1 1 1] Delay
  (Utilities|FlowControl|Delay (Utilities|Array|Get(acopy) (Variables|OpenVariables|GetDelay) (Variables|Default|GetCount)))
  (Variables|Default|SetCount (Math|Integer|SelectInt 0 (+ (Variables|Default|GetCount) 1) (> (+ (Variables|Default|GetCount) 1) (Utilities|Array|LastIndex (Variables|OpenVariables|GetDelay)))))
  (CallFunction|ActivateSpike))

(event EventBeginPlay
  ;[1 1 1] Begin play
  (Components|Timeline|SetPlayRate (Variables|Default|GetSpike) (Variables|OpenVariables|GetPlayRate))
  (if (Variables|OpenVariables|GetIsInfinite)
    (CallFunction|ActivateSpike)))

(fn ConstructionScript
  (Components|StaticMesh|SetStaticMesh (Variables|Default|GetStaticMesh) (Variables|OpenVariables|GetMesh)))