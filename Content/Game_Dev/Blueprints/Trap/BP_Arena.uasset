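; Wave-based combat arena that shuts its doors when the player enters and reopens them once every wave is cleared.
; Each wave's class-to-count map feeds a randomly delayed, self-recalling spawner that places mobs via downward traces in the box, optionally involving a spawn platform.
; Kill counts advance waves, while ResetArena destroys mobs and rewinds an active fight.
; Seen events update overlapping trash mobs' blackboards and seed new spawns' awareness.
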(event OnComponentBeginOverlap(Box)
  (params (OverlappedComponent :type Primitive%20Component%20Object%20Reference) (OtherActor :type Actor%20Object%20Reference) (OtherComp :type Primitive%20Component%20Object%20Reference) (OtherBodyIndex :type Integer) (bFromSweep :type Boolean) (SweepResult :type Hit%20Result%20Structure%20%28by%20ref%29))
  ;[1 1 1] In Fct Of the Number Of Mobs Door Close/Open
  (Utilities|Casting|CastToBP_PlayerTest OtherActor)
  (if (and (Variables|OpenVariable|GetSpawn) (not (Variables|Default|GetCleared)))
    (Utilities|FlowControl|DoOnce false
      (:Completed
        (if (not (< (Utilities|Array|LastIndex (Variables|OpenVariable|GetMobs)) 0))
          (CallFunction|LaunchWave)
          (Variables|ResetArena|SetActive true)
          (for _array_element (Variables|OpenVariable|GetBp_Door)
            (Default|CloseDoor _array_element)))))))

(event Custom|UnSeen
  ;[1 1 1] IA SEEN SYSTEM
  (Variables|Default|SetSeen false)
  (for _array_element (Collision|GetOverlappingActors (Variables|Default|GetBox) "/Game/Game_Dev/Blueprints/IA/Trashmob/Blueprints/BP_IA_TrashMob.BP_IA_TrashMob_C" :!class /Script/Engine.PrimitiveComponent)
    (bind _asbp_ia_trash_mob (Utilities|Casting|CastToBP_IA_TrashMob _array_element))
    (Utilities|IsValid (AI|GetBlackboard _array_element)
      (:Is%20Valid
        (Variables|/Script/Engine.CharacterMovementComponent|SetMaxWalkSpeed (Variables|/Script/Engine.Character|GetCharacterMovement _asbp_ia_trash_mob) (Variables|/Game/Game_Dev/Blueprints/IA/Trashmob/Blueprints/BP_IA_TrashMob.BP_IA_TrashMob_C|GetSpeed _asbp_ia_trash_mob))
        (AI|Components|Blackboard|SetValueasBool (AI|GetBlackboard _array_element) (Utilities|Name|MakeLiteralName "Seen?") false)))))

(event Custom|RespawnMob
  (bind _mobs (Variables|OpenVariable|GetMobs))
  (bind _bp_platform_spawn_ennemie (Variables|OpenVariable|GetBP_Platform_Spawn_Ennemie))
  (bind _currentwave (Variables|Default|GetCurrentWave))
  (bind _output (Utilities|Array|Get(acopy) _mobs _currentwave))
  (bind _mobs_2 (Utilities|Struct|BreakStruct_Arena _output))
  ;[1 1 1] Respawn Mobs
  (Utilities|IsValid _bp_platform_spawn_ennemie
    (:Is%20Valid
      (if (not (Variables|/Game/Game_Dev/Blueprints/Platform/PlatformSpawningEnnemie/BP_Platform_SpawnEnnemie.BP_Platform_SpawnEnnemie_C|GetStopSpawn _bp_platform_spawn_ennemie))
        (Utilities|FlowControl|Delay (Math|Random|RandomFloatinRange 0.0 1.0) :!label _label)
        (bind _keys (Utilities|Map|Keys _mobs_2))
        (Variables|Map|SetMobsMap _keys)
        (bind _values (Utilities|Map|Values _mobs_2))
        (Variables|Map|SetNbMobsMap _values)
        (if (not (== (Utilities|Array|Get(acopy) (Variables|Map|GetNbMobsMap) (Variables|Default|GetIndex)) (Variables|Default|GetCompteur)))
          (bind _returnvalue (Game|SpawnActorfromClass (Utilities|Array|Get(acopy) (Variables|Map|GetMobsMap) (Variables|Default|GetIndex)) (Math|Transform|MakeTransform (CallFunction|CalculateSpawnLocation) "0, 0, 0" "1,1,1") "AdjustIfPossibleButDontSpawnIfColliding" 0 self true (Variables|OpenVariable|GetNiagaraSystem) (Variables|Default|GetSeen) 0 :!label _label_2))
          (Utilities|IsValid _returnvalue
            (:Is%20Valid
              (Math|Integer|DecrementInt (Variables|Default|GetNumberMob)
                (:%20%20
                  (Math|Integer|IncrementInt (Variables|Default|GetCompteur)
                    (:%20%20
                      (Utilities|Array|Add (Variables|ResetArena|GetListMobs) _returnvalue)
                      (Class|AkGameplayStatics|PostEvent "/Game/WwiseAudio/Events/Default_Work_Unit/Mob/Event_Spawn.Event_Spawn" self)
                      (if (not (== (Variables|Default|GetNumberMob) 0))
                        (CallFunction|RespawnMob)))))))
            (:Is%20Not%20Valid
              (CallFunction|RespawnMob)))
          (else
            (Variables|Default|SetCompteur 0)
            (if (!= (Variables|Default|GetIndex) (Utilities|Array|LastIndex (Variables|Map|GetMobsMap)))
              (Math|Integer|IncrementInt (Variables|Default|GetIndex)
                (:%20%20
                  (goto _label_2))))))))
    (:Is%20Not%20Valid
      (goto _label))))

(event Custom|ResetArena
  ;[1 1 1] Reset de l'arene
  (if (Variables|ResetArena|GetActive)
    (for _array_element (Variables|ResetArena|GetListMobs)
      (Utilities|IsValid _array_element
        (:Is%20Valid
          (Default|DeathSound _array_element)
          (Actor|DestroyActor _array_element))))
    (for _array_element_2 (Variables|OpenVariable|GetBp_Door)
      (Default|OpenDoor _array_element_2))
    (Variables|ResetArena|SetActive false)
    (Variables|Default|SetKilledMob 0)
    (Variables|Default|SetNumberMob 0)
    (Variables|Default|SetCompteur 0)
    (Variables|Default|SetIndex 0)
    (Variables|Default|SetCurrentWave 0)
    (CallFunction|ResetRespawnDoOnce)
    (CallFunction|ResetDoOnce)))

(event Custom|RemoveMobs
  ;[1 1 1] Compteur de kill
  (Math|Integer|IncrementInt (Variables|Default|GetKilledMob)
    (:%20%20
      (if (and (>= (Variables|Default|GetKilledMob) (Variables|Default|GetNBMobsPerWawe)) (== (Variables|Default|GetCurrentWave) (Variables|Default|GetNbWave)))
        (Variables|Default|SetCleared true)
        (Variables|ResetArena|SetActive false)
        (Utilities|FlowControl|DoOnce false
          (:Completed
            (for _array_element (Variables|OpenVariable|GetBp_Door)
              (Default|OpenDoor _array_element))))
        (elif (>= (Variables|Default|GetKilledMob) (Variables|Default|GetNBMobsPerWawe))
          (Math|Integer|IncrementInt (Variables|Default|GetCurrentWave)
            (:%20%20
              (Variables|Default|SetKilledMob 0)
              (Variables|Default|SetCompteur 0)
              (Variables|Default|SetIndex 0)
              (CallFunction|LaunchWave))))))))

(event Custom|SetSeen
  ;[1 1 1] IA SEEN SYSTEM
  (Variables|Default|SetSeen true)
  (for _array_element (Collision|GetOverlappingActors (Variables|Default|GetBox) "/Game/Game_Dev/Blueprints/IA/Trashmob/Blueprints/BP_IA_TrashMob.BP_IA_TrashMob_C" :!class /Script/Engine.PrimitiveComponent)
    (bind _asbp_ia_trash_mob (Utilities|Casting|CastToBP_IA_TrashMob _array_element))
    (Utilities|IsValid (AI|GetBlackboard _array_element)
      (:Is%20Valid
        (Variables|/Script/Engine.CharacterMovementComponent|SetMaxWalkSpeed (Variables|/Script/Engine.Character|GetCharacterMovement _asbp_ia_trash_mob) (Variables|/Game/Game_Dev/Blueprints/IA/Trashmob/Blueprints/BP_IA_TrashMob.BP_IA_TrashMob_C|GetSpeed _asbp_ia_trash_mob))
        (AI|Components|Blackboard|SetValueasBool (AI|GetBlackboard _array_element) (Utilities|Name|MakeLiteralName "Seen?") true)))))

(event Custom|LaunchWave
  ;[1 1 1] NB mobs per wawe
  (if (not (Variables|Default|GetCleared))
    (bind _values (Utilities|Map|Values (Utilities|Struct|BreakStruct_Arena (Utilities|Array|Get(acopy) (Variables|OpenVariable|GetMobs) (Variables|Default|GetCurrentWave)))))
    (for _array_element _values
      (Variables|Default|SetNumberMob (+ (Variables|Default|GetNumberMob) _array_element)))
    ;;[1 1 1] Wave Variables
    (Variables|Default|SetNBMobsPerWawe (Variables|Default|GetNumberMob))
    (Utilities|IsValid (Variables|OpenVariable|GetBP_Platform_Spawn_Ennemie)
      (:Is%20Valid
        (if (== (Variables|Default|GetCurrentWave) 1)
          (Default|Shake (Variables|OpenVariable|GetBP_Platform_Spawn_Ennemie))
          (else
            (CallFunction|RespawnMob :!label _label))))
      (:Is%20Not%20Valid
        (goto _label)))))

(event Custom|ResetRespawnDoOnce
  ;[1 1 1] In Fct Of the Number Of Mobs Door Close/Open
  (Utilities|FlowControl|DoOnce false) ; enters at Reset
)

(event Custom|ResetDoOnce
  ;[1 1 1] Compteur de kill
  (Utilities|FlowControl|DoOnce false) ; enters at Reset
)

(event EventTick
  (params (DeltaSeconds :type Float%20%28single-precision%29)))

(event EventBeginPlay
  ;[1 1 1] Wave
  (Variables|Default|SetNbWave (Utilities|Array|LastIndex (Variables|OpenVariable|GetMobs))))

(fn ConstructionScript)

(fn CalculateSpawnLocation
  (bind _returnvalue (Transformation|GetActorLocation))
  (bind _box (Variables|Default|GetBox))
  (bind _z (Math|Vector|BreakVector _returnvalue))
  (bind _returnvalue_2 (Components|Box|GetScaledBoxExtent _box))
  (bind _returnvalue_3 (Math|Random|RandomPointinBoundingBox _returnvalue _returnvalue_2))
  (bind _z_2 (Math|Vector|BreakVector _returnvalue_2))
  (bind _returnvalue_4 (+ _z _z_2))
  (bind _outhit (Collision|LineTraceByChannel (Math|Vector|MakeVector (.x _returnvalue_3) (.y _returnvalue_3) _returnvalue_4) (Math|Vector|MakeVector (.x _returnvalue_3) (.y _returnvalue_3) (- _returnvalue_4 5e+03)) "TraceTypeQuery1" true 0 "None"))
  (return (.impactpoint _outhit)))