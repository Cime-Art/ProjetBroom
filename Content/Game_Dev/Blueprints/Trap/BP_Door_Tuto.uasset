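; Tutorial door Blueprint that swings open once when the player character overlaps its box trigger.
; The overlap casts to BP_PlayerTest and passes a DoOnce that is never reset.
; The sign of the player's forward-vector Y picks one of two timelines, each driving the yaw of StaticMesh2, so swing direction depends on player facing.
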(event OnComponentBeginOverlap(Box)
  (params (OverlappedComponent :type Primitive%20Component%20Object%20Reference) (OtherActor :type Actor%20Object%20Reference) (OtherComp :type Primitive%20Component%20Object%20Reference) (OtherBodyIndex :type Integer) (bFromSweep :type Boolean) (SweepResult :type Hit%20Result%20Structure%20%28by%20ref%29))
  (bind _staticmesh2 (Variables|Default|GetStaticMesh2))
  (bind _staticmesh2_2 (Variables|Default|GetStaticMesh2))
  (bind _relativerotation (Variables|/Script/Engine.SceneComponent|GetRelativeRotation _staticmesh2))
  (bind _relativerotation_2 (Variables|/Script/Engine.SceneComponent|GetRelativeRotation _staticmesh2_2))
  (bind _asbp_player_test (Utilities|Casting|CastToBP_PlayerTest OtherActor))
  (Utilities|FlowControl|DoOnce false
    (:Completed
      (if (select (>= (.Y (Math|Vector|BreakVector (Transformation|GetActorForwardVector _asbp_player_test))) 0.0) false (<= (.Y (Math|Vector|BreakVector (Transformation|GetActorForwardVector _asbp_player_test))) 0.0))
        (bind _rotation (Timeline|Timeline_0 Play)
          (:Update
            (Transformation|SetRelativeRotation _staticmesh2_2 (Math|Rotator|MakeRotator (.roll _relativerotation_2) (.pitch _relativerotation_2) _rotation) false false)))
        (else
          (bind _rotation_2 (Timeline|Timeline_1 Play)
            (:Update
              (Transformation|SetRelativeRotation _staticmesh2 (Math|Rotator|MakeRotator (.roll _relativerotation) (.pitch _relativerotation) _rotation_2) false false))))))))

(event EventBeginPlay)

(fn ConstructionScript)