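; BP_Blade_Lava is a trap whose configurable mesh slides back and forth along its local X axis.
; A looping timeline drives the travel at an adjustable play rate and distance, reversing after a delay at each end.
; The timeline's event track toggles the damage window.
; While it is open, a player starting to overlap the box takes a massive HP hit.
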(event OnComponentBeginOverlap(Box)
  (params (OverlappedComponent :type Primitive%20Component%20Object%20Reference) (OtherActor :type Actor%20Object%20Reference) (OtherComp :type Primitive%20Component%20Object%20Reference) (OtherBodyIndex :type Integer) (bFromSweep :type Boolean) (SweepResult :type Hit%20Result%20Structure%20%28by%20ref%29))
  ;[1 1 1] Damage
  (if (Variables|Default|GetDoDamage)
    (bind _asbp_player_test (Utilities|Casting|CastToBP_PlayerTest OtherActor))
    (Default|SetterHP _asbp_player_test 1e+04 false)))

(event Custom|EventMovement
  (params (Begin :type Boolean))
  (bind _staticmesh (Variables|Default|GetStaticMesh))
  (bind _relativelocation (Variables|/Script/Engine.SceneComponent|GetRelativeLocation _staticmesh))
  ;[1 1 1] Movement
  (if Begin
    (bind _movement (Timeline|Movement PlayFromStart)
      (:Update
        (Transformation|SetRelativeLocation _staticmesh (Math|Vector|MakeVector (Math|Float|Lerp 0.0 (Variables|OpenVariables|GetDistance) _movement) (.y _relativelocation) (.z _relativelocation)) false false))
      (:Finished
        (Utilities|FlowControl|Delay (Variables|OpenVariables|GetDelayBeforeAttack))
        (CallFunction|EventMovement (not Begin)))
      (:Event
        (Variables|Default|SetDoDamage (not (Variables|Default|GetDoDamage)))))
    (else
      (Timeline|Movement ReverseFromEnd))))

(event EventBeginPlay
  ;[1 1 1] Initialise
  (Components|Timeline|SetPlayRate (Variables|Default|GetMovement) (Variables|OpenVariables|GetPlayRateDeplacement))
  (CallFunction|EventMovement true))

(fn ConstructionScript
  (Components|StaticMesh|SetStaticMesh (Variables|Default|GetStaticMesh) (Variables|OpenVariables|GetMesh)))