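; BP_Tuto is a trigger volume that shows a tutorial preview when the player character walks into its box.
; The overlap, filtered to BP_PlayerTest, closes the referenced BPDoor if valid, then through a DoOnce creates the HUD_Tuto_Preview widget with the Tuto enum and adds it to the viewport.
; The actor then destroys itself, and a debug "Hello" string prints on overlap.
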(event OnComponentBeginOverlap(Box)
  (params (OverlappedComponent :type Primitive%20Component%20Object%20Reference) (OtherActor :type Actor%20Object%20Reference) (OtherComp :type Primitive%20Component%20Object%20Reference) (OtherBodyIndex :type Integer) (bFromSweep :type Boolean) (SweepResult :type Hit%20Result%20Structure%20%28by%20ref%29))
  (Utilities|Casting|CastToBP_PlayerTest OtherActor)
  (Development|PrintString "Hello")
  (Utilities|IsValid (Variables|Default|GetBP_Door)
    (:Is%20Valid
      (Default|CloseDoor (Variables|Default|GetBP_Door)))
    (:Is%20Not%20Valid
      _))
  (Utilities|FlowControl|DoOnce false
    (:Completed
      (bind _returnvalue (UserInterface|CreateWidget "/Game/Game_Dev/Blueprints/Widget/Tuto/HUD_Tuto_Preview.HUD_Tuto_Preview_C" 0 (Variables|Default|GetTuto)))
      (UserInterface|Viewport|AddtoViewport _returnvalue 0)
      (Actor|DestroyActor))))

(fn ConstructionScript)