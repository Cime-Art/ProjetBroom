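; Crown pickup that adds to the player's saved crown count when BP_PlayerTest overlaps its box.
; A DoOnce guards the overlap, then the Game Instance's Crowns count increments and is copied into CrownSaveData.
; That object saves asynchronously to the "Crowns" slot, and the actor destroys itself only when the save completes.
; Tick prints the current crown count on screen every frame.
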(event OnComponentBeginOverlap(Box)
  (params (OverlappedComponent :type Primitive%20Component%20Object%20Reference) (OtherActor :type Actor%20Object%20Reference) (OtherComp :type Primitive%20Component%20Object%20Reference) (OtherBodyIndex :type Integer) (bFromSweep :type Boolean) (SweepResult :type Hit%20Result%20Structure%20%28by%20ref%29))
  (bind _gameinstance (CallFunction|CastGameInstance))
  (bind _crownsavedata (Variables|/Game/Game_Dev/Blueprints/GameSettings/BP_GameInstance.BP_GameInstance_C|GetCrownSaveData _gameinstance))
  (Utilities|Casting|CastToBP_PlayerTest OtherActor)
  (Utilities|FlowControl|DoOnce false
    (:Completed
      (bind _result (Math|Integer|IncrementInt (Variables|/Game/Game_Dev/Blueprints/GameSettings/BP_GameInstance.BP_GameInstance_C|GetCrowns _gameinstance))
        (:%20%20
          (Variables|/Game/Game_Dev/Blueprints/GameSettings/BP_SaveGame.BP_SaveGame_C|SetCrowns _crownsavedata _result)
          (|AsyncSaveGametoSlot _crownsavedata "Crowns"
            (:Completed
              (Actor|DestroyActor))))))))

(event EventBeginPlay)

(event Collision|EventActorBeginOverlap
  (params (OtherActor :type Actor%20Object%20Reference)))

(event EventTick
  (params (DeltaSeconds :type Float%20%28single-precision%29))
  (Development|PrintString (Utilities|String|ToString(Integer) (Variables|/Game/Game_Dev/Blueprints/GameSettings/BP_GameInstance.BP_GameInstance_C|GetCrowns (CallFunction|CastGameInstance))) true true "(R=0.000000,G=0.660000,B=1.000000,A=1.000000)" 0.0))

(fn ConstructionScript)