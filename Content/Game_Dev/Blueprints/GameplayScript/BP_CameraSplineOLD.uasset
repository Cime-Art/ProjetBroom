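; Spline-rail camera actor that follows the player while its PlayerIn flag is set.
; Each tick it rotates the camera component to look directly at the player's location.
; It also eases the camera toward the spline point closest to the player, using a lerp with world delta seconds as alpha.
; Nothing in this file sets PlayerIn, and a distance-to-player string conversion is left unused.
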(event EventTick
  (params (DeltaSeconds :type Float%20%28single-precision%29))
  (bind _asbp_player_test (CallFunction|CastPlayer))
  (bind _returnvalue (Utilities|Time|GetWorldDeltaSeconds))
  (bind _cameracomponent (Variables|CameraActor|GetCameraComponent))
  (bind _cameracomponent_2 (Variables|CameraActor|GetCameraComponent))
  (bind _spline (Variables|Default|GetSpline))
  (bind _returnvalue_2 (Transformation|GetActorLocation _asbp_player_test))
  (bind _returnvalue_3 (Transformation|GetWorldLocation _cameracomponent))
  (bind _returnvalue_4 (Spline|FindLocationClosesttoWorldLocation _spline _returnvalue_2 "World"))
  (bind _returnvalue_5 (Math|Vector|Lerp(Vector) _returnvalue_3 _returnvalue_4 _returnvalue))
  (if (Variables|Default|GetPlayerIn)
    (Transformation|SetWorldRotation _cameracomponent_2 (Math|Rotator|FindLookatRotation (Transformation|GetWorldLocation _cameracomponent_2) (Transformation|GetActorLocation (CallFunction|CastPlayer))) false false)
    (Transformation|SetWorldLocation _cameracomponent (Math|Vector|MakeVector (.x _returnvalue_5) (.y _returnvalue_5) (.z _returnvalue_5)) false false)
    (if true
      _)))

(fn ConstructionScript)