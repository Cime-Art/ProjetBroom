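; BP_Checkpoint is a one-time checkpoint that saves player progress when BP_PlayerTest overlaps its box.
; On first overlap it launches Niagara on its campfires, refills HP and mana, and records lives, continues, level name and respawn point.
; The respawn point combines the box's XY with the player's Z, and the GameInstance saves the updated InfoPlayer.
; DestroyKids recursively destroys the linked Kids actor.
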(event OnComponentBeginOverlap(Box)
  (params (OverlappedComponent :type Primitive%20Component%20Object%20Reference) (OtherActor :type Actor%20Object%20Reference) (OtherComp :type Primitive%20Component%20Object%20Reference) (OtherBodyIndex :type Integer) (bFromSweep :type Boolean) (SweepResult :type Hit%20Result%20Structure%20%28by%20ref%29))
  (bind _box (Variables|Default|GetBox))
  (bind _returnvalue (Transformation|GetWorldLocation _box))
  (if (not (Variables|Default|GetActivated?))
    (bind _asbp_player_test (Utilities|Casting|CastToBP_PlayerTest OtherActor))
    (for _array_element (Variables|Default|GetMeshCampfire)
      (Default|LaunchNiagara _array_element))
    (bind _returnvalue_2 (Game|GetCurrentLevelName true))
    (|SetBy-RefVar (Variables|/Game/Game_Dev/Blueprints/Player/BP_PlayerTest.BP_PlayerTest_C|GetInfoPlayer _asbp_player_test) (Utilities|Struct|MakeStruct_InfoPlayer (.maxhp (Variables|/Game/Game_Dev/Blueprints/Player/BP_PlayerTest.BP_PlayerTest_C|GetInfoPlayer _asbp_player_test)) (.maxhp (Variables|/Game/Game_Dev/Blueprints/Player/BP_PlayerTest.BP_PlayerTest_C|GetInfoPlayer _asbp_player_test)) (.maxmana (Variables|/Game/Game_Dev/Blueprints/Player/BP_PlayerTest.BP_PlayerTest_C|GetInfoPlayer _asbp_player_test)) (.maxmana (Variables|/Game/Game_Dev/Blueprints/Player/BP_PlayerTest.BP_PlayerTest_C|GetInfoPlayer _asbp_player_test)) (Math|Vector|MakeVector (.x _returnvalue) (.y _returnvalue) (.z (Transformation|GetActorLocation (CallFunction|CastPlayer)))) (.currentlife (Variables|/Game/Game_Dev/Blueprints/Player/BP_PlayerTest.BP_PlayerTest_C|GetInfoPlayer _asbp_player_test)) (.currentcontinue (Variables|/Game/Game_Dev/Blueprints/Player/BP_PlayerTest.BP_PlayerTest_C|GetInfoPlayer _asbp_player_test)) (Utilities|String|StringToName _returnvalue_2)))
    (Variables|Default|SetActivated? true)
    (Default|SaveData (CallFunction|CastGameInstance) (Variables|/Game/Game_Dev/Blueprints/Player/BP_PlayerTest.BP_PlayerTest_C|GetInfoPlayer _asbp_player_test))))

(event Custom|DestroyKids
  (bind _kids (Variables|Default|GetKids))
  (Utilities|IsValid _kids
    (:Is%20Valid
      (CallFunction|DestroyKids _kids)
      (Actor|DestroyActor _kids))))

(fn ConstructionScript)