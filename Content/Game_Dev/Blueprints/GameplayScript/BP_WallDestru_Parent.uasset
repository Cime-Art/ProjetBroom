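; Parent Blueprint for destructible walls that play a break animation, dissolve and remove themselves.
; PlayAnimation runs once: it plays the skeletal mesh animation, disables mesh and box collision, and posts an optional Wwise destruction event.
; After a configurable delay, a timeline drives the materials' Dissolve parameter, then the actor's audio stops and it is destroyed shortly after.
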(event Custom|PlayAnimation
  (bind _audiodestructible (Variables|Default|GetAudioDestructible))
  (bind _skeletalmesh (Variables|Default|GetSkeletalMesh))
  (Utilities|FlowControl|DoOnce false
    (:Completed
      (Audio|Components|Audio|Play _skeletalmesh false)
      (Collision|SetCollisionEnabled _skeletalmesh "NoCollision")
      (Utilities|IsValid _audiodestructible
        (:Is%20Valid
          (Class|AkGameplayStatics|PostEvent _audiodestructible self))
        (:Is%20Not%20Valid
          _))
      (Utilities|FlowControl|Delay (Variables|Default|GetDelayBeforeDissolve))
      (bind _newtrack_0 (Timeline|Timeline_0 PlayFromStart)
        (:Update
          (Rendering|Material|SetScalarParameterValueonMaterials (Variables|Default|GetSkeletalMesh) "Dissolve" _newtrack_0))
        (:Finished
          (Class|AkGameplayStatics|StopActor)
          (Utilities|FlowControl|Delay 2.0)
          (Actor|DestroyActor))))))

(fn ConstructionScript)