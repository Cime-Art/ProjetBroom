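; Loot chest that grants one equipment piece, chosen by item type and set, when the player enters its trigger box.
; The construction script builds the item data from those choices, and MeshRender supplies the drop's mesh.
; Chained timelines open the lid (also calling Taniere on any linked AI), raise the spawned item, then fly it to the player and add it.
; After a short BeginPlay delay, the chest shows as open if the player's inventory holds the item.
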(event OnComponentBeginOverlap(Box)
  (params (OverlappedComponent :type Primitive%20Component%20Object%20Reference) (OtherActor :type Actor%20Object%20Reference) (OtherComp :type Primitive%20Component%20Object%20Reference) (OtherBodyIndex :type Integer) (bFromSweep :type Boolean) (SweepResult :type Hit%20Result%20Structure%20%28by%20ref%29))
  (bind _objecttype (Variables|Default|GetObjectType))
  (bind (_nameobj _lifegiving _managiving _logo _type _set) (Utilities|Struct|BreakStruct_Object _objecttype))
  ;[1 1 1] Loot system
  (Utilities|Casting|CastToBP_PlayerTest OtherActor)
  (if (not (Variables|Default|GetOpen))
    (Utilities|FlowControl|DoOnce false
      (:Completed
        (Class|AkGameplayStatics|PostEvent "/Game/WwiseAudio/Events/Default_Work_Unit/Props/MagicChest/Event_MagicChestOpen.Event_MagicChestOpen" self)
        (Components|Activation|SetActive (Variables|Default|GetNiagara) true true)
        (bind _rotation (Timeline|OpenChest PlayFromStart)
          (:Update
            (Transformation|SetRelativeRotation (Variables|Default|GetCoffre_Couvercle_coffe) (Math|Rotator|MakeRotator (Math|Float|MapRangeClamped _rotation 0.0 1.0 0.0 (Variables|Default|GetRotation%20coffre)) 0.0 0.0) false false)
            (bind _bpiaref (Variables|OpenVariable|GetBpIARef)
              (:then
                (Default|Taniere _bpiaref))
              (:else)))
          (:Finished
            (Utilities|FlowControl|DoOnce false
              (:Completed
                (Components|DestroyComponent (Variables|Default|GetSpotLight))
                (Variables|Default|SetOpen true)
                (bind _returnvalue (Game|SpawnActorfromClass "/Game/Game_Dev/Blueprints/GameplayScript/BP_ItemDrop.BP_ItemDrop_C" (Math|Transform|MakeTransform (Transformation|GetActorLocation) "0, 0, 0" "1,1,1") "AlwaysSpawn" 0 (Utilities|MeshRender _type _set _set _set) _objecttype 0))
                (Variables|Default|SetItemLooted _returnvalue)
                (Transformation|AttachActorToActor _returnvalue self "None" "KeepRelative" "KeepRelative" "KeepRelative" true)
                (bind _newtrack_0 (Timeline|OutItem PlayFromStart)
                  (:Update
                    (Transformation|SetActorRelativeLocation (Variables|Default|GetItemLooted) (Math|Vector|MakeVector 0.0 0.0 (Math|Float|MapRangeClamped _newtrack_0 0.0 1.0 0.0 5e+01))))
                  (:Finished
                    (Variables|Default|SetLerpVectorBeginPos (Transformation|GetActorLocation (Variables|Default|GetItemLooted)))
                    (bind _newtrack_0_2 (Timeline|LerpToPlayer PlayFromStart)
                      (:Update
                        (Transformation|SetActorLocation (Variables|Default|GetItemLooted) (Math|Vector|Lerp(Vector) (Variables|Default|GetLerpVectorBeginPos) (Transformation|GetActorLocation (CallFunction|CastPlayer)) _newtrack_0_2) false false))
                      (:Finished
                        (Default|AddItem (Variables|Default|GetItemLooted))
                        (Rendering|SetVisibility (Variables|/Game/Game_Dev/Blueprints/GameplayScript/BP_ItemDrop.BP_ItemDrop_C|GetStaticMesh (Variables|Default|GetItemLooted)) false false)))))))))))))

(event EventBeginPlay
  ;[1 1 1] Loot system
  (Utilities|FlowControl|Delay 0.5)
  (if (!= (Utilities|Array|FindItem (Variables|/Game/Game_Dev/Blueprints/Player/BP_PlayerTest.BP_PlayerTest_C|GetInventory (CallFunction|CastPlayer)) (Variables|Default|GetObjectType)) -1)
    (Variables|Default|SetOpen true)
    (Transformation|SetRelativeRotation (Variables|Default|GetCoffre_Couvercle_coffe) (Math|Rotator|MakeRotator (Variables|Default|GetRotation%20coffre) 0.0 0.0) false false)
    (Development|PrintString "Hello")))

(fn ConstructionScript
  (bind _typeitem (Variables|OpenVariable|GetTypeItem))
  (bind _setitem (Variables|OpenVariable|GetSetItem))
  (bind _typeitem_2 (Variables|OpenVariable|GetTypeItem))
  (bind _setitem_2 (Variables|OpenVariable|GetSetItem))
  (bind _typeitem_3 (Variables|OpenVariable|GetTypeItem))
  (bind _setitem_3 (Variables|OpenVariable|GetSetItem))
  (bind _setitem_4 (Variables|OpenVariable|GetSetItem))
  (Components|StaticMesh|SetStaticMesh (Variables|Default|GetCoffre_Couvercle_coffe) (Variables|OpenVariable|GetStaticMeshCouvercle))
  (Components|StaticMesh|SetStaticMesh (Variables|Default|GetCoffre_Support_coffre) (Variables|OpenVariable|GetStaticMeshCoffre))
  (switch Utilities|FlowControl|Switch|SwitchonEnum_WGItem (Variables|OpenVariable|GetTypeItem)
    (:NewEnumerator0
      (switch Utilities|FlowControl|Switch|SwitchonEnum_SetItem _setitem_4
        (:NewEnumerator0
          (Variables|Default|SetObjectType (Utilities|Struct|MakeStruct_Object "Helmet" 3e+01 15.0 "/Game/UI/HUD/Stuff/casque_fer_Sprite.casque_fer_Sprite" _typeitem _setitem "/Game/Game_Dev/TestChangeMesh/Slasher/SK_Head_Slasher.SK_Head_Slasher")))
        (:NewEnumerator1
          (Variables|Default|SetObjectType (Utilities|Struct|MakeStruct_Object "Helmet" 1e+01 1e+01 "/Game/UI/HUD/Stuff/casque_bois__Sprite.casque_bois__Sprite" _typeitem _setitem "/Game/Game_Dev/TestChangeMesh/Paysan/SK_Head_Paysan.SK_Head_Paysan")))
        (:NewEnumerator2
          (Variables|Default|SetObjectType (Utilities|Struct|MakeStruct_Object "Helmet" 15.0 2e+01 "/Game/UI/HUD/Stuff/capuche_violette_Sprite.capuche_violette_Sprite" _typeitem _setitem "/Game/Game_Dev/TestChangeMesh/Mage/SK_Head_Mage.SK_Head_Mage")))))
    (:NewEnumerator1
      (switch Utilities|FlowControl|Switch|SwitchonEnum_SetItem _setitem_4
        (:NewEnumerator0
          (Variables|Default|SetObjectType (Utilities|Struct|MakeStruct_Object "Body" 3e+01 15.0 "/Game/UI/HUD/Stuff/Armure_fer_Sprite.Armure_fer_Sprite" _typeitem_2 _setitem_2 "/Game/Game_Dev/TestChangeMesh/Slasher/SK_Torso_Slasher.SK_Torso_Slasher")))
        (:NewEnumerator1
          (Variables|Default|SetObjectType (Utilities|Struct|MakeStruct_Object "Body" 1e+01 1e+01 "/Game/UI/HUD/Stuff/Plastron_bois_Sprite.Plastron_bois_Sprite" _typeitem_2 _setitem_2 "/Game/Game_Dev/TestChangeMesh/Paysan/SK_Torso_Paysan.SK_Torso_Paysan")))
        (:NewEnumerator2
          (Variables|Default|SetObjectType (Utilities|Struct|MakeStruct_Object "Body" 2e+01 4e+01 "/Game/UI/HUD/Stuff/Manteau_violet_Sprite.Manteau_violet_Sprite" _typeitem_2 _setitem_2 "/Game/Game_Dev/TestChangeMesh/Mage/SK_Torso_Mage.SK_Torso_Mage")))))
    (:NewEnumerator2
      (switch Utilities|FlowControl|Switch|SwitchonEnum_SetItem _setitem_4
        (:NewEnumerator0
          (Variables|Default|SetObjectType (Utilities|Struct|MakeStruct_Object "Broom" 4e+01 2e+01 "/Game/UI/HUD/Stuff/Balai_fer_Sprite1.Balai_fer_Sprite1" _typeitem_3 _setitem_3 0)))
        (:NewEnumerator1
          (Variables|Default|SetObjectType (Utilities|Struct|MakeStruct_Object "Broom" 1e+01 1e+01 "/Game/UI/HUD/Stuff/balai_bois_Sprite1.balai_bois_Sprite1" _typeitem_3 _setitem_3 0)))
        (:NewEnumerator2
          (Variables|Default|SetObjectType (Utilities|Struct|MakeStruct_Object "Broom" 15.0 4e+01 "/Game/UI/HUD/Stuff/Balai_Violet_Sprite1.Balai_Violet_Sprite1" _typeitem_3 _setitem_3 0)))))))