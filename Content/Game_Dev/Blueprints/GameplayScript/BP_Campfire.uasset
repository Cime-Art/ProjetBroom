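; BP_Campfire is a campfire actor that lights up once when LaunchNiagara is called, apparently serving as a checkpoint torch.
; A DoOnce gate fires the checkpoint Wwise sound, sets the Player_Life RTPC to 1.0 and activates the Niagara effect with a reset.
; A timeline then ramps the point light, scaling its curve by the Intensity variable.
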(event Custom|LaunchNiagara
  (Utilities|FlowControl|DoOnce false
    (:Completed
      (Class|AkGameplayStatics|PostEvent "/Game/WwiseAudio/Events/Default_Work_Unit/Props/Event_Play_Checkpoint_torch.Event_Play_Checkpoint_torch" self)
      (Class|AkGameplayStatics|SetRTPCValue "/Game/WwiseAudio/Game_Parameters/Default_Work_Unit/Player/Player_Life.Player_Life" 1.0)
      (Components|Activation|SetActive (Variables|Default|GetNiagara) true true)
      (bind _newtrack_0 (Timeline|Timeline_0 Play)
        (:Update
          (Rendering|Components|Light|SetIntensity (Variables|Default|GetPointLight) (* _newtrack_0 (Variables|Default|GetIntensity))))))))

(fn ConstructionScript)