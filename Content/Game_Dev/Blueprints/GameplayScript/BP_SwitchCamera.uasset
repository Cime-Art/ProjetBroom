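; BP_SwitchCamera is a trigger volume that blends the player's follow camera to a configured field of view.
; The first BP_PlayerTest overlap with its Box starts the Alpha timeline through a DoOnce that is never reset, at a rate set from Speed on BeginPlay.
; Each update remaps the track value between the camera's current FOV and the target, so the blend compounds from the live value.
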(event OnComponentBeginOverlap(Box)
  (params (OverlappedComponent :type Primitive%20Component%20Object%20Reference) (OtherActor :type Actor%20Object%20Reference) (OtherComp :type Primitive%20Component%20Object%20Reference) (OtherBodyIndex :type Integer) (bFromSweep :type Boolean) (SweepResult :type Hit%20Result%20Structure%20%28by%20ref%29))
  (bind _asbp_player_test (CallFunction|CastPlayer))
  (bind _followcamera (Variables|/Game/Game_Dev/Blueprints/Player/BP_PlayerTest.BP_PlayerTest_C|GetFollowCamera _asbp_player_test))
  (Utilities|Casting|CastToBP_PlayerTest OtherActor)
  (Utilities|FlowControl|DoOnce false
    (:Completed
      (bind _newtrack_0 (Timeline|Alpha PlayFromStart)
        (:Update
          (Utilities|IsValid _followcamera
            (:Is%20Valid
              (Camera|SetFieldOfView _followcamera (Math|Float|MapRangeClamped _newtrack_0 0.0 1.0 (Variables|/Script/Engine.CameraComponent|GetFieldOfView _followcamera) (Variables|Default|GetFieldOfView))))))))))

(event EventBeginPlay
  (Components|Timeline|SetPlayRate (Variables|CameraModifier|GetAlpha) (Variables|Default|GetSpeed)))

(fn ConstructionScript)