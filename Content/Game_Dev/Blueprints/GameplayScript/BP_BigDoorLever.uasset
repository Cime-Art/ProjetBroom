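; Big door lever that the player triggers once by hitting it with the broom during an attack.
; A box overlap starts the Rotate timeline, which spins the crank mesh two full turns with a Wwise sound.
; An event on that timeline plays the gate sound and starts a second timeline that moves the door spikes vertically, lerping from their current height to a fixed Z.
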(event OnComponentBeginOverlap(Box)
  (params (OverlappedComponent :type Primitive%20Component%20Object%20Reference) (OtherActor :type Actor%20Object%20Reference) (OtherComp :type Primitive%20Component%20Object%20Reference) (OtherBodyIndex :type Integer) (bFromSweep :type Boolean) (SweepResult :type Hit%20Result%20Structure%20%28by%20ref%29))
  (bind _sm_grandeporte_manivelle_low (Variables|Default|GetSM_GrandePorte_manivelle_low))
  (bind _sm_grandeporte_piques_low (Variables|Default|GetSM_GrandePorte_Piques_low))
  (bind _relativerotation (Variables|/Script/Engine.SceneComponent|GetRelativeRotation _sm_grandeporte_manivelle_low))
  (bind _relativelocation (Variables|/Script/Engine.SceneComponent|GetRelativeLocation _sm_grandeporte_piques_low))
  (Utilities|Casting|CastToBP_Broom OtherActor)
  (if (Variables|/Game/Game_Dev/Blueprints/Player/BP_PlayerTest.BP_PlayerTest_C|GetIsAttacking (CallFunction|CastPlayer))
    (Utilities|FlowControl|DoOnce false
      (:Completed
        (Class|AkGameplayStatics|PostEvent "/Game/WwiseAudio/Events/Default_Work_Unit/Level/Jail/Event_LeverRotate.Event_LeverRotate" (CallFunction|CastController))
        (bind _rotate (Timeline|Rotate PlayFromStart)
          (:Update
            (Transformation|SetRelativeRotation _sm_grandeporte_manivelle_low (Math|Rotator|MakeRotator (Math|Float|Lerp 0.0 7.2e+02 _rotate) (.pitch _relativerotation) (.yaw _relativerotation)) false false))
          (:Event
            (Class|AkGameplayStatics|PostEvent "/Game/WwiseAudio/Events/Default_Work_Unit/Level/Jail/Metal/Event_MetalGateJail.Event_MetalGateJail" (CallFunction|CastController))
            (bind _movement_z (Timeline|MovementSpick PlayFromStart)
              (:Update
                (Transformation|SetRelativeLocation _sm_grandeporte_piques_low (Math|Vector|MakeVector (.x _relativelocation) (.y _relativelocation) (Math|Float|Lerp (.z _relativelocation) 4e+01 _movement_z)) false false)))))))))

(event EventBeginPlay)

(fn ConstructionScript)