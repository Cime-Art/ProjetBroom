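; BP_BigDoorEndJail is the large jail-end door, opened once through its OpenDoor event.
; The Rotate timeline spins the crank mesh two full turns on roll, and its event track starts MovementSpick to move the spikes vertically.
; The spike Lerp starts from the current Z each update, so motion compounds rather than following the curve directly.
; The construction script caches the first BP_IA_Spider found, though these graphs never use it.
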(event Custom|OpenDoor
  (bind _sm_grandeporte_manivelle_low (Variables|Default|GetSM_GrandePorte_manivelle_low))
  (bind _sm_grandeporte_piques_low (Variables|Default|GetSM_GrandePorte_Piques_low))
  (bind _relativerotation (Variables|/Script/Engine.SceneComponent|GetRelativeRotation _sm_grandeporte_manivelle_low))
  (bind _relativelocation (Variables|/Script/Engine.SceneComponent|GetRelativeLocation _sm_grandeporte_piques_low))
  (Utilities|FlowControl|DoOnce false
    (:Completed
      (bind _rotate (Timeline|Rotate PlayFromStart)
        (:Update
          (Transformation|SetRelativeRotation _sm_grandeporte_manivelle_low (Math|Rotator|MakeRotator (Math|Float|Lerp 0.0 7.2e+02 _rotate) (.pitch _relativerotation) (.yaw _relativerotation)) false false))
        (:Event
          (bind _movement_z (Timeline|MovementSpick PlayFromStart)
            (:Update
              (Transformation|SetRelativeLocation _sm_grandeporte_piques_low (Math|Vector|MakeVector (.x _relativelocation) (.y _relativelocation) (Math|Float|Lerp (.z _relativelocation) 4e+01 _movement_z)) false false))))))))

(fn ConstructionScript
  (bind _outactors (Actor|GetAllActorsOfClass "/Game/Game_Dev/Blueprints/IA/Generals/Spider/Blueprint/BP_IA_Spider.BP_IA_Spider_C"))
  (Variables|Default|SetSpiderRef (Utilities|Array|Get(acopy) _outactors)))