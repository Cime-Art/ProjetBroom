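; Hanging pig carcass on a chain that swings and reacts to hits, and also drives tutorial steps by showing preview widgets or opening a door.
; Spell hits add a random impulse, play Wwise sounds and swap in an Immo or Poison material for four seconds.
; TakeHit applies a DoOnce-gated force on the chain, while physical contact triggers light-hit and squeak sounds.
; A per-tick trace spawns a very short-lived decal as a fake shadow.
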(event OnComponentHit(SkeletalMesh)
  (params (HitComponent :type Primitive%20Component%20Object%20Reference) (OtherActor :type Actor%20Object%20Reference) (OtherComp :type Primitive%20Component%20Object%20Reference) (NormalImpulse :type Vector :default "0, 0, 0") (Hit :type Hit%20Result%20Structure%20%28by%20ref%29))
  ;[1 1 1] get hit light
  (Utilities|FlowControl|Sequence
    (:then_0
      (Class|AkGameplayStatics|PostEvent "/Game/WwiseAudio/Events/Default_Work_Unit/Level/Tuto/Kitchen/Event_PigChain_GetHitLight.Event_PigChain_GetHitLight" self))
    (:then_1
      (Utilities|FlowControl|Delay 1.0)
      (Class|AkGameplayStatics|PostEvent "/Game/WwiseAudio/Events/Default_Work_Unit/Level/Tuto/Kitchen/Event_PigChainSqueak.Event_PigChainSqueak" self))))

(event Custom|StepPass
  (params (Index :type Integer))
  (Utilities|FlowControl|Delay 1.5)
  (switch int Index
    (:0
      (bind _returnvalue (UserInterface|CreateWidget "/Game/Game_Dev/Blueprints/Widget/Tuto/HUD_Tuto_Preview.HUD_Tuto_Preview_C" 0 "NewEnumerator1"))
      (UserInterface|Viewport|AddtoViewport _returnvalue 0))
    (:1
      (bind _returnvalue_2 (UserInterface|CreateWidget "/Game/Game_Dev/Blueprints/Widget/Tuto/HUD_Tuto_Preview.HUD_Tuto_Preview_C" 0 "NewEnumerator3"))
      (UserInterface|Viewport|AddtoViewport _returnvalue_2 0))
    (:2
      (bind _returnvalue_3 (UserInterface|CreateWidget "/Game/Game_Dev/Blueprints/Widget/Tuto/HUD_Tuto_Preview.HUD_Tuto_Preview_C" 0 "NewEnumerator4"))
      (UserInterface|Viewport|AddtoViewport _returnvalue_3 0))
    (:3
      (Default|OpenDoor (Variables|Default|GetBP_Door)))))

(event Custom|ResetForce
  (Utilities|FlowControl|DoOnce false) ; enters at Reset
)

(event Custom|TakeHit
  (params (Impact :type Vector))
  (Utilities|IsValid (Variables|Default|GetPhysicsConstraint)
    (:Is%20Valid
      (Utilities|FlowControl|DoOnce false
        (:Completed
          (Physics|AddForce (Variables|Default|GetSkeletalMesh) (* Impact -3e+03) "chaine29_skn" false)
          (Utilities|FlowControl|Delay 3.0)
          (CallFunction|ResetForce))))))

(event Custom|ChangeMat&Hit
  (params (TypeOfMat :type String))
  (bind _skeletalmesh (Variables|Default|GetSkeletalMesh))
  (Physics|AddImpulse (Variables|Default|GetSkeletalMesh) (Math|Vector|MakeVector (Math|Random|RandomFloatinRange -5e+04 5e+04) (Math|Random|RandomFloatinRange -5e+04 5e+04) 0.0) "joint14" false)
  (Class|AkGameplayStatics|PostEvent "/Game/WwiseAudio/Events/Default_Work_Unit/Level/Tuto/Kitchen/Event_PigChainSwing.Event_PigChainSwing" self)
  (switch string TypeOfMat
    (:Immo
      ;[1 1 1] get hit spell
      (Class|AkGameplayStatics|PostEvent "/Game/WwiseAudio/Events/Default_Work_Unit/Level/Tuto/Kitchen/Event_PigChain_GetHit.Event_PigChain_GetHit" self)
      (Rendering|Material|SetMaterial _skeletalmesh 1 "/Game/Game_Dev/Materials/Inst/M_SpellImmo_Inst.M_SpellImmo_Inst")
      (Utilities|FlowControl|Delay 4.0)
      (Rendering|Material|SetMaterial _skeletalmesh 1 (Variables|Default|GetMat_Carcass)))
    (:Poison
      (Class|AkGameplayStatics|PostEvent "/Game/WwiseAudio/Events/Default_Work_Unit/Level/Tuto/Kitchen/Event_PigChain_GetHit.Event_PigChain_GetHit" self)
      (Rendering|Material|SetMaterial (Variables|Default|GetSkeletalMesh) 1 "/Game/Game_ART/Graph/Tiling_Materials/ForBP/Acide_Inst.Acide_Inst")
      (Utilities|FlowControl|Delay 4.0)
      (Rendering|Material|SetMaterial (Variables|Default|GetSkeletalMesh) 1 (Variables|Default|GetMat_Carcass)))))

(event Custom|Spawn%20decal%20shadow
  (bind _skeletalmesh (Variables|Default|GetSkeletalMesh))
  (bind _returnvalue (Math|Vector|GetUpVector _skeletalmesh))
  (bind _returnvalue_2 (Transformation|GetWorldLocation _skeletalmesh))
  (bind (_x _y _z) (Math|Vector|BreakVector _returnvalue_2))
  (bind _outhit (Collision|LineTraceByChannel (Math|Vector|MakeVector _x _y _z) (+ (Math|Vector|MakeVector _x _y _z) (Math|Vector|SelectVector (* _returnvalue -1e+03) (* _returnvalue 1e+03) (> _z 0.0))) "TraceTypeQuery1" false 0 "None"))
  (Rendering|Decal|SpawnDecalatLocation "/Game/Game_Dev/Materials/Parents/ombre_player_Mat.ombre_player_Mat" "70.000000,70.000000,70.000000" (.impactpoint _outhit) "-90.000000,0.000000,0.000000" 0.0001))

(event EventBeginPlay
  (Utilities|FlowControl|Sequence
    (:then_0
      (Variables|Default|SetMat_Carcass (Utilities|Array|Get(acopy) (Rendering|Material|GetMaterials (Variables|Default|GetSkeletalMesh)) 1)))))

(event EventTick
  (params (DeltaSeconds :type Float%20%28single-precision%29))
  (CallFunction|SpawnDecalShadow))

(fn ConstructionScript)