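; BP_ItemDrop is an item pickup actor whose mesh is set from a variable in the construction script.
; AddItem adds its ObjectInfo to the player's inventory, copies that inventory to the game instance and shows a HUD popup with the item's logo and name.
; It then posts the Wwise magic chest pickup sound, waits briefly, stops its audio and destroys itself.
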(event Custom|Add%20Item
  (bind _objectinfo (Variables|Default|GetObjectInfo))
  (bind (_nameobj _lifegiving _managiving _logo) (Utilities|Struct|BreakStruct_Object _objectinfo))
  (Utilities|Array|Add (Variables|/Game/Game_Dev/Blueprints/Player/BP_PlayerTest.BP_PlayerTest_C|GetInventory (CallFunction|CastPlayer)) _objectinfo)
  (Variables|/Game/Game_Dev/Blueprints/GameSettings/BP_GameInstance.BP_GameInstance_C|SetInventory (CallFunction|CastGameInstance) (Variables|/Game/Game_Dev/Blueprints/Player/BP_PlayerTest.BP_PlayerTest_C|GetInventory (CallFunction|CastPlayer)))
  (Default|AfficherLaPOPUP (Variables|/Game/Game_Dev/Blueprints/Player/BP_PlayerTest.BP_PlayerTest_C|GetWG_HUD (CallFunction|CastPlayer)) _logo (Utilities|Text|ToText(String) _nameobj) "NewEnumerator3")
  (Class|AkGameplayStatics|PostEvent "/Game/WwiseAudio/Events/Default_Work_Unit/Props/MagicChest/Event_MagicChestPickup.Event_MagicChestPickup" self 0 0 0 true)
  (Utilities|FlowControl|Delay 2.0)
  (Class|AkGameplayStatics|StopActor self)
  (Actor|DestroyActor))

(fn ConstructionScript
  (Components|StaticMesh|SetStaticMesh (Variables|Default|GetStaticMesh) (Variables|Default|GetMesh)))