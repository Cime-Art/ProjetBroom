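; BP_Lever is a lever that triggers a linked Event object when activated.
; ActivateEvent plays the RotateLever timeline, lerping the Lever mesh's roll from its current value toward a fixed angle on each update.
; When the timeline finishes, it calls Interact on Event if that reference is valid.
; The construction script swaps the base and lever meshes according to OnTheGround.
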(event Custom|ActivateEvent
  (bind _lever (Variables|Default|GetLever))
  (bind _event (Variables|OpenVariables|GetEvent))
  (bind _relativerotation (Variables|/Script/Engine.SceneComponent|GetRelativeRotation _lever))
  (bind _rotation (Timeline|RotateLever PlayFromStart)
    (:Update
      (Transformation|SetRelativeRotation _lever (Math|Rotator|MakeRotator (Math|Float|Lerp (.roll _relativerotation) 6e+01 _rotation) (.pitch _relativerotation) (.yaw _relativerotation)) false false))
    (:Finished
      (Utilities|IsValid _event
        (:Is%20Valid
          (Default|Interact _event))))))

(fn ConstructionScript
  (Components|StaticMesh|SetStaticMesh (Variables|Default|GetSocleLever) (select (Variables|OpenVariables|GetOnTheGround) "/Game/Game_ART/Graph/Objects/Jail/Lever/lever_export_SM_BaseLever02.lever_export_SM_BaseLever02" "/Game/Game_ART/Graph/Objects/Jail/Lever/lever_export_SM_BaseLever01.lever_export_SM_BaseLever01"))
  (Components|StaticMesh|SetStaticMesh (Variables|Default|GetLever) (select (Variables|OpenVariables|GetOnTheGround) "/Game/Game_ART/Graph/Objects/Jail/Lever/lever_export_SM_Lever02.lever_export_SM_Lever02" "/Game/Game_ART/Graph/Objects/Jail/Lever/lever_export_SM_Lever01.lever_export_SM_Lever01")))