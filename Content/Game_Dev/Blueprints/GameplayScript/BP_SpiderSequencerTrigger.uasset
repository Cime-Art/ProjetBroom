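; BP_SpiderSequencerTrigger is a one-shot trigger that stages the spider's jail wall destruction when BP_PlayerTest enters its collision component.
; It plays the destruction animation on the referenced door, lowers every referenced pillar, calls StopActor on the door and destroys it one second later.
; Player input is disabled and re-enabled within the same execution, with no delay between, so the sequence does not hold the player.
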(event OnComponentBeginOverlap(CollisionComponent)
  (params (OverlappedComponent :type Primitive%20Component%20Object%20Reference) (OtherActor :type Actor%20Object%20Reference) (OtherComp :type Primitive%20Component%20Object%20Reference) (OtherBodyIndex :type Integer) (bFromSweep :type Boolean) (SweepResult :type Hit%20Result%20Structure%20%28by%20ref%29))
  (bind _controller (CallFunction|CastController))
  (bind _asbp_player_test (Utilities|Casting|CastToBP_PlayerTest OtherActor))
  (Utilities|FlowControl|DoOnce false
    (:Completed
      (Input|DisableInput _asbp_player_test _controller)
      (bind _bp_destrudoorref (Variables|Default|GetBp_DestruDoorRef)
        (:then
          (Components|Animation|PlayAnimation (Variables|/Game/Game_Dev/Blueprints/GameplayScript/BP_WallDestru_Parent.BP_WallDestru_Parent_C|GetSkeletalMesh _bp_destrudoorref) "/Game/Game_ART/Graph/Objects/Jail/WAll_Destru/Wall_Jail_Destru_Spider_Anim.Wall_Jail_Destru_Spider_Anim" false)
          (for _array_element (Variables|Default|GetBP_PillierRef)
            (Default|DownPilar _array_element))
          (Input|EnableInput _asbp_player_test _controller)
          (Class|AkGameplayStatics|StopActor _bp_destrudoorref)
          (Utilities|FlowControl|Delay 1.0)
          (Actor|DestroyActor _bp_destrudoorref))
        (:else)))))

(event EventBeginPlay)

(event Collision|EventActorBeginOverlap
  (params (OtherActor :type Actor%20Object%20Reference)))

(event EventTick
  (params (DeltaSeconds :type Float%20%28single-precision%29)))

(fn ConstructionScript)