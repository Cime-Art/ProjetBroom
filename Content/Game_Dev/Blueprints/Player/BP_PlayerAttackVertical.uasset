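; Anim notify state for the player's vertical attack, applying weapon hits during the animation window.
; Each tick sphere-traces between the weapon sockets and dispatches hits by class to trash mobs, carcasses, destructible meshes, bananas, spiders and levers.
; Trash mobs and spiders take double player damage; a player-held array prevents repeat damage on trash mobs, which also get impulse direction and Niagara effects.
; Surface types feed the player's material-hit response.
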(fn ReceivedNotifyTick
  (params (MeshComp :type Skeletal%20Mesh%20Component%20Object%20Reference) (Animation :type Anim%20Sequence%20Base%20Object%20Reference) (FrameDeltaTime :type Float%20%28single-precision%29))
  (bind _returnvalue (Game|GetPlayerCharacter MeshComp))
  (bind _asbp_player_test (CallFunction|CastPlayer MeshComp))
  (bind _asbp_player_test_2 (Utilities|Casting|CastToBP_PlayerTest _returnvalue))
  (bind _ia_trashmob_attac_system (Variables|/Game/Game_Dev/Blueprints/Player/BP_PlayerTest.BP_PlayerTest_C|GetIA_Trashmob_Attac_System _asbp_player_test_2))
  (bind _infoplayer (Variables|/Game/Game_Dev/Blueprints/Player/BP_PlayerTest.BP_PlayerTest_C|GetInfoPlayer _asbp_player_test_2))
  (bind _returnvalue_2 (* (.damage _infoplayer) 2))
  (bind _returnvalue_3 (Math|Conversions|ToFloat(Integer) _returnvalue_2))
  (bind _outhits (Collision|MultiSphereTraceByChannel MeshComp (Transformation|GetSocketLocation MeshComp "Socket_Weapon") (Transformation|GetSocketLocation MeshComp "Socket_Weapon_End") 4e+01 "TraceTypeQuery1" false (Utilities|Array|MakeArray (CallFunction|CastPlayer MeshComp)) "None"))
  (bind _array_element (Utilities|Array|ForEachLoopwithBreak _outhits)
    (:LoopBody
      (Utilities|FlowControl|Sequence
        (:then_0
          (bind _asbp_ia_trash_mob (Utilities|Casting|CastToBP_IA_TrashMob (.HitActor (Collision|BreakHitResult _array_element)))
            (:then
              (Default|HitMaterial _asbp_player_test (Variables|/Script/Engine.PhysicalMaterial|GetSurfaceType (.PhysMat (Collision|BreakHitResult _array_element))))
              (Variables|/Game/Game_Dev/Blueprints/IA/Trashmob/Blueprints/BP_IA_TrashMob.BP_IA_TrashMob_C|SetImpulseDirection _asbp_ia_trash_mob (Math|Vector|Normalize (Math|Vector|MakeVector (.x (* (.ImpactNormal (Collision|BreakHitResult _array_element)) -1)) (.y (* (.ImpactNormal (Collision|BreakHitResult _array_element)) -1)) 0.0)))
              (if (not (Utilities|Array|ContainsItem _ia_trashmob_attac_system _asbp_ia_trash_mob))
                (Utilities|Array|Add _ia_trashmob_attac_system _asbp_ia_trash_mob)
                (Game|Damage|ApplyDamage _asbp_ia_trash_mob _returnvalue_3 0 0)
                (Niagara|SpawnSystematLocation _asbp_ia_trash_mob (select (== _asbp_ia_trash_mob "/Game/Game_Dev/Blueprints/IA/Generals/Blueprints/BP_IA_Generals_CraneDeFeu.BP_IA_Generals_CraneDeFeu") "/Game/Game_Dev/FX/NiagaraSystems/NS_Hit.NS_Hit" "/Game/Game_Dev/FX/NiagaraSystems/NS_Hit_Trashmob.NS_Hit_Trashmob") (.ImpactPoint (Collision|BreakHitResult _array_element)) (Math|Rotator|MakeRotator (Math|Random|RandomFloatinRange -6e+01 6e+01) (Math|Random|RandomFloatinRange -6e+01 6e+01) (Math|Random|RandomFloatinRange -6e+01 6e+01)) "0.300000,0.300000,0.300000")
                (return true)))
            (:CastFailed
              (bind _asbp_carcass (Utilities|Casting|CastToBP_Carcass (.HitActor (Collision|BreakHitResult _array_element)))
                (:then
                  (Default|TakeHit _asbp_carcass (Math|Vector|Normalize (Math|Vector|MakeVector (.x (* (.ImpactNormal (Collision|BreakHitResult _array_element)) -1)) (.y (* (.ImpactNormal (Collision|BreakHitResult _array_element)) -1)) 0.0))))
                (:CastFailed
                  (bind _asbp_destructible_mesh (Utilities|Casting|CastToBp_DestructibleMesh (.HitActor (Collision|BreakHitResult _array_element)))
                    (:then
                      (Default|DestroyMesh _asbp_destructible_mesh (Math|Vector|Normalize (Math|Vector|MakeVector (.x (* (.ImpactNormal (Collision|BreakHitResult _array_element)) -1)) (.y (* (.ImpactNormal (Collision|BreakHitResult _array_element)) -1)) 0.0)))
                      (return true))
                    (:CastFailed
                      (bind _asbp_banana (Utilities|Casting|CastToBP_Banana (.HitActor (Collision|BreakHitResult _array_element)))
                        (:then
                          (Class|INTAnimBpIA|GetHit(Message) _asbp_banana))
                        (:CastFailed
                          (bind _asbp_ia_spider (Utilities|Casting|CastToBP_IA_Spider (.HitActor (Collision|BreakHitResult _array_element)))
                            (:then
                              (Default|TakeDamage _asbp_ia_spider _returnvalue_3))
                            (:CastFailed
                              (bind _asbp_lever (Utilities|Casting|CastToBP_Lever (.HitActor (Collision|BreakHitResult _array_element))))
                              (Default|ActivateEvent _asbp_lever))))))))))))
        (:then_1
          (if (.bBlockingHit (Collision|BreakHitResult _array_element))
            (Default|HitMaterial _asbp_player_test (Variables|/Script/Engine.PhysicalMaterial|GetSurfaceType (.PhysMat (Collision|BreakHitResult _array_element))))))))))