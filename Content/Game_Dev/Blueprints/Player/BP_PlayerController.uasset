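; Player controller that handles menu input, pausing and switching between gamepad and mouse.
; Any key press sets the gamepad flag and cursor visibility from the key type.
; P or PauseMenu toggles the pause widget in-game when allowed and no inventory exists; OpenInventaire opens the player menu paused, or calls its close when the pause widget exists.
; UI actions forward as messages to WGRef, validated as on screen.
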(event EventBeginPlay
  (Variables|Default|SetbShowMouseCursor true)
  (Input|SetInputModeGameandUI self 0 "DoNotLock" false))

(event Input|KeyboardEvents|AnyKey
  (params (Key :type Key%20Structure))
  (:Pressed
    (if (Class|KismetInputLibrary|KeyIsGamepadKey Key)
      (Variables|Default|SetGamepad? true)
      (Variables|Default|SetbShowMouseCursor false)
      (Class|PlayerController|SetMouseLocation)
      (else
        (Variables|Default|SetGamepad? false)
        (Variables|Default|SetbShowMouseCursor true)))))

(event Custom|Resume
  (Game|SetGamePaused false)
  (Widget|RemovefromParent (Variables|Default|GetWg_Pause))
  (Variables|Default|SetWg_Pause 0))

(event Input|ActionEvents|InputActionUI_ChangeItemLeft
  (params (Key :type Key%20Structure))
  (:Pressed
    (bind _wg_ref (CallFunction|WGRefValid?))
    (Class|INTWidgetInterface|UIChangeItemLeft(Message) _wg_ref)))

(event Input|ActionEvents|InputActionUI_ChangeItemRight
  (params (Key :type Key%20Structure))
  (:Pressed
    (bind _wg_ref (CallFunction|WGRefValid?))
    (Class|INTWidgetInterface|UIChangeItemRight(Message) _wg_ref)))

(event Input|ActionEvents|InputActionUI_SkipMainMenu
  (params (Key :type Key%20Structure))
  (:Pressed
    (bind _wg_ref (CallFunction|WGRefValid?))
    (Class|INTWidgetInterface|UISkipMainMenu(Message) _wg_ref)))

(event Input|ActionEvents|InputActionOpenInventaire
  (params (Key :type Key%20Structure))
  (:Pressed
    (Utilities|IsValid (Variables|Default|GetWg_Pause)
      (:Is%20Valid
        (Default|CloseMenu (Variables|Default|GetWG_Inventaire)))
      (:Is%20Not%20Valid
        (bind _returnvalue (UserInterface|CreateWidget "/Game/Game_Dev/Blueprints/Widget/Menu/WG_PlayerMenu.WG_PlayerMenu_C"))
        (bind _output_get (Variables|Default|SetWG_Inventaire _returnvalue))
        (UserInterface|Viewport|AddtoViewport _output_get 0)
        (Game|SetGamePaused true)))))

(event Input|ActionEvents|InputActionPauseMenu
  (params (Key :type Key%20Structure))
  (:Pressed
    (if (Variables|/Game/Game_Dev/Blueprints/GameSettings/BP_GameInstance.BP_GameInstance_C|GetIsInGame (CallFunction|CastGameInstance))
      (if (Variables|Default|GetCanResumeWithBtn)
        (Utilities|IsValid (Variables|Default|GetWG_Inventaire)
          (:Is%20Not%20Valid
            (Utilities|IsValid (Variables|Default|GetWg_Pause)
              (:Is%20Valid
                (Game|SetGamePaused false)
                (Widget|RemovefromParent (Variables|Default|GetWg_Pause))
                (Variables|Default|SetWg_Pause 0))
              (:Is%20Not%20Valid
                (Game|SetGamePaused true)
                (bind _returnvalue (UserInterface|CreateWidget "/Game/Game_Dev/Blueprints/Widget/Menu/WG_PauseMenu.WG_PauseMenu_C"))
                (bind _output_get (Variables|Default|SetWg_Pause _returnvalue))
                (UserInterface|Viewport|AddtoViewport _output_get 0)))))))))

(event Input|ActionEvents|InputActionUI_BtnA
  (params (Key :type Key%20Structure))
  (:Pressed
    (bind _wg_ref (CallFunction|WGRefValid?))
    (Class|INTWidgetInterface|UIBtnA(Message) _wg_ref)))

(event Input|ActionEvents|InputActionUI_ButtonApply
  (params (Key :type Key%20Structure))
  (:Pressed
    (bind _wg_ref (CallFunction|WGRefValid?))
    (Class|INTWidgetInterface|UIButtonApply(Message) _wg_ref)))

(event Input|ActionEvents|InputActionUI_ChangeMenuLeft
  (params (Key :type Key%20Structure))
  (:Pressed
    (bind _wg_ref (CallFunction|WGRefValid?))
    (Class|INTWidgetInterface|UIChangeMenuLeft(Message) _wg_ref)))

(event Input|ActionEvents|InputActionUI_ChangeMenuRight
  (params (Key :type Key%20Structure))
  (:Pressed
    (bind _wg_ref (CallFunction|WGRefValid?))
    (Class|INTWidgetInterface|UIChangeMenuRight(Message) _wg_ref)))

(event Input|ActionEvents|InputActionUI_DetectAuto
  (params (Key :type Key%20Structure))
  (:Pressed
    (bind _wg_ref (CallFunction|WGRefValid?))
    (Class|INTWidgetInterface|UIDetectAuto(Message) _wg_ref)))

(event Input|ActionEvents|InputActionUI_Return
  (params (Key :type Key%20Structure))
  (:Pressed
    (bind _wg_ref (CallFunction|WGRefValid?))
    (Class|INTWidgetInterface|UIReturn(Message) _wg_ref)))

(event Input|KeyboardEvents|P
  (params (Key :type Key%20Structure))
  (:Pressed
    (if (Variables|/Game/Game_Dev/Blueprints/GameSettings/BP_GameInstance.BP_GameInstance_C|GetIsInGame (CallFunction|CastGameInstance))
      (if (Variables|Default|GetCanResumeWithBtn)
        (Utilities|IsValid (Variables|Default|GetWG_Inventaire)
          (:Is%20Not%20Valid
            (Utilities|IsValid (Variables|Default|GetWg_Pause)
              (:Is%20Valid
                (Game|SetGamePaused false)
                (Widget|RemovefromParent (Variables|Default|GetWg_Pause))
                (Variables|Default|SetWg_Pause 0))
              (:Is%20Not%20Valid
                (Game|SetGamePaused true)
                (bind _returnvalue (UserInterface|CreateWidget "/Game/Game_Dev/Blueprints/Widget/Menu/WG_PauseMenu.WG_PauseMenu_C"))
                (bind _output_get (Variables|Default|SetWg_Pause _returnvalue))
                (UserInterface|Viewport|AddtoViewport _output_get 0)))))))))

(fn ConstructionScript)

(fn WGRefValid?
  (bind _wg_ref (Variables|Default|GetWG_Ref)
    (:then
      (if (UserInterface|Viewport|IsinViewport _wg_ref)
        (return _wg_ref)
        (else
          (Variables|Default|SetWG_Ref 0))))
    (:else)))