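; Player-related Blueprint function library that gathers shared helpers for access, input display and footstep audio.
; Cast helpers return the typed player controller, game instance and player pawn.
; Input helpers turn key names into short button labels and check whether a key is mapped to an action.
; GetTextureGround traces below the player, maps the physical surface to a Wwise switch and posts the footstep event, which IsJump can suppress.
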(fn CastController
  (bind _asbp_player_controller (Utilities|Casting|CastToBP_PlayerController (Game|GetPlayerController 0)))
  (return _asbp_player_controller))

(fn CastGameInstance
  (bind _asbp_game_instance (Utilities|Casting|CastToBP_GameInstance (Game|GetGameInstance)))
  (return _asbp_game_instance))

(fn CastPlayer
  (bind _asbp_player_test (Utilities|Casting|CastToBP_PlayerTest (Game|Player|GetPlayerPawn 0)))
  (return _asbp_player_test))

(fn ReturnRealInput
  (params (Selection :type Name))
  (switch name Selection
    (:Default
      (LocalVariables|SetReturnInput Selection))
    (:Gamepad%20Left%20Trigger
      (LocalVariables|SetReturnInput "LT"))
    (:Gamepad%20Right%20Trigger
      (LocalVariables|SetReturnInput "RT"))
    (:Gamepad%20Left%20Shoulder
      (LocalVariables|SetReturnInput "LB"))
    (:Gamepad%20Right%20Shoulder
      (LocalVariables|SetReturnInput "RB"))
    (:Gamepad%20Face%20Button%20Bottom
      (LocalVariables|SetReturnInput "A"))
    (:Gamepad%20Face%20Button%20Right
      (LocalVariables|SetReturnInput "B"))
    (:Gamepad%20Face%20Button%20Left
      (LocalVariables|SetReturnInput "X"))
    (:Gamepad%20Face%20Button%20Top
      (LocalVariables|SetReturnInput "Y"))
    (:Gamepad%20Special%20Left
      (LocalVariables|SetReturnInput "OPTION"))
    (:Gamepad%20Special%20Right
      (LocalVariables|SetReturnInput "START"))
    (:Gamepad%20Right%20Thumbstick%20Button
      (LocalVariables|SetReturnInput "R3"))
    (:Escape
      (LocalVariables|SetReturnInput "ESC")))
  (return (LocalVariables|GetReturnInput)))

(fn CheckifKeyIsMapped
  (params (Action%20Name :type Name) (Input :type Key%20Event%20Structure%20%28by%20ref%29))
  (return (Utilities|Array|ContainsItem (Class|InputSettings|GetActionMappingbyName (Class|InputSettings|GetInputSettings) Action%20Name) (Utilities|Struct|MakeInputActionKeyMapping Action%20Name false false false false (Class|KismetInputLibrary|GetKey Input)))))

(fn GetTextureGround
  (params (PlayerRef :type BP%20Player%20Test%20Object%20Reference) (IsJump :type Boolean))
  (bind _returnvalue (Game|Player|GetPlayerPawn 0))
  (bind _returnvalue_2 (Transformation|GetActorLocation _returnvalue))
  (LocalVariables|SetRefPlayer PlayerRef)
  (bind (_outhit _returnvalue_3) (Collision|LineTraceByChannel 0 _returnvalue_2 (- _returnvalue_2 "0, 0,150.000000") "TraceTypeQuery1" false 0 "None"))
  (if _returnvalue_3
    (if (!= (Utilities|Select :Index (Variables|/Script/Engine.PhysicalMaterial|GetSurfaceType (.PhysMat (Collision|BreakHitResult _outhit))) :SurfaceType_Default "/Game/WwiseAudio/Switches/Default_Work_Unit/Player/FTPS_Ground_Texture/FTPS_Ground_Texture-Grass.FTPS_Ground_Texture-Grass" :SurfaceType1 "/Game/WwiseAudio/Switches/Default_Work_Unit/Player/FTPS_Ground_Texture/FTPS_Ground_Texture-Grass.FTPS_Ground_Texture-Grass" :SurfaceType2 "/Game/WwiseAudio/Switches/Default_Work_Unit/Player/FTPS_Ground_Texture/FTPS_Ground_Texture-Rock.FTPS_Ground_Texture-Rock" :SurfaceType3 "/Game/WwiseAudio/Switches/Default_Work_Unit/Player/FTPS_Ground_Texture/FTPS_Ground_Texture-Wood.FTPS_Ground_Texture-Wood" :SurfaceType4 "/Game/WwiseAudio/Switches/Default_Work_Unit/Player/FTPS_Ground_Texture/FTPS_Ground_Texture-Bones.FTPS_Ground_Texture-Bones" :SurfaceType5 "/Game/WwiseAudio/Switches/Default_Work_Unit/Player/FTPS_Ground_Texture/FTPS_Ground_Texture-Marble.FTPS_Ground_Texture-Marble" :SurfaceType6 "/Game/WwiseAudio/Switches/Default_Work_Unit/Player/FTPS_Ground_Texture/FTPS_Ground_Texture-HollowWood.FTPS_Ground_Texture-HollowWood" :SurfaceType7 "/Game/WwiseAudio/Switches/Default_Work_Unit/Player/FTPS_Ground_Texture/FTPS_Ground_Texture-Dirt.FTPS_Ground_Texture-Dirt" :SurfaceType8 "/Game/WwiseAudio/Switches/Default_Work_Unit/Player/FTPS_Ground_Texture/FTPS_Ground_Texture-Metal.FTPS_Ground_Texture-Metal" :SurfaceType9 0 :SurfaceType10 0 :SurfaceType11 0 :SurfaceType12 0 :SurfaceType13 0 :SurfaceType14 "/Game/WwiseAudio/Switches/Default_Work_Unit/Player/FTPS_Ground_Texture/FTPS_Ground_Texture-Water.FTPS_Ground_Texture-Water" :SurfaceType15 "/Game/WwiseAudio/Switches/Default_Work_Unit/Player/FTPS_Ground_Texture/FTPS_Ground_Texture-Sand.FTPS_Ground_Texture-Sand") (LocalVariables|GetSwitch%20Mat))
      (bind _output_get (LocalVariables|SetSwitch%20Mat (Utilities|Select :Index (Variables|/Script/Engine.PhysicalMaterial|GetSurfaceType (.PhysMat (Collision|BreakHitResult _outhit))) :SurfaceType_Default "/Game/WwiseAudio/Switches/Default_Work_Unit/Player/FTPS_Ground_Texture/FTPS_Ground_Texture-Grass.FTPS_Ground_Texture-Grass" :SurfaceType1 "/Game/WwiseAudio/Switches/Default_Work_Unit/Player/FTPS_Ground_Texture/FTPS_Ground_Texture-Grass.FTPS_Ground_Texture-Grass" :SurfaceType2 "/Game/WwiseAudio/Switches/Default_Work_Unit/Player/FTPS_Ground_Texture/FTPS_Ground_Texture-Rock.FTPS_Ground_Texture-Rock" :SurfaceType3 "/Game/WwiseAudio/Switches/Default_Work_Unit/Player/FTPS_Ground_Texture/FTPS_Ground_Texture-Wood.FTPS_Ground_Texture-Wood" :SurfaceType4 "/Game/WwiseAudio/Switches/Default_Work_Unit/Player/FTPS_Ground_Texture/FTPS_Ground_Texture-Bones.FTPS_Ground_Texture-Bones" :SurfaceType5 "/Game/WwiseAudio/Switches/Default_Work_Unit/Player/FTPS_Ground_Texture/FTPS_Ground_Texture-Marble.FTPS_Ground_Texture-Marble" :SurfaceType6 "/Game/WwiseAudio/Switches/Default_Work_Unit/Player/FTPS_Ground_Texture/FTPS_Ground_Texture-HollowWood.FTPS_Ground_Texture-HollowWood" :SurfaceType7 "/Game/WwiseAudio/Switches/Default_Work_Unit/Player/FTPS_Ground_Texture/FTPS_Ground_Texture-Dirt.FTPS_Ground_Texture-Dirt" :SurfaceType8 "/Game/WwiseAudio/Switches/Default_Work_Unit/Player/FTPS_Ground_Texture/FTPS_Ground_Texture-Metal.FTPS_Ground_Texture-Metal" :SurfaceType9 0 :SurfaceType10 0 :SurfaceType11 0 :SurfaceType12 0 :SurfaceType13 0 :SurfaceType14 "/Game/WwiseAudio/Switches/Default_Work_Unit/Player/FTPS_Ground_Texture/FTPS_Ground_Texture-Water.FTPS_Ground_Texture-Water" :SurfaceType15 "/Game/WwiseAudio/Switches/Default_Work_Unit/Player/FTPS_Ground_Texture/FTPS_Ground_Texture-Sand.FTPS_Ground_Texture-Sand")))
      (Class|AkGameplayStatics|SetSwitch _output_get (LocalVariables|GetRefPlayer))
      (if IsJump
        _
        (else
          (Class|AkGameplayStatics|PostEvent "/Game/WwiseAudio/Events/Default_Work_Unit/Player/FTPS/Event_FTPS.Event_FTPS" (LocalVariables|GetRefPlayer) :!label _label)))
      (else
        (goto _label)))
    (return)))