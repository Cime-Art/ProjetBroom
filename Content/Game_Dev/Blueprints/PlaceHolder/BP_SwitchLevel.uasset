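; Placeholder level-transition trigger that moves the player to the level named in its Level variable.
; The BorderPop volume slides HUD top and bottom borders through a timeline, reversed on exit.
; The ChangeLevel volume stops the tutorial music and animates a HUD screen wipe.
; When the wipe finishes, it optionally saves player info with the new level and a zeroed vector via the GameInstance, then opens the level.
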(event OnComponentBeginOverlap(BorderPop)
  (params (OverlappedComponent :type Primitive%20Component%20Object%20Reference) (OtherActor :type Actor%20Object%20Reference) (OtherComp :type Primitive%20Component%20Object%20Reference) (OtherBodyIndex :type Integer) (bFromSweep :type Boolean) (SweepResult :type Hit%20Result%20Structure%20%28by%20ref%29))
  (bind _asbp_player_test (CallFunction|CastPlayer))
  (bind _wg_hud (Variables|/Game/Game_Dev/Blueprints/Player/BP_PlayerTest.BP_PlayerTest_C|GetWG_HUD _asbp_player_test))
  (Utilities|Casting|CastToBP_PlayerTest OtherActor)
  (bind (_direction _topborder _botborder) (Timeline|Border Play)
    (:Update
      (Class|Widget|SetRenderTranslation (Variables|/Game/Game_Dev/Blueprints/Widget/PlayerInterface/WG_Hud.WG_Hud_C|GetBotBorder_1 _wg_hud) (Math|Vector2D|MakeVector2D 0.0 _botborder))
      (Class|Widget|SetRenderTranslation (Variables|/Game/Game_Dev/Blueprints/Widget/PlayerInterface/WG_Hud.WG_Hud_C|GetTopBorder _wg_hud) (Math|Vector2D|MakeVector2D 0.0 _topborder)))))

(event OnComponentEndOverlap(BorderPop)
  (params (OverlappedComponent :type Primitive%20Component%20Object%20Reference) (OtherActor :type Actor%20Object%20Reference) (OtherComp :type Primitive%20Component%20Object%20Reference) (OtherBodyIndex :type Integer))
  (bind _asbp_player_test (CallFunction|CastPlayer))
  (bind _wg_hud (Variables|/Game/Game_Dev/Blueprints/Player/BP_PlayerTest.BP_PlayerTest_C|GetWG_HUD _asbp_player_test))
  (Utilities|Casting|CastToBP_PlayerTest OtherActor)
  (bind (_direction _topborder _botborder) (Timeline|Border Reverse)
    (:Update
      (Class|Widget|SetRenderTranslation (Variables|/Game/Game_Dev/Blueprints/Widget/PlayerInterface/WG_Hud.WG_Hud_C|GetBotBorder_1 _wg_hud) (Math|Vector2D|MakeVector2D 0.0 _botborder))
      (Class|Widget|SetRenderTranslation (Variables|/Game/Game_Dev/Blueprints/Widget/PlayerInterface/WG_Hud.WG_Hud_C|GetTopBorder _wg_hud) (Math|Vector2D|MakeVector2D 0.0 _topborder)))))

(event OnComponentBeginOverlap(ChangeLevel)
  (params (OverlappedComponent :type Primitive%20Component%20Object%20Reference) (OtherActor :type Actor%20Object%20Reference) (OtherComp :type Primitive%20Component%20Object%20Reference) (OtherBodyIndex :type Integer) (bFromSweep :type Boolean) (SweepResult :type Hit%20Result%20Structure%20%28by%20ref%29))
  (bind _asbp_player_test (CallFunction|CastPlayer))
  (bind _gameinstance (CallFunction|CastGameInstance))
  (bind _gameinstance_2 (CallFunction|CastGameInstance))
  (bind _wg_hud (Variables|/Game/Game_Dev/Blueprints/Player/BP_PlayerTest.BP_PlayerTest_C|GetWG_HUD _asbp_player_test))
  (bind _middle (Variables|/Game/Game_Dev/Blueprints/Widget/PlayerInterface/WG_Hud.WG_Hud_C|GetMiddle _wg_hud))
  (bind _asbp_player_test_2 (Utilities|Casting|CastToBP_PlayerTest OtherActor))
  (switch name (.currentlevel (Variables|/Game/Game_Dev/Blueprints/Player/BP_PlayerTest.BP_PlayerTest_C|GetInfoPlayer _asbp_player_test_2))
    (:Default
      _)
    (:level0_TutoDef
      _))
  (Default|StopMusique (CallFunction|CastGameInstance) "/Game/WwiseAudio/Events/Default_Work_Unit/Music/Event_Stop_Musique_Tuto_Playlist.Event_Stop_Musique_Tuto_Playlist")
  (bind _newtrack_0 (Timeline|AllScreen Play)
    (:Update
      (Widget|SetRenderOpacity _middle 1.0)
      (Class|Widget|SetRenderTranslation _middle (Math|Vector2D|MakeVector2D _newtrack_0 0.0)))
    (:Finished
      (if (Variables|Default|GetSave?)
        (Variables|/Game/Game_Dev/Blueprints/GameSettings/BP_GameInstance.BP_GameInstance_C|SetInfoPlayer _gameinstance_2 (Utilities|Struct|MakeStruct_InfoPlayer (.hpplayer (Variables|/Game/Game_Dev/Blueprints/GameSettings/BP_GameInstance.BP_GameInstance_C|GetInfoPlayer _gameinstance_2)) (.maxhp (Variables|/Game/Game_Dev/Blueprints/GameSettings/BP_GameInstance.BP_GameInstance_C|GetInfoPlayer _gameinstance_2)) (.manaplayer (Variables|/Game/Game_Dev/Blueprints/GameSettings/BP_GameInstance.BP_GameInstance_C|GetInfoPlayer _gameinstance_2)) (.maxmana (Variables|/Game/Game_Dev/Blueprints/GameSettings/BP_GameInstance.BP_GameInstance_C|GetInfoPlayer _gameinstance_2)) (Math|Vector|MakeVector 0.0 0.0 0.0) (.currentlife (Variables|/Game/Game_Dev/Blueprints/GameSettings/BP_GameInstance.BP_GameInstance_C|GetInfoPlayer _gameinstance_2)) (.currentcontinue (Variables|/Game/Game_Dev/Blueprints/GameSettings/BP_GameInstance.BP_GameInstance_C|GetInfoPlayer _gameinstance_2)) (Variables|Default|GetLevel)))
        (Variables|/Game/Game_Dev/Blueprints/GameSettings/BP_GameInstance.BP_GameInstance_C|SetSwitchLevel (CallFunction|CastGameInstance) true)
        (Default|SaveData _gameinstance (Variables|/Game/Game_Dev/Blueprints/GameSettings/BP_GameInstance.BP_GameInstance_C|GetInfoPlayer _gameinstance))
        (Utilities|FlowControl|Delay 1.0))
      (Game|OpenLevel(byName) (Variables|Default|GetLevel)))))

(event EventBeginPlay
  (Components|Timeline|SetPlayRate (Variables|Default|GetBorder) (Variables|Default|GetBorderPopSpeed)))

(fn ConstructionScript)