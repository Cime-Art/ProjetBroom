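; Preview actor that renders bestiary creatures via a SceneCapture2D showing only itself, with a slowly spinning spring arm.
; Switch takes a row index into the bestiary DataTable and applies its mesh, AnimBP and scale.
; Skeleton melee and ranged entries get random socketed gear plus a weapon, using static mesh components pooled in the construction script.
; Tick calls CaptureScene while the game is paused, and the mesh is tickable during pause.
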(event Custom|Switch
  (params (Dimension%201 :type Integer))
  (bind _mobsname (Variables|Default|GetMobsName))
  (bind _mesh (Variables|Character|GetMesh))
  (bind _output (Utilities|Array|Get(acopy) _mobsname Dimension%201))
  (bind _returnvalue (Utilities|GetDataTableRow "/Game/Game_Dev/Blueprints/Datatable/Datatable_Bestiaire.Datatable_Bestiaire" _output)
    (:then
      (if (and (Utilities|IsValid (.sk _returnvalue)) (Utilities|IsValidClass (.animbp _returnvalue)))
        (Class|SkinnedMeshComponent|SetSkeletalMesh _mesh (.sk _returnvalue) true)
        (Class|SkeletalMeshComponent|SetAnimClass _mesh (.animbp _returnvalue))
        (Transformation|SetRelativeScale3D (Variables|Character|GetMesh) (.scale _returnvalue))
        (for _array_element (Variables|Default|GetStuff)
          (Components|StaticMesh|SetStaticMesh _array_element 0))
        (CallFunction|SetStuff _output)))))

(event Custom|SetStuff
  (params (MobName :type Name))
  (bind _stuff (Variables|Default|GetStuff))
  (bind _returnvalue (Utilities|Array|LastIndex _stuff))
  (bind _output (Utilities|Array|Get(acopy) _stuff _returnvalue))
  (switch name MobName
    (:SkeletonCaC
      (CallFunction|RandomStuff (Variables|Default|GetStuffCaC))
      (Components|StaticMesh|SetStaticMesh _output "/Game/Game_ART/Graph/Objects/Jail/Weapons_Skeleton/SM_SkeletonSword.SM_SkeletonSword")
      (Transformation|AttachComponentToComponent _output (Variables|Character|GetMesh) "Weapon" "KeepRelative" "KeepRelative" "KeepRelative" true))
    (:SkeletonDist
      (CallFunction|RandomStuff (Variables|Default|GetStuffDist))
      (Components|StaticMesh|SetStaticMesh _output "/Game/Game_ART/Graph/Objects/Jail/Weapons_Skeleton/SM_SkeletonCrossbow.SM_SkeletonCrossbow")
      (Transformation|AttachComponentToComponent _output (Variables|Character|GetMesh) "Weapon_Crossbow" "KeepRelative" "KeepRelative" "KeepRelative" true))))

(event Custom|RandomStuff
  (params (Stuff :type Map%20of%20Names%20to%20Objects))
  ;[1 1 1] Stuff
  (bind _keys (Utilities|Map|Keys Stuff))
  (bind _values (Utilities|Map|Values Stuff))
  (for (_array_element _array_index) _values
    (if (<= (Math|Random|RandomFloat) 0.5)
      (Components|StaticMesh|SetStaticMesh (Utilities|Array|Get(acopy) (Variables|Default|GetStuff) _array_index) _array_element)
      (Transformation|AttachComponentToComponent (Utilities|Array|Get(acopy) (Variables|Default|GetStuff) _array_index) (Variables|Character|GetMesh) (Utilities|Array|Get(acopy) _keys _array_index) "KeepRelative" "KeepRelative" "KeepRelative" true)
      (Collision|SetCollisionEnabled (Utilities|Array|Get(acopy) (Variables|Default|GetStuff) _array_index) "NoCollision"))))

(event EventBeginPlay
  (Class|ActorComponent|SetTickablewhenPaused (Variables|Character|GetMesh) true)
  (bind _outrownames (DataTable|GetDataTableRowNames "/Game/Game_Dev/Blueprints/Datatable/Datatable_Bestiaire.Datatable_Bestiaire"))
  (Variables|Default|SetMobsName _outrownames)
  (CallFunction|Switch (Variables|Default|GetIndex)))

(event Collision|EventActorBeginOverlap
  (params (OtherActor :type Actor%20Object%20Reference)))

(event EventTick
  (params (DeltaSeconds :type Float%20%28single-precision%29))
  (Transformation|AddRelativeRotation (Variables|Default|GetSpringArm) "0,0.500000, 0" false false)
  (if (Game|IsGamePaused)
    (Rendering|SceneCapture|CaptureScene (Variables|Default|GetSceneCaptureComponent2D) :!class /Script/Engine.SceneCaptureComponent2D)))

(fn ConstructionScript
  (Variables|/Script/Engine.SceneCaptureComponent|SetShowOnlyActors (Variables|Default|GetSceneCaptureComponent2D) (Utilities|Array|MakeArray self))
  (bind _keys (Utilities|Map|Keys (Variables|Default|GetStuffCaC)))
  (bind _keys_2 (Utilities|Map|Keys (Variables|Default|GetStuffDist)))
  (for _index (range 0 (+ (Math|Integer|Max(Integer) (Utilities|Array|LastIndex _keys) (Utilities|Array|LastIndex _keys_2)) 1))
    (bind _returnvalue (AddComponent|AddStaticMeshComponent false))
    (Utilities|Array|Add (Variables|Default|GetStuff) _returnvalue)))