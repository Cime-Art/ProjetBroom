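; BP_PlayerRender is a player preview actor that renders a character with a broom through a SceneCaptureComponent2D, which captures only this actor.
; The construction script makes head and torso follow Mesh as master pose and attaches the broom to its weapon socket.
; Tick rotates the SpringArm by a fixed per-frame step and manually captures the scene while the game is paused, with Mesh set to tick during pause.
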(event EventBeginPlay
  (Class|ActorComponent|SetTickablewhenPaused (Variables|Character|GetMesh) true))

(event EventTick
  (params (DeltaSeconds :type Float%20%28single-precision%29))
  (Transformation|AddRelativeRotation (Variables|Default|GetSpringArm) "0,0.500000, 0" false false)
  (if (Game|IsGamePaused)
    (Rendering|SceneCapture|CaptureScene (Variables|Default|GetSceneCaptureComponent2D) :!class /Script/Engine.SceneCaptureComponent2D)))

(fn ConstructionScript
  (Variables|/Script/Engine.SceneCaptureComponent|SetShowOnlyActors (Variables|Default|GetSceneCaptureComponent2D) (Utilities|Array|MakeArray self))
  (Class|SkinnedMeshComponent|SetMasterPoseComponent (Variables|Default|GetSK_Head) (Variables|Character|GetMesh) true)
  (Transformation|AttachComponentToComponent (Variables|Default|GetBroom) (Variables|Character|GetMesh) "Socket_Weapon" "KeepRelative" "KeepRelative" "KeepRelative" true))