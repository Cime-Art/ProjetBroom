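; Moving platform that carries an attached enemy arena along a spline, respawning its mobs as the ride starts.
; Shake plays a camera shake, jitters the mesh and rotates two "mouth" pieces, then after a delay a timeline offsets the platform's height.
; Tick then advances it in XY along the spline, with Niagara active, until the end marks the arena cleared.
; ResetAll stops motion, restores the position and resets the arena.
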(event Custom|Shake
  (bind _returnvalue (Math|Random|RandomFloatinRange -4.0 4.0))
  (bind _scenesmouth (Variables|Default|GetSceneSmouth))
  (bind _scenesmouth1 (Variables|Default|GetSceneSmouth1))
  (bind _returnvalue_2 (Transformation|GetWorldRotation _scenesmouth1))
  (bind _returnvalue_3 (Transformation|GetWorldRotation _scenesmouth))
  ;[1 1 1] Comment
  (Camera|PlayWorldCameraShake "/Game/Game_Dev/Blueprints/Player/BP_CameraShake.BP_CameraShake_C" (Transformation|GetWorldLocation (Variables|/Game/Game_Dev/Blueprints/Player/BP_PlayerTest.BP_PlayerTest_C|GetFollowCamera (CallFunction|CastPlayer))) 0.0 5e+02)
  (Variables|Default|SetStopSpawn true)
  (Timeline|Timeline_0 PlayFromStart
    (:Update
      (Variables|Default|SetRandomX _returnvalue)
      (Variables|Default|SetRandomY _returnvalue)
      (Transformation|SetRelativeLocation (Variables|Default|GetStaticMesh) (Math|Vector|MakeVector (Variables|Default|GetRandomX) (Variables|Default|GetRandomY) (.z (Transformation|GetWorldLocation (Variables|Default|GetSceneMovement)))) false false)
      (bind (_direction _scene _sceneleft) (Timeline|Timeline_1 Play)
        (:Update
          (Utilities|FlowControl|Sequence
            (:then_0
              (Transformation|SetWorldRotation _scenesmouth (Math|Rotator|MakeRotator _scene (.pitch _returnvalue_3) (.yaw _returnvalue_3)) false false))
            (:then_1
              (Transformation|SetWorldRotation _scenesmouth1 (Math|Rotator|MakeRotator _sceneleft (.pitch _returnvalue_2) (.yaw _returnvalue_2)) false false))))))
    (:Finished
      (Utilities|FlowControl|Delay (Variables|Default|GetDelayBeforeFalling))
      (CallFunction|MovingZ))))

(event Custom|Moving%20Z
  (bind _scenemovement (Variables|Default|GetSceneMovement))
  (bind _scenesmouth (Variables|Default|GetSceneSmouth))
  (bind _scenesmouth1 (Variables|Default|GetSceneSmouth1))
  (bind _returnvalue (Transformation|GetWorldRotation _scenesmouth1))
  (bind _returnvalue_2 (Transformation|GetWorldRotation _scenesmouth))
  (bind _returnvalue_3 (Transformation|GetWorldLocation _scenemovement))
  ;[1 1 1] Comment
  (Variables|Default|SetOldZAxis (.z (Transformation|GetWorldLocation (Variables|Default|GetSceneMovement))))
  (bind _movingz (Timeline|MovingZ PlayFromStart)
    (:Update
      (if (not (Variables|Default|GetReset))
        (Transformation|SetWorldLocation (Variables|Default|GetSceneMovement) (Math|Vector|MakeVector (.x _returnvalue_3) (.y _returnvalue_3) (+ (Variables|Default|GetOldZAxis) (Math|Float|MapRangeClamped _movingz 0.0 1.0 0.0 (Variables|OpenVariable|GetZAXIS)))) false false)))
    (:Finished
      (Variables|Default|SetMovePlatform? true)
      (Variables|Default|SetStopSpawn false)
      (Default|RespawnMob (Variables|Default|GetbpArena))
      (Components|Activation|SetActive (Variables|Default|GetNiagara) true true)
      (bind (_direction _scene _sceneleft) (Timeline|Timeline_1 Play)
        (:Update
          (Utilities|FlowControl|Sequence
            (:then_0
              (Transformation|SetWorldRotation _scenesmouth (Math|Rotator|MakeRotator _scene (.pitch _returnvalue_2) (.yaw _returnvalue_2)) false false))
            (:then_1
              (Transformation|SetWorldRotation _scenesmouth1 (Math|Rotator|MakeRotator _sceneleft (.pitch _returnvalue) (.yaw _returnvalue)) false false))))))))

(event EventBeginPlay
  ;[1 1 1] Comment
  (Components|Timeline|SetPlayRate (Variables|Default|GetTimeline_0) (Variables|OpenVariable|GetShakingTime))
  (Components|Timeline|SetPlayRate (Variables|Default|GetTimeline_1) (Variables|OpenVariable|GetRotationY)))

(event EventResetAll
  ;[1 1 1] Comment
  (Variables|Default|SetReset true)
  (Variables|Default|SetMovePlatform? false)
  (Audio|Components|Audio|Stop (Variables|Default|GetTimeline_1))
  (Audio|Components|Audio|Stop (Variables|Default|GetMovingZ))
  (Transformation|SetRelativeLocation (Variables|Default|GetSceneMovement) "0, 0, 0" false false)
  (Components|Timeline|SetPlaybackPosition (Variables|Default|GetMovingZ) 0.0 false true)
  (Default|ResetArena (Variables|Default|GetbpArena))
  (Variables|Default|SetReset false)
  (Components|Activation|SetActive (Variables|Default|GetNiagara) false false))

(event EventTick
  (params (DeltaSeconds :type Float%20%28single-precision%29))
  (bind _spline (Variables|Default|GetSpline))
  ;[1 1 1] Comment
  (if (Variables|Default|GetMovePlatform?)
    (Variables|Default|SetDistance%20Along%20Spline (+ (* DeltaSeconds (Variables|OpenVariable|Getspeed)) (Variables|Default|GetDistance%20Along%20Spline)))
    (Transformation|SetWorldLocation (Variables|Default|GetSceneMovement) (Math|Vector|MakeVector (.x (Spline|GetLocationatDistanceAlongSpline _spline (Variables|Default|GetDistance%20Along%20Spline) "World")) (.y (Spline|GetLocationatDistanceAlongSpline _spline (Variables|Default|GetDistance%20Along%20Spline) "World")) (.z (Transformation|GetWorldLocation (Variables|Default|GetSceneMovement)))) false false)
    (if (>= (Variables|Default|GetDistance%20Along%20Spline) (Spline|GetSplineLength _spline))
      (Variables|Default|SetMovePlatform? false)
      (Variables|/Game/Game_Dev/Blueprints/Trap/BP_Arena.BP_Arena_C|SetCleared (Variables|Default|GetbpArena) true)
      (Components|Activation|SetActive (Variables|Default|GetNiagara) false false)
      (Audio|Components|Audio|Stop (Variables|Default|GetTimeline_1)))))

(fn ConstructionScript
  (bind _bparena (Variables|Default|GetbpArena))
  (Transformation|AttachComponentToComponent _bparena (Variables|Default|GetStaticMesh) "None" "KeepRelative" "SnapToTarget" "KeepWorld" true)
  (Transformation|SetActorRelativeLocation _bparena "0,0.000000,400.000000")
  (Variables|/Game/Game_Dev/Blueprints/Trap/BP_Arena.BP_Arena_C|SetSpawn (Variables|Default|GetbpArena) true))