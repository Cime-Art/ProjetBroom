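; BP_Platforme_Pizza is a moving platform that shuttles back and forth along its local Y axis, pausing at each end.
; The construction script applies a configurable mesh, and BeginPlay sets the timeline play rate and starts movement.
; The Movement timeline lerps the mesh's relative Y between zero and Distance.
; When it finishes, EventMovement waits DelayBeforeMoving, then calls itself with the direction flipped, looping endlessly.
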(event Custom|EventMovement
  (params (Begin :type Boolean))
  (bind _staticmesh (Variables|Default|GetStaticMesh))
  (bind _relativelocation (Variables|/Script/Engine.SceneComponent|GetRelativeLocation _staticmesh))
  ;[1 1 1] Movement
  (if Begin
    (bind _movement (Timeline|Movement PlayFromStart)
      (:Update
        (Transformation|SetRelativeLocation _staticmesh (Math|Vector|MakeVector (.x _relativelocation) (Math|Float|Lerp 0.0 (Variables|OpenVariables|GetDistance) _movement) (.z _relativelocation)) false false))
      (:Finished
        (Utilities|FlowControl|Delay (Variables|OpenVariables|GetDelayBeforeMoving))
        (CallFunction|EventMovement (not Begin))))
    (else
      (Timeline|Movement ReverseFromEnd))))

(event EventBeginPlay
  ;[1 1 1] Initialise
  (Components|Timeline|SetPlayRate (Variables|Default|GetMovement) (Variables|OpenVariables|GetPlayRateMovement))
  (CallFunction|EventMovement true))

(fn ConstructionScript
  (Components|StaticMesh|SetStaticMesh (Variables|Default|GetStaticMesh) (Variables|OpenVariables|GetMesh)))