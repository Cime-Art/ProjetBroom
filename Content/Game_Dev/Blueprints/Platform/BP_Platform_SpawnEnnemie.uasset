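; Moving platform that carries an attached BpArena and triggers its enemy respawn as it travels.
; Shake jitters the mesh via timeline, waits, then a second timeline shifts the platform vertically by ZAXIS.
; It then respawns the arena's mobs and Tick moves it along a spline in XY, marking the arena Cleared at the end.
; ResetAll returns the platform to its relative origin and resets the arena.
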(event Custom|Shake
  (bind _returnvalue (Math|Random|RandomFloatinRange -4.0 4.0))
  ;[1 1 1] Comment
  (Variables|Default|SetStopSpawn true)
  (Timeline|Timeline_0 PlayFromStart
    (:Update
      (Variables|Default|SetRandomX _returnvalue)
      (Variables|Default|SetRandomY _returnvalue)
      (Transformation|SetRelativeLocation (Variables|Default|GetStaticMesh) (Math|Vector|MakeVector (Variables|Default|GetRandomX) (Variables|Default|GetRandomY) 0.0) false false))
    (:Finished
      (Utilities|FlowControl|Delay (Variables|Default|GetDelayBeforeFalling))
      (CallFunction|MovingZ))))

(event Custom|Moving%20Z
  (bind _scenemovement (Variables|Default|GetSceneMovement))
  (bind _returnvalue (Transformation|GetWorldLocation _scenemovement))
  ;[1 1 1] Comment
  (Variables|Default|SetOldZAxis (.z (Transformation|GetWorldLocation (Variables|Default|GetSceneMovement))))
  (bind _movingz (Timeline|MovingZ PlayFromStart)
    (:Update
      (if (not (Variables|Default|GetReset))
        (Transformation|SetWorldLocation (Variables|Default|GetSceneMovement) (Math|Vector|MakeVector (.x _returnvalue) (.y _returnvalue) (+ (Variables|Default|GetOldZAxis) (Math|Float|MapRangeClamped _movingz 0.0 1.0 0.0 (Variables|Default|GetZAXIS)))) false false)))
    (:Finished
      (Variables|Default|SetMovePlatform? true)
      (Variables|Default|SetStopSpawn false)
      (Default|RespawnMob (Variables|Default|GetbpArena)))))

(event EventBeginPlay
  ;[1 1 1] Comment
  (Components|Timeline|SetPlayRate (Variables|Default|GetTimeline_0) (Variables|Default|GetShakingTime)))

(event EventResetAll
  ;[1 1 1] Comment
  (Variables|Default|SetReset true)
  (Variables|Default|SetMovePlatform? false)
  (Audio|Components|Audio|Stop (Variables|Default|GetMovingZ))
  (Transformation|SetRelativeLocation (Variables|Default|GetSceneMovement) "0, 0, 0" false false)
  (Components|Timeline|SetPlaybackPosition (Variables|Default|GetMovingZ) 0.0 false true)
  (Default|ResetArena (Variables|Default|GetbpArena))
  (Variables|Default|SetReset false))

(event EventTick
  (params (DeltaSeconds :type Float%20%28single-precision%29))
  (bind _spline (Variables|Default|GetSpline))
  ;[1 1 1] Comment
  (if (Variables|Default|GetMovePlatform?)
    (Variables|Default|SetDistance%20Along%20Spline (+ (* DeltaSeconds (Variables|Default|Getspeed)) (Variables|Default|GetDistance%20Along%20Spline)))
    (Transformation|SetWorldLocation (Variables|Default|GetSceneMovement) (Math|Vector|MakeVector (.x (Spline|GetLocationatDistanceAlongSpline _spline (Variables|Default|GetDistance%20Along%20Spline) "World")) (.y (Spline|GetLocationatDistanceAlongSpline _spline (Variables|Default|GetDistance%20Along%20Spline) "World")) (.z (Transformation|GetWorldLocation (Variables|Default|GetSceneMovement)))) false false)
    (if (>= (Variables|Default|GetDistance%20Along%20Spline) (Spline|GetSplineLength _spline))
      (Variables|Default|SetMovePlatform? false)
      (Variables|/Game/Game_Dev/Blueprints/Trap/BP_Arena.BP_Arena_C|SetCleared (Variables|Default|GetbpArena) true))))

(fn ConstructionScript
  (bind _bparena (Variables|Default|GetbpArena))
  (Transformation|AttachComponentToComponent _bparena (Variables|Default|GetStaticMesh) "None" "KeepRelative" "SnapToTarget" "KeepWorld" true)
  (Transformation|SetActorRelativeLocation _bparena "0,0.000000,400.000000")
  (Variables|/Game/Game_Dev/Blueprints/Trap/BP_Arena.BP_Arena_C|SetSpawn (Variables|Default|GetbpArena) true))