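; Acid platform actor that shakes, waits, then moves its mesh vertically toward MaxHeight, either on play or when BP_PlayerTest first overlaps its box.
; A Shake timeline jitters X/Y, then after a delay the MovingPlatform timeline drives Z through the same location update.
; Loop repeats the sequence; otherwise movement stops near the top.
; ResetAll restores the start state and re-arms the trigger, using a Reset flag to block pending moves.
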(event OnComponentBeginOverlap(Box)
  (params (OverlappedComponent :type Primitive%20Component%20Object%20Reference) (OtherActor :type Actor%20Object%20Reference) (OtherComp :type Primitive%20Component%20Object%20Reference) (OtherBodyIndex :type Integer) (bFromSweep :type Boolean) (SweepResult :type Hit%20Result%20Structure%20%28by%20ref%29))
  (Utilities|Casting|CastToBP_PlayerTest OtherActor)
  (if (not (Variables|OpenVariable|GetLaunchOnPlay?))
    (Utilities|FlowControl|DoOnce false
      (:Completed
        (Development|PrintString "Hello")
        (CallFunction|LaunchPlatform)))))

(event Custom|LaunchPlatform
  (bind _returnvalue (Math|Random|RandomFloatinRange -2.0 2.0))
  (Timeline|Shake PlayFromStart
    (:Update
      (Variables|Default|SetRandomX _returnvalue)
      (Variables|Default|SetRandomY _returnvalue)
      (Transformation|SetRelativeLocation (Variables|Default|GetStaticMesh) (Math|Vector|MakeVector (Variables|Default|GetRandomX) (Variables|Default|GetRandomY) (Math|Float|MapRangeClamped (stale _movingz) 0.0 1.0 0.0 (Variables|OpenVariable|GetmaxHeight))) false false :!label _label)
      (if (and (>= (stale _movingz) 0.99) (not (Variables|OpenVariable|GetLoop?)))
        (Audio|Components|Audio|Stop (Variables|Default|GetMovingPlatform))))
    (:Finished
      (Variables|Default|SetReset false)
      (Utilities|FlowControl|Delay (Variables|OpenVariable|GetDelayBeforeMoving))
      (if (not (Variables|Default|GetReset))
        (bind _movingz (Timeline|MovingPlatform PlayFromStart)
          (:Update
            (goto _label))
          (:Finished
            (if (Variables|OpenVariable|GetLoop?)
              (CallFunction|LaunchPlatform))))))))

(event Custom|InitializePlatform
  (Components|Timeline|SetPlayRate (Variables|Default|GetShake) (Variables|OpenVariable|GetShaking%20Time))
  (Components|Timeline|SetPlayRate (Variables|Default|GetMovingPlatform) (Variables|OpenVariable|GetSpeed))
  (if (Variables|OpenVariable|GetLaunchOnPlay?)
    (CallFunction|LaunchPlatform)))

(event EventResetAll
  (Utilities|FlowControl|Delay 0.2)
  (Variables|Default|SetReset true)
  (Audio|Components|Audio|Stop (Variables|Default|GetShake))
  (Audio|Components|Audio|Stop (Variables|Default|GetMovingPlatform))
  (Transformation|SetRelativeLocation (Variables|Default|GetStaticMesh) "0, 0, 0" false false)
  (Components|Timeline|SetPlaybackPosition (Variables|Default|GetShake) 0.0 false true)
  (Components|Timeline|SetPlaybackPosition (Variables|Default|GetMovingPlatform) 0.0 false true)
  (CallFunction|InitializePlatform)
  (Utilities|FlowControl|DoOnce false) ; enters at Reset
)

(event EventBeginPlay
  (CallFunction|InitializePlatform))

(event EventTick
  (params (DeltaSeconds :type Float%20%28single-precision%29))
  (|CallParentFunction DeltaSeconds) ; This node is disabled and will not be called.\nDrag off pins to build functionality.
)

(event Collision|EventActorBeginOverlap
  (params (OtherActor :type Actor%20Object%20Reference))
  (|CallParentFunction OtherActor) ; This node is disabled and will not be called.\nDrag off pins to build functionality.
)

(fn ConstructionScript
  (|CallParentFunction)
  (Components|StaticMesh|SetStaticMesh (Variables|Default|GetStaticMesh) (Variables|OpenVariable|GetMesh)))