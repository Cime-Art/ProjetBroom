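; Collapsing bridge platform that shakes and breaks apart after BP_PlayerTest enters its trigger.
; A DoOnce-gated overlap waits a delay, then posts a Wwise event and starts the Shake timeline, randomly jittering the skeletal mesh.
; When shaking ends, the mesh animation plays while the Destru timeline drives material dissolve and disables five collision boxes one by one.
; ResetAll restores animation, dissolve, collision and the trigger gate.
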(event OnComponentBeginOverlap(Trigger)
  (params (OverlappedComponent :type Primitive%20Component%20Object%20Reference) (OtherActor :type Actor%20Object%20Reference) (OtherComp :type Primitive%20Component%20Object%20Reference) (OtherBodyIndex :type Integer) (bFromSweep :type Boolean) (SweepResult :type Hit%20Result%20Structure%20%28by%20ref%29))
  (Utilities|Casting|CastToBP_PlayerTest OtherActor)
  (Utilities|FlowControl|DoOnce false
    (:Completed
      (Utilities|FlowControl|Delay (Variables|OpenVariables|GetDelayBeforeShaking))
      (CallFunction|BEGINSHAKE)
      (Class|AkGameplayStatics|PostEventatLocation "/Game/WwiseAudio/Events/Default_Work_Unit/Level/Jail/Event_PlatformDestructionVoid.Event_PlatformDestructionVoid" "0, 0, 0" "0, 0, 0"))))

(event Custom|BEGIN_SHAKE
  (bind _returnvalue (Math|Random|RandomFloatinRange -2.0 2.0))
  (bind _skeletalmesh (Variables|Default|GetSkeletalMesh))
  (Timeline|Shake PlayFromStart
    (:Update
      (Variables|Default|SetRandomX _returnvalue)
      (Variables|Default|SetRandomY _returnvalue)
      (Transformation|SetRelativeLocation _skeletalmesh (Math|Vector|MakeVector (Variables|Default|GetRandomX) (.y (Variables|/Script/Engine.SceneComponent|GetRelativeLocation _skeletalmesh)) (Variables|Default|GetRandomY)) false false))
    (:Finished
      (Audio|Components|Audio|Play (Variables|Default|GetSkeletalMesh) false)
      (bind _dissolve (Timeline|Destru PlayFromStart)
        (:Update
          (Rendering|Material|SetScalarParameterValueonMaterials (Variables|Default|GetSkeletalMesh) "Dissolve" _dissolve))
        (:Destroy
          (Collision|SetCollisionEnabled (Utilities|Array|Get(acopy) (Variables|Default|GetTabBox) (Variables|Default|Getindex)) "NoCollision")
          (Math|Integer|IncrementInt (Variables|Default|Getindex)))))))

(event Collision|EventActorBeginOverlap
  (params (OtherActor :type Actor%20Object%20Reference))
  (|CallParentFunction OtherActor) ; This node is disabled and will not be called.\nDrag off pins to build functionality.
)

(event EventTick
  (params (DeltaSeconds :type Float%20%28single-precision%29))
  (|CallParentFunction DeltaSeconds) ; This node is disabled and will not be called.\nDrag off pins to build functionality.
)

(event EventBeginPlay
  (Components|Timeline|SetPlayRate (Variables|Default|GetShake) (Variables|OpenVariables|GetPlayRateShake))
  (Components|Timeline|SetPlayRate (Variables|Default|GetDestru) (Variables|OpenVariables|GetPlayRateDestru)))

(event EventResetAll
  (bind _destru (Variables|Default|GetDestru))
  (if (Audio|Components|Audio|IsPlaying (Variables|Default|GetShake))
    (Audio|Components|Audio|Stop (Variables|Default|GetShake)))
  (if (Audio|Components|Audio|IsPlaying _destru)
    (Audio|Components|Audio|Stop _destru))
  (Audio|Components|Audio|Stop (Variables|Default|GetSkeletalMesh))
  (Components|Animation|SetPosition (Variables|Default|GetSkeletalMesh) 0.0 true)
  (Rendering|Material|SetScalarParameterValueonMaterials (Variables|Default|GetSkeletalMesh) "Dissolve" 1.5)
  (Variables|Default|Setindex 0)
  (for _array_element (Variables|Default|GetTabBox)
    (Collision|SetCollisionEnabled _array_element "QueryAndPhysics"))
  (Utilities|FlowControl|DoOnce false) ; enters at Reset
)

(fn ConstructionScript
  (|CallParentFunction)
  (Variables|Default|SetInitialScale (.y (Variables|/Script/Engine.BoxComponent|GetBoxExtent (Variables|Default|GetBox))))
  (Variables|Default|SetTabBox (Utilities|Array|MakeArray (Variables|Default|GetBox4) (Variables|Default|GetBox3) (Variables|Default|GetBox2) (Variables|Default|GetBox1) (Variables|Default|GetBox))))