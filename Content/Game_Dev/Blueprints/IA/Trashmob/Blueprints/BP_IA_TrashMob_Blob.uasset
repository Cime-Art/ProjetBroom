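; Blob trash-mob enemy that runs its own behavior tree and splits into smaller blobs when it dies.
; Tick switches walk speed between moving and near-standstill from CanMoveBlob, using paired DoOnce gates to apply each change once.
; Once dead, Divide spawns two half-scale copies at its location, with the size guard reading the blob returned by GetActorOfClass rather than itself.
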(event Custom|Divide
  ;[1 1 1] Divide
  (if (Variables|Default|Getisdead)
    (bind _returnvalue (Actor|GetActorOfClass "BP_IA_TrashMob_Blob_C"))
    (if (not (Math|Vector|Equal(Vector) (Transformation|GetActorScale3D _returnvalue) "0.500000,0.500000,0.500000" 0.0001))
      (Utilities|FlowControl|DoOnce false
        (:Completed
          (for _index (range 0 1)
            (bind _returnvalue_2 (AI|SpawnAIFromClass "BP_IA_TrashMob_Blob_C" "/Game/Game_Dev/Blueprints/IA/Trashmob/BehaviorTree_Blackboard/BT_IA_BLOB.BT_IA_BLOB" (Transformation|GetActorLocation) "0, 0, 0" false 0))
            (bind _output_get (Variables|Default|SetMiniBlobRef _returnvalue_2))
            (Transformation|SetActorScale3D _output_get "0.500000,0.500000,0.500000")))))))

(event EventBeginPlay
  (|CallParentFunction)
  (Default|ChangeBehaviorTree (.AsIA%20Controller%20Trashmob (Utilities|Casting|CastToIA_Controller_Trashmob (AI|GetAIController self))) "/Game/Game_Dev/Blueprints/IA/Trashmob/BehaviorTree_Blackboard/BT_IA_BLOB.BT_IA_BLOB"))

(event EventTick
  (params (DeltaSeconds :type Float%20%28single-precision%29))
  (bind _charactermovement (Variables|Character|GetCharacterMovement))
  (|CallParentFunction DeltaSeconds)
  (Utilities|FlowControl|Sequence
    (:then_0
      (CallFunction|Divide))
    (:then_1
      (if (Variables|Default|GetCanMoveBlob)
        (Utilities|FlowControl|Sequence
          (:then_0
            (Utilities|FlowControl|DoOnce false :!label _label
              (:Completed
                (Variables|/Script/Engine.CharacterMovementComponent|SetMaxWalkSpeed _charactermovement 3e+02))))
          (:then_1
            (goto _label_2 Reset)))
        (else
          (Utilities|FlowControl|Sequence
            (:then_0
              (goto _label Reset))
            (:then_1
              (Utilities|FlowControl|DoOnce false :!label _label_2
                (:Completed
                  (Variables|/Script/Engine.CharacterMovementComponent|SetMaxWalkSpeed _charactermovement 0.1))))))))))

(fn ConstructionScript
  (|CallParentFunction))