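; Trash mob enemy character with a health bar widget, normal and big attacks, and a dissolve effect when spawned or killed.
; Player perception or damage alerts it and its Arena, while seen, hit and stunned states feed its AI blackboard.
; It handles poison ticks, falls and an immobilize spell that swaps its material and freezes animation.
; Lethal hits launch a ragdoll, or shatter a destructible mesh if stunned.
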(event OnTargetPerceptionUpdated(AIPerception)
  (params (Actor :type Actor%20Object%20Reference) (Stimulus :type AI%20Stimulus%20Structure))
  ;[1 1 1] Seen?
  (Utilities|Casting|CastToBP_PlayerTest Actor)
  (if (not (Variables|Default|Getisdead))
    (if (not (ScalableFloat|GetValueasBool (AI|GetBlackboard 0) (Utilities|Name|MakeLiteralName "Seen?")))
      (Utilities|IsValid (Variables|OpenVariable|GetArena)
        (:Is%20Valid
          (Default|SetSeen (Variables|OpenVariable|GetArena)))
        (:Is%20Not%20Valid
          _))
      (AI|Components|Blackboard|SetValueasBool (AI|GetBlackboard 0) (Utilities|Name|MakeLiteralName "Seen?") true)
      (Variables|/Script/Engine.CharacterMovementComponent|SetMaxWalkSpeed (Variables|Character|GetCharacterMovement) (Variables|OpenVariable|GetSpeed)))))

(event Custom|StartBigAttack
  ;[1 1 1] BigAttack
  (if (Math|Boolean|ANDBoolean (not (Variables|Default|GetIsHit?)) (not (Variables|Default|Getisdead)) (not (Variables|Default|GetIsBigAttacking?)) (not (Variables|Default|GetSpawned?)))
    (Class|INTAnimBpIA|BigAttack(Message) (Components|SkeletalMesh|GetAnimInstance (Variables|Character|GetMesh)))
    (Variables|Default|SetIsBigAttacking? true)
    (Variables|Utilities|SetHit%20Player%20? false)))

(event Custom|TakeDamage
  (params (Degats :type Float%20%28single-precision%29) (IsTraps :type Boolean))
  (bind _arena (Variables|OpenVariable|GetArena))
  (bind _mesh (Variables|Character|GetMesh))
  (bind _destructible (Variables|Default|GetDestructible))
  ;[1 1 1] Mort
  (if (not (or (Variables|Default|Getisdead) (Variables|Default|GetSpawned?)))
    (Rendering|SetVisibility (Variables|Default|GetWidget) true false)
    (bind _output_get (Variables|Default|SetCurrentHp (- (Variables|Default|GetCurrentHp) Degats)))
    (if (<= _output_get 0.0)
      (Class|Pawn|DetachfromControllerPendingDestroy)
      (Collision|SetCollisionProfileName (Variables|Collision|GetCapsuleComponent) "Ragdoll" true :!class /Script/Engine.PrimitiveComponent)
      (Development|SetHiddeninGame (Variables|Default|GetWidget) true false)
      (Variables|Default|Setisdead true)
      (if (not (Variables|Default|GetStunned?))
        (Physics|SetSimulatePhysics _mesh true)
        (Physics|AddImpulse _mesh (Math|Vector|MakeVector (Math|Random|RandomFloatinRange -5e+03 5e+03) (Math|Random|RandomFloatinRange -5e+03 5e+03) 5e+03) "None" true)
        (Utilities|FlowControl|DoOnce false
          (:Completed
            (Utilities|IsValid _arena
              (:Is%20Valid
                (Default|RemoveMobs _arena))
              (:Is%20Not%20Valid
                _))
            (CallFunction|DeathSound)
            (Utilities|FlowControl|Delay 2.0)
            (CallFunction|DissolveEvent false)))
        (else
          (Rendering|ToggleVisibility (Variables|Character|GetMesh) true)
          (Collision|SetCollisionEnabled (Variables|Collision|GetCapsuleComponent) "NoCollision")
          (Rendering|SetVisibility _destructible true false)
          (Physics|SetSimulatePhysics _destructible true)
          (Class|DestructibleComponent|ApplyDamage _destructible 5e+05 (Variables|Default|GetLocationHurt) (Variables|Default|GetImpulseDirection) 1.3e+03)
          (CallFunction|DeathSound)
          (Utilities|FlowControl|Delay 2.0)
          (Actor|DestroyActor)))
      (elif (not (or (Variables|Default|GetIsHit?) IsTraps))
        (bind _output_get_2 (Variables|Default|SetIsHit? true))
        (AI|Components|Blackboard|SetValueasBool (AI|GetBlackboard 0) (Utilities|Name|MakeLiteralName "IsHit") _output_get_2)
        (if (not (Variables|Default|GetIsIAGeneral))
          (Class|INTAnimBpIA|GetHit(Message) (Components|SkeletalMesh|GetAnimInstance (Variables|Character|GetMesh))))))))

(event Custom|DeathSound
  (Class|AkGameplayStatics|PostEvent (Variables|Default|GetSoundEventDeath) self))

(event Custom|EndHit
  (bind _self self)
  (bind _returnvalue (AI|GetAIController _self))
  (bind _returnvalue_2 (AI|GetBlackboard _returnvalue))
  (bind _returnvalue_3 (AI|GetBlackboard _returnvalue))
  ;[1 1 1] EndHit
  (Variables|Default|SetIsAttacking? false)
  (Variables|Default|SetIsBigAttacking? false)
  (bind _output_get (Variables|Default|SetIsHit? false))
  (Utilities|IsValid _returnvalue_3
    (:Is%20Valid
      (AI|Components|Blackboard|SetValueasBool _returnvalue_3 (Utilities|Name|MakeLiteralName "IsHit") _output_get))
    (:Is%20Not%20Valid
      _))
  (if (Variables|Default|GetStunned?)
    (bind _output_get_2 (Variables|Default|SetStunned? false))
    (Utilities|IsValid _returnvalue_2
      (:Is%20Valid
        (AI|Components|Blackboard|SetValueasBool _returnvalue_2 (Utilities|Name|MakeLiteralName "Stunned?") _output_get_2)))))

(event Custom|Fall
  (bind _arena (Variables|OpenVariable|GetArena))
  ;[1 1 1] Mort
  ;;[1 1 1] Chute
  (if (not (Variables|Default|Getisdead))
    (Variables|Default|SetCurrentHp 0.0)
    (Class|Pawn|DetachfromControllerPendingDestroy)
    (Variables|Default|Setisdead true)
    (Utilities|FlowControl|DoOnce false
      (:Completed
        (Utilities|IsValid _arena
          (:Is%20Valid
            (Default|RemoveMobs _arena))
          (:Is%20Not%20Valid
            _))
        (CallFunction|DeathSound)
        (Utilities|FlowControl|Delay 1.0)
        (Actor|DestroyActor)))))

(event Custom|CanMove
  (params (canRotate? :type Boolean))
  (bind _charactermovement (Variables|Character|GetCharacterMovement))
  ;[1 1 1] Can Move
  (bind _output_get (Variables|Default|SetCanRotate? canRotate?))
  (if _output_get
    (Pawn|Components|CharacterMovement|SetMovementMode _charactermovement "MOVE_Walking" 0)
    (else
      (Pawn|Components|CharacterMovement|DisableMovement _charactermovement))))

(event Custom|IsImmo
  (params (TimeImmo :type Float%20%28single-precision%29) (Damage :type Float%20%28single-precision%29))
  (bind _mesh (Variables|Character|GetMesh))
  ;[1 1 1] Immobilisation
  (if (not (Variables|Default|GetIsIAGeneral))
    (if (not (or (Variables|Default|Getisdead) (Variables|Default|GetSpawned?)))
      (Components|Movement|StopMovementImmediately (Variables|Character|GetCharacterMovement))
      (Variables|Default|SetMaterialBody (Rendering|Material|GetMaterial _mesh 0))
      (Rendering|Material|SetMaterial _mesh 0 "/Game/Game_Dev/Materials/Inst/M_SpellImmo_Inst.M_SpellImmo_Inst")
      (bind _output_get (Variables|Default|SetStunned? true))
      (AI|Components|Blackboard|SetValueasBool (AI|GetBlackboard 0) (Utilities|Name|MakeLiteralName "Stunned?") _output_get)
      (bind _output_get_2 (Variables|Default|SetIsHit? true))
      (AI|Components|Blackboard|SetValueasBool (AI|GetBlackboard 0) (Utilities|Name|MakeLiteralName "IsHit") _output_get_2)
      (Utilities|FlowControl|RetriggerableDelay TimeImmo)
      (if (not (Variables|Default|Getisdead))
        (Rendering|Material|SetMaterial (Variables|Character|GetMesh) 0 (Variables|Default|GetMaterialBody))
        (bind _output_get_3 (Variables|Default|SetStunned? false))
        (AI|Components|Blackboard|SetValueasBool (AI|GetBlackboard 0) (Utilities|Name|MakeLiteralName "Stunned?") _output_get_3)
        (bind _output_get_4 (Variables|Default|SetIsHit? false))
        (AI|Components|Blackboard|SetValueasBool (AI|GetBlackboard 0) (Utilities|Name|MakeLiteralName "IsHit") _output_get_4)))))

(event Custom|StartAttack
  ;[1 1 1] StartAttack
  (if (Math|Boolean|ANDBoolean (not (Variables|Default|GetIsHit?)) (not (Variables|Default|Getisdead)) (not (Variables|Default|GetIsAttacking?)) (not (Variables|Default|GetSpawned?)))
    (Class|INTAnimBpIA|Attack(Message) (Components|SkeletalMesh|GetAnimInstance (Variables|Character|GetMesh)))
    (Variables|Default|SetIsAttacking? true)
    (Variables|Utilities|SetHit%20Player%20? false)))

(event Custom|PoisonDamage
  (params (Degats :type Float%20%28single-precision%29) (Count :type Integer))
  ;[1 1 1] Poison Damage
  (if (not (or (Variables|Default|Getisdead) (Variables|Default|GetSpawned?)))
    (if (> Count 0)
      (bind _result (Math|Integer|DecrementInt Count)
        (:%20%20
          (Game|Damage|ApplyDamage self Degats 0 0)
          (if (<= (Variables|Default|GetCurrentHp) 0.0)
            (Class|Pawn|DetachfromControllerPendingDestroy)
            (Variables|Default|Setisdead true)
            (Class|INTAnimBpIA|Death(Message) (Components|SkeletalMesh|GetAnimInstance (Variables|Character|GetMesh)))
            (else
              (Utilities|FlowControl|Delay 1.0)
              (CallFunction|PoisonDamage Degats _result))))))))

(event Custom|Set%20Seen
  (bind _returnvalue (AI|GetBlackboard 0))
  ;[1 1 1] Seen?
  (Utilities|IsValid _returnvalue
    (:Is%20Valid
      (AI|Components|Blackboard|SetValueasBool _returnvalue (Utilities|Name|MakeLiteralName "Seen?") true)
      (Variables|/Script/Engine.CharacterMovementComponent|SetMaxWalkSpeed (Variables|Character|GetCharacterMovement) (Variables|OpenVariable|GetSpeed)))))

(event Custom|DissolveEvent
  (params (Spawn :type Boolean))
  (if Spawn
    (bind _newtrack_0 (Timeline|Dissolve PlayFromStart)
      (:Update
        (Rendering|Material|SetScalarParameterValueonMaterials (Variables|Character|GetMesh) "Dissolve" _newtrack_0))
      (:Finished
        (if Spawn
          (Variables|Default|SetSpawned? false)
          (if (Variables|Default|GetSpawnSeen)
            (CallFunction|SetSeen))
          (else
            (Actor|DestroyActor)))))
    (else
      (Timeline|Dissolve ReverseFromEnd))))

(event Game|Damage|EventAnyDamage
  (params (Damage :type Float%20%28single-precision%29) (DamageType :type Damage%20Type%20Object%20Reference) (InstigatedBy :type Controller%20Object%20Reference) (DamageCauser :type Actor%20Object%20Reference))
  (bind _returnvalue (Utilities|GetClass DamageCauser))
  ;[1 1 1] Mort
  (CallFunction|SetSeen)
  (if (not (Variables|Default|GetInvincible))
    (if (not (== _returnvalue "/Game/Game_Dev/Blueprints/IA/Trashmob/Blueprints/BP_Puddle.BP_Puddle_C"))
      (CallFunction|TakeDamage Damage (== _returnvalue "/Game/Game_Dev/Blueprints/Trap/BP_Spike.BP_Spike_C")))))

(event EventTick
  (params (DeltaSeconds :type Float%20%28single-precision%29))
  (bind _stunned_ (Variables|Default|GetStunned?))
  (bind _returnvalue (select _stunned_ true false))
  (if (AI|Components|NavMovement|IsFalling (Variables|Character|GetCharacterMovement))
    (Audio|Components|Audio|Stop (Variables|Character|GetMesh))
    (else
      ;[1 1 1] Stun Immo
      (if (Math|Boolean|NotEqual(Boolean) (Variables|/Script/Engine.SkeletalMeshComponent|GetbPauseAnims (Variables|Character|GetMesh)) _returnvalue)
        (Variables|/Script/Engine.SkeletalMeshComponent|SetbPauseAnims (Variables|Character|GetMesh) _returnvalue)))))

(event EventBeginPlay
  (bind _niagara (Variables|Default|GetNiagara))
  ;[1 1 1] Widget Barre de vie
  (Variables|/Game/Game_Dev/Blueprints/Widget/LifesBar/WG_EnemyLife.WG_EnemyLife_C|SetTrashmob_ref (.AsWG%20Enemy%20Life (Utilities|Casting|CastToWG_EnemyLife (UserInterface|GetUserWidgetObject (Variables|Default|GetWidget)))) self)
  (if (Variables|Default|GetSpawned?)
    (Class|NiagaraComponent|SetAsset _niagara (Variables|OpenVariable|GetNiagaraSystem))
    (Niagara|ResetSystem _niagara)
    (CallFunction|DissolveEvent true)
    (else
      (Components|Activation|SetActive (Variables|Default|GetNiagara) false false))))

(fn ConstructionScript)