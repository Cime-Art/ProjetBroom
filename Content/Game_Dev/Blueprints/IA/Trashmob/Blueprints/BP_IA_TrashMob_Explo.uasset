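; Explosive snail trash mob character, a child Blueprint that switches its AI controller to the explosion behavior tree on BeginPlay.
; A state event maps idle, forward and attack to Wwise audio states, with attack using the explosion state.
; A timeline drives the explosion warning material parameter, resetting it and destroying the preview component if hit or dead.
; Death detaches the controller, disables capsule collision, removes the widget, notifies the arena and starts dissolving.
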(event Custom|Feedback%20Explo
  (bind _previewref (Variables|Default|GetPreviewRef))
  (bind _explo (Timeline|Explo PlayFromStart)
    (:Update
      (if (or (Variables|Default|GetIsHit?) (Variables|Default|Getisdead))
        (Rendering|Material|SetScalarParameterValueonMaterials (Variables|Character|GetMesh) "FeedbackExplo" 0.0)
        (Utilities|IsValid _previewref
          (:Is%20Valid
            (Components|DestroyComponent _previewref)))
        (else
          (Rendering|Material|SetScalarParameterValueonMaterials (Variables|Character|GetMesh) "FeedbackExplo" _explo))))))

(event Custom|StatesSnail
  (params (States :type String))
  (switch string States
    (:Default
      (Class|AkGameplayStatics|SetState "/Game/WwiseAudio/States/Default_Work_Unit/Mob/Snail/snail_stateGroup/snail_stateGroup-snail_idle_state.snail_stateGroup-snail_idle_state" :!label _label))
    (:Idle
      (goto _label))
    (:Forward
      (Class|AkGameplayStatics|SetState "/Game/WwiseAudio/States/Default_Work_Unit/Mob/Snail/snail_stateGroup/snail_stateGroup-snail_forward_state.snail_stateGroup-snail_forward_state"))
    (:Attack
      (Class|AkGameplayStatics|SetState "/Game/WwiseAudio/States/Default_Work_Unit/Mob/Snail/snail_stateGroup/snail_stateGroup-snail_explosion_state.snail_stateGroup-snail_explosion_state"))))

(event EventBeginPlay
  (|CallParentFunction)
  (Default|ChangeBehaviorTree (.AsIA%20Controller%20Trashmob (Utilities|Casting|CastToIA_Controller_Trashmob (AI|GetAIController self))) "/Game/Game_Dev/Blueprints/IA/Trashmob/BehaviorTree_Blackboard/BT_IA_Explo.BT_IA_Explo")
  (Class|AkGameplayStatics|SetState "/Game/WwiseAudio/States/Default_Work_Unit/Mob/Snail/snail_stateGroup/snail_stateGroup-snail_idle_state.snail_stateGroup-snail_idle_state")
  (Class|AkGameplayStatics|PostEvent "/Game/WwiseAudio/Events/Default_Work_Unit/Mob/Snail/Event_Snail_States.Event_Snail_States" self))

(event Collision|EventActorBeginOverlap
  (params (OtherActor :type Actor%20Object%20Reference)))

(event EventTick
  (params (DeltaSeconds :type Float%20%28single-precision%29))
  (|CallParentFunction DeltaSeconds) ; This node is disabled and will not be called.\nDrag off pins to build functionality.
)

(event EventDeath
  (bind _arena (Variables|Default|GetArena))
  (Variables|Default|Setisdead true)
  (Class|Pawn|DetachfromControllerPendingDestroy)
  (Collision|SetCollisionEnabled (Variables|Default|GetCapsuleComponent) "NoCollision")
  (Components|DestroyComponent (Variables|Default|GetWidget))
  (Utilities|IsValid _arena
    (:Is%20Valid
      (Default|RemoveMobs _arena))
    (:Is%20Not%20Valid
      _))
  (CallFunction|DissolveEvent false))

(fn ConstructionScript
  (|CallParentFunction))