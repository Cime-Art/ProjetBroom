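; Ranged trashmob arrow projectile that damages the player and sticks into what it hits.
; ActivatePhysics adds a projectile movement component at runtime and sets the arrow to overlap pawns with query-only collision.
; The first overlap with the player or a static mesh attaches the arrow, removes its movement and Niagara effect, damages only players, then destroys it after a delay.
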(event OnComponentBeginOverlap(Arrow)
  (params (OverlappedComponent :type Primitive%20Component%20Object%20Reference) (OtherActor :type Actor%20Object%20Reference) (OtherComp :type Primitive%20Component%20Object%20Reference) (OtherBodyIndex :type Integer) (bFromSweep :type Boolean) (SweepResult :type Hit%20Result%20Structure%20%28by%20ref%29))
  (bind _projectile_ref (Variables|Default|GetProjectile%20Ref))
  (bind _asbp_player_test (Utilities|Casting|CastToBP_PlayerTest OtherActor)
    (:then
      (Variables|Default|SetIsPlayer true))
    (:CastFailed
      (bind _asstatic_mesh_component (Utilities|Casting|CastToStaticMeshComponent OtherComp))))
  (Utilities|FlowControl|DoOnce false
    (:Completed
      (Transformation|AttachComponentToComponent (select (Variables|Default|GetIsPlayer) (Variables|/Script/Engine.Character|GetMesh _asbp_player_test) _asstatic_mesh_component) "None" "KeepWorld" "KeepWorld" "KeepWorld" true)
      (Utilities|IsValid _projectile_ref
        (:Is%20Valid
          (Components|DestroyComponent _projectile_ref)
          (if (Variables|Default|GetIsPlayer)
            (Game|Damage|ApplyDamage _asbp_player_test (Variables|Default|GetDamage) 0 0))
          (Collision|SetCollisionEnabled (Variables|Default|GetArrow) "QueryOnly")
          (Utilities|FlowControl|Delay 1e+01))
        (:Is%20Not%20Valid
          _))
      (Actor|DestroyActor))))

(event Custom|ActivatePhysics
  (bind _returnvalue (AddComponent|AddProjectileMovementComponent))
  (Variables|Default|SetProjectile%20Ref _returnvalue)
  (Collision|SetCollisionEnabled (Variables|Default|GetArrow) "QueryOnly")
  (Collision|SetCollisionResponsetoChannel (Variables|Default|GetArrow) "ECC_Pawn" "ECR_Overlap"))

(fn ConstructionScript)