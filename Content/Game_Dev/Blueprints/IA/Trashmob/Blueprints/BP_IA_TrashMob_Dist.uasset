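; Ranged trash mob enemy, a child Blueprint that switches its AI controller to the BT_IA_Dist behavior tree on begin play.
; The construction script attaches a crossbow and randomly picks socketed props from StuffToAdd into the Stuff array.
; Stuff dissolves through a timeline on spawn or despawn, and Tick sets Fuite (flee) when the player is close.
; IsImmo temporarily applies an immobilize-spell material, restoring the props' saved materials unless the mob is dead.
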(event EventBeginPlay
  (|CallParentFunction)
  (Default|ChangeBehaviorTree (.AsIA%20Controller%20Trashmob (Utilities|Casting|CastToIA_Controller_Trashmob (AI|GetAIController self))) "/Game/Game_Dev/Blueprints/IA/Trashmob/BehaviorTree_Blackboard/BT_IA_Dist.BT_IA_Dist")
  (CallFunction|DissolveEvent true))

(event EventTick
  (params (DeltaSeconds :type Float%20%28single-precision%29))
  (|CallParentFunction DeltaSeconds)
  (if (<= (Transformation|GetDistanceTo (Game|GetPlayerCharacter 0)) 4.5e+02)
    (Variables|Default|SetFuite? true)
    (else
      (Variables|Default|SetFuite? false))))

(event Collision|EventActorBeginOverlap
  (params (OtherActor :type Actor%20Object%20Reference)))

(event EventIsImmo
  (params (TimeImmo :type Float%20%28single-precision%29) (Damage :type Float%20%28single-precision%29))
  (|CallParentFunction TimeImmo Damage)
  (for _array_element (Variables|Default|GetStuff)
    (Utilities|Array|Add (Variables|Default|GetStuffMaterial) (Rendering|Material|GetMaterial _array_element 0)))
  (Rendering|Material|SetMaterial (Variables|Character|GetMesh) 0 "/Game/Game_Dev/Materials/Inst/M_SpellImmo_Inst.M_SpellImmo_Inst")
  (for _array_element_2 (Variables|Default|GetStuff)
    (Rendering|Material|SetMaterial _array_element_2 0 "/Game/Game_Dev/Materials/Inst/M_SpellImmo_Inst.M_SpellImmo_Inst"))
  (Utilities|FlowControl|Delay 3.0)
  (if (not (Variables|Default|Getisdead))
    (for (_array_element_3 _array_index) (Variables|Default|GetStuff)
      (Rendering|Material|SetMaterial _array_element_3 0 (Utilities|Array|Get(acopy) (Variables|Default|GetStuffMaterial) _array_index)))))

(event EventDissolveEvent
  (params (Spawn :type Boolean))
  (|CallParentFunction Spawn)
  (if Spawn
    (bind _newtrack_0 (Timeline|Timeline_0 PlayFromStart)
      (:Update
        (for _array_element (Variables|Default|GetStuff)
          (Rendering|Material|SetScalarParameterValueonMaterials _array_element "Dissolve" _newtrack_0))))
    (else
      (Timeline|Timeline_0 ReverseFromEnd))))

(fn ConstructionScript
  (bind _stufftoadd (Variables|Default|GetStuffToAdd))
  (|CallParentFunction)
  (Utilities|Array|Clear (Variables|Default|GetStuff))
  (bind _returnvalue (AddComponent|AddStaticMeshComponent false))
  (Transformation|AttachComponentToComponent _returnvalue (Variables|Character|GetMesh) "Weapon_Crossbow" "KeepRelative" "KeepRelative" "KeepRelative" true)
  (Collision|SetCollisionEnabled _returnvalue "NoCollision")
  (Utilities|Array|AddUnique (Variables|Default|GetStuff) _returnvalue)
  (bind _keys (Utilities|Map|Keys _stufftoadd))
  ;[1 1 1] Stuff
  (bind _values (Utilities|Map|Values _stufftoadd))
  (for (_array_element _array_index) _values
    (if (<= (Math|Random|RandomFloat) 0.5)
      (bind _returnvalue_2 (AddComponent|AddStaticMeshComponent false))
      (Components|StaticMesh|SetStaticMesh _returnvalue_2 _array_element)
      (Utilities|Array|AddUnique (Variables|Default|GetStuff) _returnvalue_2)
      (Transformation|AttachComponentToComponent _returnvalue_2 (Variables|Character|GetMesh) (Utilities|Array|Get(acopy) _keys _array_index) "KeepRelative" "KeepRelative" "KeepRelative" true)
      (Collision|SetCollisionEnabled _returnvalue_2 "NoCollision"))))