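; BP_Puddle is a short-lived damaging puddle actor, filed under the Trashmob AI assets.
; On BeginPlay it spawns an Alambic Niagara effect at its location and starts a looping timer that applies radial damage around the actor.
; After a brief delay it deactivates the effect and destroys itself.
; Damage relies on the timed radius pulse, as the overlap event is unused.
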(event Custom|TickDamage
  (Game|Damage|ApplyRadialDamage (Math|Conversions|ToFloat(Integer) (Variables|Default|GetDamage)) (Transformation|GetActorLocation) 2.5e+02 0 0 self 0 false "ECC_Visibility"))

(event EventBeginPlay
  (Utilities|FlowControl|Sequence
    (:then_0
      (bind _returnvalue (Niagara|SpawnSystematLocation "/Game/Game_Dev/FX/NiagaraSystems/NS_Alambic_SystemV2.NS_Alambic_SystemV2" (Transformation|GetActorLocation)))
      (Variables|Default|SetNiagara _returnvalue)
      (Utilities|FlowControl|Delay 2.0)
      (Components|Activation|Deactivate (Variables|Default|GetNiagara))
      (Actor|DestroyActor self))
    (:then_1
      (Utilities|Time|SetTimerbyEvent (delegate Custom|TickDamage) 0.2 true))))

(event Collision|EventActorBeginOverlap
  (params (OtherActor :type Actor%20Object%20Reference)))

(fn ConstructionScript)