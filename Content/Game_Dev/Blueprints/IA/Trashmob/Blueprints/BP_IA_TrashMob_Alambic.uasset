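; BP_IA_TrashMob_Alambic is the Alambic variant of the trash mob AI enemy.
; On BeginPlay it switches its trash mob controller to the Alambic behavior tree, and StartAttack messages the AnimInstance unless hit, dead or already attacking.
; Tick tracks an attack timer and toggles walk speed through paired DoOnce nodes based on CanMoveAlambic.
; DissolveEvent swaps in dissolve materials and plays one timeline forward for spawning or backward before destroying the actor.
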(event EventBeginPlay
  (|CallParentFunction)
  (Default|ChangeBehaviorTree (.AsIA%20Controller%20Trashmob (Utilities|Casting|CastToIA_Controller_Trashmob (AI|GetAIController self))) "/Game/Game_Dev/Blueprints/IA/Trashmob/BehaviorTree_Blackboard/BT_IA_Alambic.BT_IA_Alambic"))

(event Collision|EventActorBeginOverlap
  (params (OtherActor :type Actor%20Object%20Reference)))

(event EventTick
  (params (DeltaSeconds :type Float%20%28single-precision%29))
  (bind _charactermovement (Variables|Character|GetCharacterMovement))
  (|CallParentFunction DeltaSeconds)
  (Variables|Default|SetTimerAttack (Math|Float|SelectFloat 0.0 (+ (Variables|Default|GetTimerAttack) (Utilities|Time|GetWorldDeltaSeconds)) (Variables|Default|GetLaunchingAttack)))
  (if (Variables|Default|GetCanMoveAlambic)
    (Utilities|FlowControl|Sequence
      (:then_0
        (Utilities|FlowControl|DoOnce false :!label _label
          (:Completed
            (Variables|/Script/Engine.CharacterMovementComponent|SetMaxWalkSpeed _charactermovement 3e+02))))
      (:then_1
        (goto _label_2 Reset)))
    (else
      (Utilities|FlowControl|Sequence
        (:then_0
          (goto _label Reset))
        (:then_1
          (Utilities|FlowControl|DoOnce false :!label _label_2
            (:Completed
              (Variables|/Script/Engine.CharacterMovementComponent|SetMaxWalkSpeed _charactermovement 1.5e+02))))))))

(event EventStartAttack
  (if (Math|Boolean|ANDBoolean (not (Variables|Default|GetIsHit?)) (not (Variables|Default|Getisdead)) (not (Variables|Default|GetIsAttacking?)))
    (Class|INTAnimBpIA|Attack(Message) (Components|SkeletalMesh|GetAnimInstance (Variables|Character|GetMesh)))
    (Variables|Default|SetIsAttacking? true)))

(event EventDissolveEvent
  (params (Spawn :type Boolean))
  (bind _mesh (Variables|Character|GetMesh))
  (bind _mesh_2 (Variables|Character|GetMesh))
  (Rendering|Material|SetMaterial _mesh_2 0 "/Game/Game_Dev/Materials/Inst/M_DissolveIA_Inst_Alambic.M_DissolveIA_Inst_Alambic")
  (Rendering|Material|SetMaterial _mesh_2 1 "/Game/Game_Dev/Materials/Inst/M_DissolveIA_Inst_Alambic.M_DissolveIA_Inst_Alambic")
  (Rendering|Material|SetMaterial _mesh_2 2 "/Game/Game_Dev/Materials/Parents/M_DissolveTrans_Inst.M_DissolveTrans_Inst")
  (if Spawn
    (bind _newtrack_0 (Timeline|Timeline_1 PlayFromStart)
      (:Update
        (Rendering|Material|SetScalarParameterValueonMaterials (Variables|Character|GetMesh) "Dissolve" _newtrack_0))
      (:Finished
        (if Spawn
          (Rendering|Material|SetMaterial _mesh 0 "/Game/Game_ART/Graph/Chara/Mob/Alambic/MAT_Alambic_Translucent.MAT_Alambic_Translucent")
          (Rendering|Material|SetMaterial _mesh 1 "/Game/Game_ART/Graph/Chara/Mob/Alambic/MAT_Alambic_Inst.MAT_Alambic_Inst")
          (Rendering|Material|SetMaterial _mesh 2 "/Game/Game_ART/Graph/Chara/Mob/Alambic/MAT_Alambic_Translucent_Inst.MAT_Alambic_Translucent_Inst")
          (Variables|Default|SetSpawned? false)
          (if (Variables|Default|GetSpawnSeen)
            (CallFunction|SetSeen))
          (else
            (Class|AkGameplayStatics|StopActor self)
            (Utilities|FlowControl|Delay 2.0)
            (Actor|DestroyActor)))))
    (else
      (Timeline|Timeline_1 ReverseFromEnd))))

(fn ConstructionScript
  (|CallParentFunction))