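; BP_Banana is a tutorial target enemy that spawns BP_Tuto prompts and unlocks a door once defeated.
; Broom overlaps message its anim instance, while GetHit plays random hit montages, gated by CanHit, and counts hits.
; Every fifth hit advances LaunchTutorial: first teleporting it to a target point with a new prompt, then unlocking the door and destroying it.
; A timeline-driven material dissolve covers the teleport and death.
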(event OnComponentBeginOverlap(Box)
  (params (OverlappedComponent :type Primitive%20Component%20Object%20Reference) (OtherActor :type Actor%20Object%20Reference) (OtherComp :type Primitive%20Component%20Object%20Reference) (OtherBodyIndex :type Integer) (bFromSweep :type Boolean) (SweepResult :type Hit%20Result%20Structure%20%28by%20ref%29))
  (Utilities|Casting|CastToBP_Broom OtherActor)
  (Class|INTAnimBpIA|GetHit(Message) (Components|SkeletalMesh|GetAnimInstance (Variables|Character|GetMesh))))

(event Custom|Dissolve
  (params (Spawn :type Boolean))
  (if Spawn
    (bind _newtrack_0 (Timeline|TL_Dissolve PlayFromStart)
      (:Update
        (Rendering|Material|SetScalarParameterValueonMaterials (Variables|Character|GetMesh) "Dissolve" _newtrack_0)))
    (else
      (Timeline|TL_Dissolve ReverseFromEnd))))

(event Custom|LaunchTutorial
  (bind _returnvalue (Transformation|GetActorForwardVector))
  (bind _returnvalue_2 (Transformation|GetActorLocation))
  (bind _mesh (Variables|Character|GetMesh))
  (bind _returnvalue_3 (Transformation|GetWorldLocation _mesh))
  (bind _returnvalue_4 (* _returnvalue 1.5e+02))
  (bind _returnvalue_5 (+ _returnvalue_2 _returnvalue_4))
  (switch int (Variables|Default|GetTutorialIndex)
    (:0
      (Game|SpawnActorfromClass "/Game/Game_Dev/Blueprints/GameplayScript/BP_Tuto.BP_Tuto_C" (Math|Transform|MakeTransform (Math|Vector|MakeVector (.x _returnvalue_5) (.y _returnvalue_5) (.z _returnvalue_3)) "0, 0, 0" "1,1,1") "AlwaysSpawn" 0 "NewEnumerator5" 0 0))
    (:1
      (CallFunction|Dissolve false)
      (Utilities|FlowControl|Delay 1.0)
      (Transformation|SetActorLocation (Transformation|GetActorLocation (Variables|Default|GetTargetPoint)) false true)
      (CallFunction|Dissolve true)
      (Game|SpawnActorfromClass "/Game/Game_Dev/Blueprints/GameplayScript/BP_Tuto.BP_Tuto_C" (Math|Transform|MakeTransform (Math|Vector|MakeVector (.x _returnvalue_5) (.y _returnvalue_5) (.z _returnvalue_3)) "0, 0, 0" "1,1,1") "AlwaysSpawn" 0 "NewEnumerator5" 0 0))
    (:2
      (Variables|Default|SetDead true)
      (CallFunction|Dissolve false)
      (Variables|/Game/Game_Dev/Blueprints/Trap/BP_Door_Tuto.BP_Door_Tuto_C|SetUnlock (Variables|Default|GetDoor) true)
      (Utilities|FlowControl|Delay 1.0)
      (Actor|DestroyActor))))

(event EventBeginPlay
  (CallFunction|LaunchTutorial))

(event EventGetHit
  (if (and (Variables|Default|GetCanHit?) (not (Variables|Default|GetDead)))
    (bind _result (Math|Integer|IncrementInt (Variables|Default|GetCpt))
      (:%20%20
        (if (== _result 5)
          (Math|Integer|IncrementInt (Variables|Default|GetTutorialIndex)
            (:%20%20
              (Variables|Default|SetCpt 0)
              (CallFunction|LaunchTutorial)
              (Variables|Default|SetCanHit? false)))
          (else
            (Variables|Default|SetCanHit? false)
            (Animation|Montage|PlayMontage (Variables|Character|GetMesh) (Utilities|Select :Index (Math|Random|RandomIntegerinRange 0 2) :Option%200 "/Game/Game_ART/Graph/Chara/Mob/Banana_v2/Anime/Getit_01_Montage.Getit_01_Montage" :Option%201 "/Game/Game_ART/Graph/Chara/Mob/Banana_v2/Anime/Getit_02_Montage.Getit_02_Montage" :Option%202 "/Game/Game_ART/Graph/Chara/Mob/Banana_v2/Anime/Getit_03_Montage.Getit_03_Montage")
              (:OnCompleted
                (Variables|Default|SetCanHit? true)))))))))

(fn ConstructionScript)