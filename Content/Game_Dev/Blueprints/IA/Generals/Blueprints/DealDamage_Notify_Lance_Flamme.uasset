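; Anim notify state that deals flamethrower damage to the player during a trash mob AI's animation.
; Each notify tick sphere-traces on the Camera channel between the mesh's Flame_Start and Flame_End sockets.
; If the hit actor is BP_PlayerTest, it applies Damage and sets HitPlayer on the owning BP_IA_TrashMob.
; That flag blocks further hits; this file never resets it.
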(fn ReceivedNotifyTick
  (params (MeshComp :type Skeletal%20Mesh%20Component%20Object%20Reference) (Animation :type Anim%20Sequence%20Base%20Object%20Reference) (FrameDeltaTime :type Float%20%28single-precision%29))
  (bind _returnvalue (Components|GetOwner MeshComp))
  (bind _asbp_ia_trash_mob (Utilities|Casting|CastToBP_IA_TrashMob _returnvalue))
  (bind _outhit (Collision|SphereTraceByChannel MeshComp (Transformation|GetSocketLocation MeshComp "Flame_Start") (Transformation|GetSocketLocation MeshComp "Flame_End") 1e+02 "TraceTypeQuery2" false 0 "None" true "(R=1.000000,G=0.000000,B=0.000000,A=1.000000)" "(R=0.000000,G=1.000000,B=0.000000,A=1.000000)" 0.5))
  (bind _asbp_player_test (Utilities|Casting|CastToBP_PlayerTest (.hitactor _outhit)))
  (if (not (Variables|/Game/Game_Dev/Blueprints/IA/Trashmob/Blueprints/BP_IA_TrashMob.BP_IA_TrashMob_C|GetHit%20Player%20? _asbp_ia_trash_mob))
    (Game|Damage|ApplyDamage _asbp_player_test (Variables|Default|GetDamage) 0 0)
    (Variables|/Game/Game_Dev/Blueprints/IA/Trashmob/Blueprints/BP_IA_TrashMob.BP_IA_TrashMob_C|SetHit%20Player%20? _asbp_ia_trash_mob true)
    (return true)))