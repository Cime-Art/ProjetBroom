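; Boss arena trigger that starts the encounter with the CraneDeFeu General when the player enters its box.
; On the first BP_PlayerTest overlap only, it finds the General in the level by class and adds its big life bar widget to the viewport.
; It then sets the "IsSeen?" key on that General's blackboard to true, if the blackboard is valid.
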(event OnComponentBeginOverlap(Box)
  (params (OverlappedComponent :type Primitive%20Component%20Object%20Reference) (OtherActor :type Actor%20Object%20Reference) (OtherComp :type Primitive%20Component%20Object%20Reference) (OtherBodyIndex :type Integer) (bFromSweep :type Boolean) (SweepResult :type Hit%20Result%20Structure%20%28by%20ref%29))
  (Utilities|Casting|CastToBP_PlayerTest OtherActor)
  (Utilities|FlowControl|DoOnce false
    (:Completed
      (bind _returnvalue (Actor|GetActorOfClass "/Game/Game_Dev/Blueprints/IA/Generals/Blueprints/BP_IA_Generals_CraneDeFeu.BP_IA_Generals_CraneDeFeu_C"))
      (Variables|Default|SetGeneral_Ref _returnvalue)
      (bind _returnvalue_2 (UserInterface|CreateWidget "/Game/Game_Dev/Blueprints/Widget/LifesBar/WG_General_BigLifeBar.WG_General_BigLifeBar_C" 0 (Variables|Default|GetGeneral_Ref)))
      (UserInterface|Viewport|AddtoViewport _returnvalue_2 0)
      (Utilities|IsValid (AI|GetBlackboard (Variables|Default|GetGeneral_Ref))
        (:Is%20Valid
          (AI|Components|Blackboard|SetValueasBool (AI|GetBlackboard (Variables|Default|GetGeneral_Ref)) (Utilities|Name|MakeLiteralName "IsSeen?") true))))))

(event EventBeginPlay)

(event Collision|EventActorBeginOverlap
  (params (OtherActor :type Actor%20Object%20Reference)))

(event EventTick
  (params (DeltaSeconds :type Float%20%28single-precision%29)))

(fn ConstructionScript)