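; BP_FireBall is a fireball projectile actor that damages the player on contact.
; ActivatePhysics adds a projectile movement component at runtime, stores its reference and sets the Sphere to query-only collision that overlaps Pawns.
; The Sphere's begin-overlap applies Damage once to a BP_PlayerTest and destroys the fireball.
; An overlap with any other actor destroys it after a delay.
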(event OnComponentBeginOverlap(Sphere)
  (params (OverlappedComponent :type Primitive%20Component%20Object%20Reference) (OtherActor :type Actor%20Object%20Reference) (OtherComp :type Primitive%20Component%20Object%20Reference) (OtherBodyIndex :type Integer) (bFromSweep :type Boolean) (SweepResult :type Hit%20Result%20Structure%20%28by%20ref%29))
  (bind _asbp_player_test (Utilities|Casting|CastToBP_PlayerTest OtherActor)
    (:then
      (Utilities|FlowControl|DoOnce false
        (:Completed
          (Game|Damage|ApplyDamage _asbp_player_test (Variables|Default|GetDamage) 0 0)
          (Actor|DestroyActor self))))
    (:CastFailed
      (Utilities|FlowControl|Delay 1e+01)
      (Actor|DestroyActor self))))

(event Custom|ActivatePhysics
  (bind _sphere (Variables|Default|GetSphere))
  (bind _returnvalue (AddComponent|AddProjectileMovementComponent))
  (Variables|Default|SetProjectile%20Ref _returnvalue)
  (Collision|SetCollisionEnabled _sphere "QueryOnly")
  (Collision|SetCollisionResponsetoChannel _sphere "ECC_Pawn" "ECR_Overlap"))

(fn ConstructionScript)