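; AI boss character for the "Generals" that loads a behavior tree by general type and runs five attacks plus a timed stun.
; Attack events message the AnimBP, while movement, stun and hit states gate behavior, partly through Blackboard flags.
; Timelines drive trace-clamped dash and recoil, a long charge that launches the player or flags impacts, and an invincible spline move.
; The Niagara fire wave returns particle positions through a callback for one-shot, jump-avoidable damage.
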(event OnComponentHit(CapsuleComponent)
  (params (HitComponent :type Primitive%20Component%20Object%20Reference) (OtherActor :type Actor%20Object%20Reference) (OtherComp :type Primitive%20Component%20Object%20Reference) (NormalImpulse :type Vector :default "0, 0, 0") (Hit :type Hit%20Result%20Structure%20%28by%20ref%29))
  (bind _returnvalue (Transformation|GetActorForwardVector))
  (bind _returnvalue_2 (* _returnvalue 1e+03))
  ;[1 1 1] Hit Dash
  (if (Variables|Default|GetIsAttacking_4)
    (Utilities|FlowControl|DoOnce false
      (:Completed
        (bind _asbp_player_test (Utilities|Casting|CastToBP_PlayerTest OtherActor)
          (:then
            (Character|LaunchCharacter _asbp_player_test (Math|Vector|MakeVector (.x _returnvalue_2) (.y _returnvalue_2) 1.5e+03) true true))
          (:CastFailed
            (if (not (== HitComponent 0))
              (bind _output_get (Variables|Default|SetIsHit?_0 true))
              (AI|Components|Blackboard|SetValueasBool (AI|GetBlackboard 0) (Utilities|Name|MakeLiteralName "IsHit") _output_get))))))))

(event Custom|StartAttack_1
  (if (not (Variables|Default|GetIsAttacking1))
    (Class|INTAnimBpIA|AttackGeneral1(Message) (Components|SkeletalMesh|GetAnimInstance (Variables|Character|GetMesh)))
    (Variables|Default|SetIsAttacking1 true)
    (Variables|Utilities|SetHit%20Player%20?_0 false)))

(event Custom|Stunned
  (Variables|Default|SetStunned_General? true)
  (AI|Components|Blackboard|SetValueasBool (AI|GetBlackboard 0) (Utilities|Name|MakeLiteralName "Stunned_General") true)
  (Variables|Default|SetCanRotateGeneral false)
  (Utilities|FlowControl|Delay 3.0)
  (if (not (Variables|Default|Getisdead))
    (bind _output_get (Variables|Default|SetStunned_General? false))
    (AI|Components|Blackboard|SetValueasBool (AI|GetBlackboard 0) (Utilities|Name|MakeLiteralName "Stunned_General") _output_get)))

(event Custom|Scale%20Fireball
  (params (Target :type Actor%20Object%20Reference))
  ;[1 1 1] Scale FireBalle
  (bind _scale (Timeline|Timeline_1 PlayFromStart)
    (:Update
      (Transformation|SetActorScale3D Target _scale))))

(event Custom|Collision%20FireWAVE
  (bind _returnvalue (AI|GetBlackboard 0))
  ;[1 1 1] Niagara FireWave + CallBackHandler
  (CallFunction|ResetDoOnceFireWave)
  (bind _output_get (Variables|Utilities|SetHit%20Player%20?_0 false))
  (Utilities|IsValid _returnvalue
    (:Is%20Valid
      (AI|Components|Blackboard|SetValueasBool _returnvalue (Utilities|Name|MakeLiteralName "PlayerHit") _output_get))
    (:Is%20Not%20Valid
      _))
  (bind _returnvalue_2 (Niagara|SpawnSystematLocation "/Game/Game_Dev/FX/NiagaraSystems/NS_FlreWave.NS_FlreWave" (Transformation|GetActorLocation)))
  (bind _output_get_2 (Variables|Default|SetFireWave_Niagara _returnvalue_2))
  (Class|NiagaraComponent|SetVariableObject _output_get_2 "CallBackHandler" self))

(event Custom|ResetDoOnceFireWave
  ;[1 1 1] Collision particules damage player
  (Utilities|FlowControl|DoOnce false) ; enters at Reset
)

(event Custom|StartAttack_5
  (if (not (Variables|Default|GetIsAttacking_5))
    (Variables|Default|SetCanRotateGeneral true)
    (Class|INTAnimBpIA|AttackGeneral5(Message) (Components|SkeletalMesh|GetAnimInstance (Variables|Character|GetMesh)))
    (Variables|Default|SetIsAttacking_5 true)
    (Variables|Utilities|SetHit%20Player%20?_0 false)))

(event Custom|Event%20Loop%20Start%20Attack%204
  ;[1 1 1] Loop Start Attack 4
  (Animation|Montage|PlayMontage (Variables|Character|GetMesh) "/Game/Game_ART/Graph/Chara/Boss/Boss_01_Skull/Animation/ANIM_Charge_StartLoop_Boss_Skull_Anim_Montage.ANIM_Charge_StartLoop_Boss_Skull_Anim_Montage"
    (:OnCompleted
      _)
    (:OnInterrupted
      _))
  (Variables|Default|SetCanRotateGeneral false)
  (Variables|Default|SetActor%20location (Transformation|GetActorLocation))
  (Variables|Default|SetActor%20Forward%20 (* (Transformation|GetActorForwardVector) 2e+03))
  (CallFunction|ResetHitWall))

(event Custom|ResetHitWall
  (bind _returnvalue (AI|GetBlackboard 0))
  (bind _returnvalue_2 (Transformation|GetActorForwardVector))
  (bind _returnvalue_3 (* _returnvalue_2 1e+03))
  ;[1 1 1] Hit Dash
  (bind _output_get (Variables|Default|SetIsHit?_0 false))
  (Utilities|IsValid _returnvalue
    (:Is%20Valid
      (AI|Components|Blackboard|SetValueasBool _returnvalue (Utilities|Name|MakeLiteralName "IsHit") _output_get)
      (Utilities|FlowControl|DoOnce false) ; enters at Reset
    )
    (:Is%20Not%20Valid
      (Utilities|FlowControl|DoOnce false) ; enters at Reset
    )))

(event Custom|StartAttack_4
  (if (not (Variables|Default|GetIsAttacking_4))
    (Variables|Default|SetCanRotateGeneral true)
    (Class|INTAnimBpIA|AttackGeneral4(Message) (Components|SkeletalMesh|GetAnimInstance (Variables|Character|GetMesh)))
    (Variables|Default|SetIsAttacking_4 true)
    (Variables|Utilities|SetHit%20Player%20?_0 false)))

(event Custom|BossToSpline
  (Variables|Default|SetInvincible true)
  (bind _returnvalue (Actor|GetActorOfClass "/Game/Game_Dev/Blueprints/IA/Generals/Blueprints/Spline_Boss_Skull.Spline_Boss_Skull_C"))
  (bind _newtrack_0 (Timeline|Timeline_3 PlayFromStart)
    (:Update
      (bind _returnvalue_2 (Transformation|SetActorLocation (Math|Vector|Lerp(Vector) (Transformation|GetActorLocation) (Transformation|GetActorLocation _returnvalue) _newtrack_0) true false))
      (if _returnvalue_2
        (bind _newtrack_0_2 (Timeline|Timeline_2 PlayFromStart)
          (:Update
            (Transformation|SetActorRotation (Math|Rotator|FindLookatRotation (Transformation|GetActorLocation) (Variables|Default|GetCentreMap)))
            (Transformation|SetActorLocation (Spline|GetLocationatDistanceAlongSpline (Variables|/Game/Game_Dev/Blueprints/IA/Generals/Blueprints/Spline_Boss_Skull.Spline_Boss_Skull_C|GetSpline _returnvalue) (* _newtrack_0_2 (Spline|GetSplineLength (Variables|/Game/Game_Dev/Blueprints/IA/Generals/Blueprints/Spline_Boss_Skull.Spline_Boss_Skull_C|GetSpline _returnvalue))) "World") false false))
          (:Finished
            (Transformation|SetActorLocation (Variables|Default|GetCentreMap) false false)))))))

(event Custom|Dash%20Attack
  ;[1 1 1] Attack Dash
  (bind _output_get (Variables|Default|SetActor%20location (Transformation|GetActorLocation)))
  (bind _outhit (Collision|LineTraceByChannel _output_get (+ _output_get (* (Transformation|GetActorForwardVector) 3e+02)) "TraceTypeQuery1" false 0 "None"))
  (bind _newtrack_0 (Timeline|Attack%20dash PlayFromStart)
    (:Update
      (Transformation|SetActorLocation (Math|Vector|Lerp(Vector) (Variables|Default|GetActor%20location) (Math|Vector|SelectVector (.impactpoint _outhit) (.traceend _outhit) (.bblockinghit _outhit)) _newtrack_0) true false))
    (:Finished
      (Variables|Default|SetIsAttacking1 false)
      (CallFunction|ReverseDash))
    (:Event%20FX
      (Animation|Montage|PlayMontage (Variables|Character|GetMesh) "/Game/Game_ART/Graph/Chara/Boss/Boss_01_Skull/Animation/ANIM_Attack_Hit_Boss_Skull_Anim_Montage.ANIM_Attack_Hit_Boss_Skull_Anim_Montage"))))

(event Custom|Finish%20attack%204
  ;[1 1 1] Finish attack 4
  (Variables|Default|SetIsAttacking_4 false)
  (if (not (Variables|Default|GetIsHit?_0))
    (Animation|Montage|PlayMontage (Variables|Character|GetMesh) "/Game/Game_ART/Graph/Chara/Boss/Boss_01_Skull/Animation/ANIM_Charge_End_WallHit_Boss_Skull_Anim_Montage.ANIM_Charge_End_WallHit_Boss_Skull_Anim_Montage")))

(event Custom|CanMoveG
  (params (canMove? :type Boolean) (canRotate? :type Boolean))
  (bind _charactermovement (Variables|Character|GetCharacterMovement))
  ;[1 1 1] Can Move General
  (Variables|Default|SetCanMoveGeneral canMove?)
  (Variables|Default|SetCanRotateGeneral canRotate?)
  (if canMove?
    (Pawn|Components|CharacterMovement|SetMovementMode _charactermovement "MOVE_Walking" 0)
    (elif canRotate?
      (Pawn|Components|CharacterMovement|SetMovementMode _charactermovement "MOVE_Custom" 0)
      (else
        (Pawn|Components|CharacterMovement|DisableMovement _charactermovement)))))

(event Custom|StartAttack_2
  (if (not (Variables|Default|GetIsAttacking_2))
    (Variables|Default|SetCanRotateGeneral true)
    (Class|INTAnimBpIA|AttackGeneral2(Message) (Components|SkeletalMesh|GetAnimInstance (Variables|Character|GetMesh)))
    (Variables|Default|SetIsAttacking_2 true)
    (Variables|Utilities|SetHit%20Player%20?_0 false)))

(event Custom|StartAttack_3
  (if (not (Variables|Default|GetIsAttacking_3))
    (Variables|Default|SetCanRotateGeneral true)
    (Class|INTAnimBpIA|AttackGeneral3(Message) (Components|SkeletalMesh|GetAnimInstance (Variables|Character|GetMesh)))
    (Variables|Default|SetIsAttacking_3 true)
    (Variables|Utilities|SetHit%20Player%20?_0 false)))

(event Custom|DASH%20LONGUEUR
  ;[1 1 1] Dash Longueur
  (Variables|Default|SetActor%20location (Transformation|GetActorLocation))
  (bind _time_lerp (Timeline|Dash%20Longueur%20Timeline PlayFromStart)
    (:Update
      (Transformation|SetActorLocation (Math|Vector|Lerp(Vector) (Variables|Default|GetActor%20location) (+ (Variables|Default|GetActor%20location) (Variables|Default|GetActor%20Forward%20)) _time_lerp) true false))
    (:Finished
      (CallFunction|FinishAttack4))
    (:Event%20FX
      (CallFunction|EventLoopStartAttack4))))

(event Custom|Player%20Take%20Damage
  ;[1 1 1] Player Taking Damage
  (if (Variables|Default|GetFireWave)
    (bind _output_get (Variables|Utilities|SetHit%20Player%20?_0 true))
    (AI|Components|Blackboard|SetValueasBool (Variables|/Script/AIModule.AIController|GetBlackboard (AI|GetAIController self)) (Utilities|Name|MakeLiteralName "PlayerHit") _output_get)
    (Game|Damage|ApplyDamage (CallFunction|CastPlayer) 35.0 0 0)))

(event Custom|Reverse%20Dash
  (bind _attackcountbasic (Variables|Default|GetAttackCountBasic))
  ;[1 1 1] Attack Dash
  ;;[1 1 1] Reverse
  (bind _output_get (Variables|Default|SetActor%20location (Transformation|GetActorLocation)))
  (bind _outhit (Collision|LineTraceByChannel _output_get (+ _output_get (* (Transformation|GetActorForwardVector) -2e+02)) "TraceTypeQuery1" false 0 "Persistent"))
  (bind _newtrack_0 (Timeline|Timeline_0 PlayFromStart)
    (:Update
      (Transformation|SetActorLocation (Math|Vector|Lerp(Vector) (Variables|Default|GetActor%20location) (Math|Vector|SelectVector (.impactpoint _outhit) (.traceend _outhit) (.bblockinghit _outhit)) _newtrack_0) true false))
    (:Finished
      (if (< _attackcountbasic 3)
        (Math|Integer|IncrementInt _attackcountbasic
          (:%20%20
            (Effects|SpawnEmitteratLocation 0 "0, 0, 0")))))))

(event EventBeginPlay
  (|CallParentFunction)
  (Default|ChangeBehaviorTree (.AsIA%20Controller%20Generals (Utilities|Casting|CastToIA_Controller_Generals (AI|GetAIController self))) (Variables|Default|GetIA_Type_Generals))
  (Variables|Default|SetCurrentHp (Variables|Default|GetMaxHp))
  (Variables|Default|SetIsIAGeneral true))

(event EventParticleData
  (params (Data :type Array%20of%20Basic%20Particle%20Data%20Structures) (NiagaraSystem :type Niagara%20System%20Object%20Reference))
  (bind _asbp_player_test (CallFunction|CastPlayer))
  ;[1 1 1] Collision particules damage player
  (for _array_element Data
    (if (and (<= (Math|Vector|Distance(Vector) (.Position (Utilities|Struct|BreakBasicParticleData _array_element)) (Transformation|GetActorLocation _asbp_player_test)) 1.5e+02) (not (Variables|/Game/Game_Dev/Blueprints/Player/BP_PlayerTest.BP_PlayerTest_C|GetIsJumping? _asbp_player_test)))
      (Utilities|FlowControl|DoOnce false
        (:Completed
          (CallFunction|PlayerTakeDamage))))))

(fn ConstructionScript)