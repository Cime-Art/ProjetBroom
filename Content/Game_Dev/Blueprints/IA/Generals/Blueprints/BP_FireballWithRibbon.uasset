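; Fireball projectile actor that pairs a Sphere component with a Niagara effect, named as having a ribbon.
; On BeginPlay the Sphere receives a forward impulse scaled by Power.
; Its first hit turns off physics and collision on the Niagara component (not the Sphere) and deactivates it.
; A Size timeline then drives the effect's Size parameter, and the actor destroys itself when the timeline finishes.
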(event OnComponentHit(Sphere)
  (params (HitComponent :type Primitive%20Component%20Object%20Reference) (OtherActor :type Actor%20Object%20Reference) (OtherComp :type Primitive%20Component%20Object%20Reference) (NormalImpulse :type Vector :default "0, 0, 0") (Hit :type Hit%20Result%20Structure%20%28by%20ref%29))
  (bind _niagara (Variables|Default|GetNiagara))
  (Utilities|FlowControl|DoOnce false
    (:Completed
      (Physics|SetSimulatePhysics _niagara false)
      (Collision|SetCollisionEnabled _niagara "NoCollision")
      (Components|Activation|Deactivate _niagara)
      (bind _size (Timeline|Size Play)
        (:Update
          (Effects|Components|ParticleSystem|SetFloatParameter (Variables|Default|GetNiagara) "Size" _size))
        (:Finished
          (Actor|DestroyActor))))))

(event EventBeginPlay
  (bind _sphere (Variables|Default|GetSphere))
  (Physics|AddImpulse _sphere (* (Math|Vector|GetForwardVector _sphere) (Variables|Default|GetPower)) "None" false))

(fn ConstructionScript)