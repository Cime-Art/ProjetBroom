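; AI boss character for the Generals, whose type selects speed, anim Blueprint and behavior tree, plus the Skull mesh for Tete De Feu.
; Three attack events message the anim instance, with timelines driving dash, recoil and fire wave distances.
; Niagara particle callbacks damage a nearby, non-jumping player during fire waves, gated by DoOnce.
; Fire wave, player hit and timed stun states feed the Blackboard, while CanMoveG switches movement modes.
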(event Custom|StartAttack_1
  (if (not (Variables|Default|GetIsAttacking1))
    (Class|INTAnimBpIA|AttackGeneral1(Message) (Components|SkeletalMesh|GetAnimInstance (Variables|Character|GetMesh)))
    (Variables|Default|SetIsAttacking1 true)
    (Variables|Utilities|SetHit%20Player%20?_0 false)))

(event Custom|Stunned
  (Variables|Default|SetStunned_General? true)
  (AI|Components|Blackboard|SetValueasBool (AI|GetBlackboard 0) (Utilities|Name|MakeLiteralName "Stunned_General") true)
  (CallFunction|CanMove false false)
  (Utilities|FlowControl|Delay 3.0)
  (if (not (Variables|Default|Getisdead))
    (Variables|Default|SetStunned_General? false)
    (CallFunction|CanMove true true)
    (AI|Components|Blackboard|SetValueasBool (AI|GetBlackboard 0) (Utilities|Name|MakeLiteralName "Stunned_General") false)))

(event Custom|Scale%20Fireball
  (params (Target :type Actor%20Object%20Reference))
  ;[1 1 1] Scale FireBalle
  (bind _scale (Timeline|Timeline_1 PlayFromStart)
    (:Update
      (Transformation|SetActorScale3D Target _scale))))

(event Custom|Collision%20FireWAVE
  (Development|PrintString "FIREWAE")
  (CallFunction|ResetDoOnceFireWave)
  (bind _returnvalue (Niagara|SpawnSystematLocation "/Game/Game_Dev/FX/NiagaraSystems/NS_FlreWave.NS_FlreWave" (Transformation|GetActorLocation)))
  (bind _output_get (Variables|Default|SetFireWave_Niagara _returnvalue))
  (Class|NiagaraComponent|SetVariableObject _output_get "CallBackHandler" self))

(event Custom|ResetDoOnceFireWave
  (Utilities|FlowControl|DoOnce false) ; enters at Reset
)

(event Custom|Raycast%20Distance%20To%20Player
  ;[1 1 1] Distance Player -> Boss
  (bind _outhit (Collision|LineTraceByChannel (Transformation|GetActorLocation) (Transformation|GetActorLocation (CallFunction|CastPlayer)) "TraceTypeQuery2" false 0 "ForOneFrame"))
  (Variables|Default|SetDistanceToPlayer (.distance _outhit)))

(event Custom|Timeline%20FireWave
  ;[1 1 1] Timeline Fire Wave
  (bind _output_get (Variables|Default|SetFireWave true))
  (AI|Components|Blackboard|SetValueasBool (AI|GetBlackboard 0) (Utilities|Name|MakeLiteralName "FireWave") _output_get)
  (Variables|Default|SetMaxDistance -1.0)
  (Variables|Default|SetMinDistance -1.0)
  (bind _mxdist (Timeline|MaxDist PlayFromStart)
    (:Update
      (Variables|Default|SetMaxDistance (* _mxdist 1.5e+03)))
    (:Event
      (bind _mndist (Timeline|MinDist PlayFromStart)
        (:Update
          (Variables|Default|SetMinDistance (* _mndist 1.45e+03)))
        (:Finished
          (Math|Integer|IncrementInt (Variables|Default|GetFireWaveCount)
            (:%20%20
              (if (== (Variables|Default|GetFireWaveCount) 3)
                (bind _output_get_2 (Variables|Default|SetFireWave false))
                (AI|Components|Blackboard|SetValueasBool (AI|GetBlackboard 0) (Utilities|Name|MakeLiteralName "FireWave") _output_get_2)))))))))

(event Custom|CanMoveG
  (params (canMove? :type Boolean) (canRotate? :type Boolean))
  (bind _charactermovement (Variables|Character|GetCharacterMovement))
  ;[1 1 1] Can Move General
  (Variables|Default|SetCanMoveGeneral canMove?)
  (Variables|Default|SetCanRotateGeneral canRotate?)
  (if canMove?
    (Pawn|Components|CharacterMovement|SetMovementMode _charactermovement "MOVE_Walking" 0)
    (elif canRotate?
      (Pawn|Components|CharacterMovement|SetMovementMode _charactermovement "MOVE_Custom" 0)
      (else
        (Pawn|Components|CharacterMovement|DisableMovement _charactermovement)))))

(event Custom|StartAttack_2
  (if (not (Variables|Default|GetIsAttacking_2))
    (CallFunction|CanMove false true)
    (Class|INTAnimBpIA|AttackGeneral2(Message) (Components|SkeletalMesh|GetAnimInstance (Variables|Character|GetMesh)))
    (Variables|Default|SetIsAttacking_2 true)
    (Variables|Utilities|SetHit%20Player%20?_0 false)))

(event Custom|StartAttack_3
  (if (not (Variables|Default|GetIsAttacking_3))
    (CallFunction|CanMove false true)
    (Class|INTAnimBpIA|AttackGeneral3(Message) (Components|SkeletalMesh|GetAnimInstance (Variables|Character|GetMesh)))
    (Variables|Default|SetIsAttacking_3 true)
    (Variables|Utilities|SetHit%20Player%20?_0 false)))

(event Custom|Dash%20Attack
  ;[1 1 1] Attack Dash PlaceHolder
  (bind _output_get (Variables|Default|SetActor%20location (Transformation|GetActorLocation)))
  (bind _outhit (Collision|LineTraceByChannel _output_get (+ _output_get (* (Transformation|GetActorForwardVector) 3e+02)) "TraceTypeQuery1" false 0 "None"))
  (bind _newtrack_0 (Timeline|Attack%20dash PlayFromStart)
    (:Update
      (Transformation|SetActorLocation (Math|Vector|Lerp(Vector) (Variables|Default|GetActor%20location) (Math|Vector|SelectVector (.impactpoint _outhit) (.traceend _outhit) (.bblockinghit _outhit)) _newtrack_0) true false))
    (:Finished
      (Variables|Default|SetIsAttacking1 false)
      (CallFunction|ReverseDash))
    (:Event%20FX
      (Animation|Montage|PlayMontage (Variables|Character|GetMesh) "/Game/Game_ART/Graph/Chara/Boss/Boss_01_Skull/Animation/ANIM_Attack_Hit_Boss_Skull_Anim_Montage.ANIM_Attack_Hit_Boss_Skull_Anim_Montage"))))

(event Custom|Player%20Take%20Damage
  ;[1 1 1] Player Taking Damage
  (if (Variables|Default|GetFireWave)
    (Utilities|FlowControl|DoOnce false :!label _label
      (:Completed
        (bind _output_get (Variables|Utilities|SetHit%20Player%20?_0 true))
        (AI|Components|Blackboard|SetValueasBool (Variables|/Script/AIModule.AIController|GetBlackboard (AI|GetAIController self)) (Utilities|Name|MakeLiteralName "PlayerHit") _output_get)
        (Game|Damage|ApplyDamage (CallFunction|CastPlayer) 35.0 0 0)))
    (else
      (bind _output_get_2 (Variables|Utilities|SetHit%20Player%20?_0 false))
      (AI|Components|Blackboard|SetValueasBool (Variables|/Script/AIModule.AIController|GetBlackboard (AI|GetAIController self)) (Utilities|Name|MakeLiteralName "PlayerHit") _output_get_2)
      (goto _label Reset))))

(event Custom|Reverse%20Dash
  (bind _attackcountbasic (Variables|Default|GetAttackCountBasic))
  ;[1 1 1] Attack Dash PlaceHolder
  ;;[1 1 1] Reverse
  (bind _output_get (Variables|Default|SetActor%20location (Transformation|GetActorLocation)))
  (bind _outhit (Collision|LineTraceByChannel _output_get (+ _output_get (* (Transformation|GetActorForwardVector) -2e+02)) "TraceTypeQuery1" false 0 "Persistent"))
  (bind _newtrack_0 (Timeline|Timeline_0 PlayFromStart)
    (:Update
      (Transformation|SetActorLocation (Math|Vector|Lerp(Vector) (Variables|Default|GetActor%20location) (Math|Vector|SelectVector (.impactpoint _outhit) (.traceend _outhit) (.bblockinghit _outhit)) _newtrack_0) true false))
    (:Finished
      (if (< _attackcountbasic 3)
        (Math|Integer|IncrementInt _attackcountbasic
          (:%20%20
            (Effects|SpawnEmitteratLocation 0 "0, 0, 0")
            (CallFunction|CanMove true true)))))))

(event EventTick
  (params (DeltaSeconds :type Float%20%28single-precision%29)))

(event EventBeginPlay
  (|CallParentFunction)
  (Default|ChangeBehaviorTree (.AsIA%20Controller%20Generals (Utilities|Casting|CastToIA_Controller_Generals (AI|GetAIController self))) (Variables|Default|GetIA_Type_Generals))
  (Variables|Default|SetCurrentHp (Variables|Default|GetMaxHp))
  (Variables|Default|SetIsIAGeneral true))

(event EventParticleData
  (params (Data :type Array%20of%20Basic%20Particle%20Data%20Structures) (NiagaraSystem :type Niagara%20System%20Object%20Reference))
  (bind _asbp_player_test (CallFunction|CastPlayer))
  (for _array_element Data
    (if (and (<= (Math|Vector|Distance(Vector) (.Position (Utilities|Struct|BreakBasicParticleData _array_element)) (Transformation|GetActorLocation _asbp_player_test)) 1.5e+02) (not (Variables|/Game/Game_Dev/Blueprints/Player/BP_PlayerTest.BP_PlayerTest_C|GetIsJumping? _asbp_player_test)))
      (Utilities|FlowControl|DoOnce false
        (:Completed
          (Development|PrintString "EH CA FAIT MAL")
          (CallFunction|PlayerTakeDamage))))))

(fn ConstructionScript
  (bind _mesh (Variables|Character|GetMesh))
  (switch Utilities|FlowControl|Switch|SwitchonIA_Types_Generals (Variables|Default|GetIA_Type_Generals)
    (:NewEnumerator0
      (Variables|Default|SetRadiusExplo 3e+02)
      (Variables|/Script/Engine.CharacterMovementComponent|SetMaxWalkSpeed (Variables|Character|GetCharacterMovement) 5e+02)
      (Class|SkeletalMeshComponent|SetAnimClass _mesh "/Game/Game_Dev/Blueprints/IA/Generals/AnimBP_Skull.AnimBP_Skull_C")
      (Class|SkinnedMeshComponent|SetSkeletalMesh _mesh "/Game/Game_ART/Graph/Chara/Boss/Boss_01_Skull/SM_Boss_Skull.SM_Boss_Skull" true))
    (:NewEnumerator1
      (Variables|Default|SetRadiusExplo 3e+02)
      (Variables|/Script/Engine.CharacterMovementComponent|SetMaxWalkSpeed (Variables|Character|GetCharacterMovement) 2e+02)
      (Class|SkeletalMeshComponent|SetAnimClass (Variables|Character|GetMesh) "/Game/Game_Dev/Blueprints/IA/Generals/AnimBP_FullBody.AnimBP_FullBody_C"))
    (:NewEnumerator2
      (Variables|Default|SetRadiusExplo 3e+02)
      (Variables|/Script/Engine.CharacterMovementComponent|SetMaxWalkSpeed (Variables|Character|GetCharacterMovement) 2e+02)
      (Class|SkeletalMeshComponent|SetAnimClass (Variables|Character|GetMesh) "/Game/Game_Dev/Blueprints/IA/Generals/AnimBP_Fusion.AnimBP_Fusion_C"))))