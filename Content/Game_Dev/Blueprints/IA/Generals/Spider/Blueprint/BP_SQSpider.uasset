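; BP_SQSpider is a trigger box that starts the SQ_Spider cutscene when BP_PlayerTest overlaps it.
; It disables player input, fades with WG_Fade, blends the view to the second CineCameraActor found, then reverses the fade and plays the sequence with movement and HUD off.
; Input is re-enabled right after playback starts, and delays time each step.
; The construction script caches the first BP_IA_Spider, unused in the event graph.
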(event OnComponentBeginOverlap(Box)
  (params (OverlappedComponent :type Primitive%20Component%20Object%20Reference) (OtherActor :type Actor%20Object%20Reference) (OtherComp :type Primitive%20Component%20Object%20Reference) (OtherBodyIndex :type Integer) (bFromSweep :type Boolean) (SweepResult :type Hit%20Result%20Structure%20%28by%20ref%29))
  (bind _asbp_player_test (Utilities|Casting|CastToBP_PlayerTest OtherActor))
  (Input|DisableInput _asbp_player_test (CallFunction|CastController))
  (bind _returnvalue (UserInterface|CreateWidget "/Game/Game_Dev/Blueprints/Widget/WG_Fade.WG_Fade_C"))
  (bind _output_get (Variables|Default|SetWG_Fade _returnvalue))
  (UserInterface|Viewport|AddtoViewport _returnvalue 0)
  (Utilities|FlowControl|Delay 0.5)
  (UserInterface|Animation|PlayAnimation _returnvalue (Variables|/Game/Game_Dev/Blueprints/Widget/WG_Fade.WG_Fade_C|GetFadeRenderOpacity _output_get) 0.0 1 "Forward" 1.0 false)
  (bind _outactors (Actor|GetAllActorsOfClass "/Script/CinematicCamera.CineCameraActor"))
  (Utilities|FlowControl|Delay 0.85)
  (Game|Player|SetViewTargetwithBlend (Game|GetPlayerController 0) (Utilities|Array|Get(acopy) _outactors 1) 0.2 "VTBlend_Linear" 0.0 false)
  (Utilities|FlowControl|Delay 1.0)
  (bind _returnvalue_2 (Sequencer|Player|CreateLevelSequencePlayer "/Game/Game_Dev/Sequence/SQ_Spider.SQ_Spider" (Utilities|Struct|MakeMovieSceneSequencePlaybackSettings false (Utilities|Struct|MakeMovieSceneSequenceLoopCount 0) 1.0 0.0 false false true false false true false false)))
  (Utilities|FlowControl|Delay 1.5)
  (UserInterface|Animation|PlayAnimation _returnvalue (Variables|/Game/Game_Dev/Blueprints/Widget/WG_Fade.WG_Fade_C|GetFadeRenderOpacity (Variables|Default|GetWG_Fade)) 0.0 1 "Reverse" 1.0 false)
  (Sequencer|Player|Play _returnvalue_2 :!class /Script/MovieScene.MovieSceneSequencePlayer)
  (Input|EnableInput _asbp_player_test (CallFunction|CastController)))

(fn ConstructionScript
  (bind _outactors (Actor|GetAllActorsOfClass "/Game/Game_Dev/Blueprints/IA/Generals/Spider/Blueprint/BP_IA_Spider.BP_IA_Spider_C"))
  (Variables|Default|SetSpiderRef (Utilities|Array|Get(acopy) _outactors)))