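; Spider web actor that alters the player's walk speed when BP_PlayerTest overlaps its sphere, then removes itself.
; Overlap calls Slow(false), which plays a timeline from the start; Slow(true) reverses it.
; Timeline updates lerp the player's MaxWalkSpeed between SlowSpeed and WalkSpeed, then a two-second delay leads to destroying the web.
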(event OnComponentBeginOverlap(Sphere)
  (params (OverlappedComponent :type Primitive%20Component%20Object%20Reference) (OtherActor :type Actor%20Object%20Reference) (OtherComp :type Primitive%20Component%20Object%20Reference) (OtherBodyIndex :type Integer) (bFromSweep :type Boolean) (SweepResult :type Hit%20Result%20Structure%20%28by%20ref%29))
  (Utilities|Casting|CastToBP_PlayerTest OtherActor)
  (CallFunction|Slow false))

(event Custom|Slow
  (params (Slow? :type Boolean))
  (if Slow?
    (bind _slowspeed (Timeline|Timeline_0 Reverse)
      (:Update
        (Variables|/Script/Engine.CharacterMovementComponent|SetMaxWalkSpeed (Variables|/Script/Engine.Character|GetCharacterMovement (CallFunction|CastPlayer)) (Math|Float|Lerp (Variables|Default|GetSlowSpeed) (Variables|Default|GetWalkSpeed) _slowspeed))
        (Utilities|FlowControl|Delay 2.0)
        (Actor|DestroyActor)))
    (else
      (Timeline|Timeline_0 PlayFromStart))))

(event EventDestroyed)

(fn ConstructionScript)