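; Spider boss character that runs BT_IA_Spider, with death opening the jail's end door and playing the ending cinematic.
; Tick feeds player-distance flags to the Blackboard and sets health-threshold flags.
; Events drive melee, radial attack, spawning, den and spawner-relocation behaviors through montages and AnimInstance messages.
; Spit lerps a projectile to the player's saved position, leaving a web on a miss; damage handling adds hit-count reactions and recursive poison ticks.
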(event Custom|Spawning
  ;[1 1 1] set Spawning
  (if (Math|Boolean|ANDBoolean (not (Variables|Default|GetIsAttacking?)) (not (Variables|Default|GetIsHit?)) (not (Variables|Default|GetDead?)) (not (Variables|Default|GetSecondAttack)) (not (Variables|Default|GetSpawning?)))
    (Class|INTAnimBpIA|SpawningSpider(Message) (Components|SkeletalMesh|GetAnimInstance (Variables|Character|GetMesh)))))

(event Custom|FirstAttack
  ;[1 1 1] Attack
  (if (and (not (Variables|Default|GetBigAttack)) (not (Variables|Default|GetSpawnTaniere)))
    (Class|INTAnimBpIA|AttackSpider(Message) (Components|SkeletalMesh|GetAnimInstance (Variables|Character|GetMesh)))
    (Variables|Default|SetApparition false)
    (Variables|Default|SetIsAttacking? true)))

(event Custom|Taniere
  (bind _returnvalue (Transformation|GetActorLocation))
  ;[1 1 1] taniere
  (Animation|Montage|PlayMontage (Variables|Character|GetMesh) "/Game/Game_Dev/Blueprints/IA/Generals/Spider/Animation/AnimMontage_SpiderFleeApparition.AnimMontage_SpiderFleeApparition"
    (:then
      (Variables|Default|SetSpawnTaniere true)
      (Utilities|FlowControl|Delay 1.0)
      (Transformation|SetActorLocation (Math|Vector|MakeVector (- (.x _returnvalue) 2.5e+02) (+ (.y _returnvalue) 2e+02) (.z _returnvalue)) false false)
      (Utilities|FlowControl|Delay 1.3)
      (CallFunction|Spawning))))

(event Custom|CanTakeDamage
  ;[1 1 1] Hit
  (Utilities|FlowControl|DoOnce false) ; enters at Reset
)

(event Custom|SpawnLocation
  ;[1 1 1] Spawner
  (if (and (Variables|Default|GetAlreadySpawn) (Variables|Default|GetSpawn))
    (bind _output_get (Variables|Default|SetAlreadySpawn false))
    (AI|Components|Blackboard|SetValueasBool (AI|GetBlackboard 0) (Utilities|Name|MakeLiteralName "AlreadySpawn") _output_get)
    (bind _output_get_2 (Variables|Default|SetSpawn false))
    (AI|Components|Blackboard|SetValueasBool (AI|GetBlackboard 0) (Utilities|Name|MakeLiteralName "Spawn") _output_get_2)
    (else
      (bind _outactors (Actor|GetAllActorsOfClass "/Game/Game_Dev/Blueprints/IA/Generals/Spider/Blueprint/Bp_SpawnSpider.Bp_SpawnSpider_C"))
      (bind _array_element (Utilities|Array|ForEachLoopwithBreak _outactors :!label _label)
        (:LoopBody
          (if (!= _array_element (Variables|OpenVariable|GetCurrentSpawner))
            (Variables|OpenVariable|SetCurrentSpawner _array_element)
            (goto _label Break)))
        (:Completed
          (Animation|Montage|PlayMontage (Variables|Character|GetMesh) "/Game/Game_Dev/Blueprints/IA/Generals/Spider/Animation/AnimMontage_SpiderFlee.AnimMontage_SpiderFlee"
            (:OnCompleted
              _)
            (:OnBlendOut
              _))
          (bind _output_get_3 (Variables|Default|SetSpawn true))
          (AI|Components|Blackboard|SetValueasBool (AI|GetBlackboard 0) (Utilities|Name|MakeLiteralName "Spawn") _output_get_3)
          (Utilities|FlowControl|Delay 0.1)
          (bind _returnvalue (Transformation|SetActorLocation (- (Transformation|GetActorLocation (Variables|OpenVariable|GetCurrentSpawner)) "100.000000, 0, 0") false false))
          (if _returnvalue
            (Animation|Montage|PlayMontage (Variables|Character|GetMesh) "/Game/Game_Dev/Blueprints/IA/Generals/Spider/Animation/AnimMontage_SpiderFleeApparition.AnimMontage_SpiderFleeApparition"
              (:OnCompleted
                _)
              (:OnBlendOut
                _))
            (bind _output_get_4 (Variables|Default|SetAlreadySpawn true))
            (AI|Components|Blackboard|SetValueasBool (AI|GetBlackboard 0) (Utilities|Name|MakeLiteralName "AlreadySpawn") _output_get_4)))))))

(event Custom|ApparitionSpider
  ;[1 1 1] Apparition
  (if (and (not (Variables|Default|GetIsAttacking?)) (not (Variables|Default|GetSecondAttack)))
    (Class|INTAnimBpIA|ApparitionSpider(Message) (Components|SkeletalMesh|GetAnimInstance (Variables|Character|GetMesh)))
    (bind _output_get (Variables|Default|SetApparition true))
    (AI|Components|Blackboard|SetValueasBool (AI|GetBlackboard 0) (Utilities|Name|MakeLiteralName "Apparition") _output_get)))

(event Custom|Spit
  (bind _asbp_player_test (CallFunction|CastPlayer))
  (bind _returnvalue (Transformation|GetActorLocation _asbp_player_test))
  ;[1 1 1] Spit
  (Variables|Default|SetSpiderSpit true)
  (if (or (not (Variables|Default|GetBigAttack)) (not (Variables|Default|GetSpawning?)))
    (Class|INTAnimBpIA|SpiderSpit(Message) (Components|SkeletalMesh|GetAnimInstance (Variables|Character|GetMesh)))
    (Variables|Default|SetPosPlayer (Math|Vector|MakeVector (.x _returnvalue) (.y _returnvalue) 0.0))
    (Utilities|FlowControl|Delay 1.4)
    (bind _returnvalue_2 (Game|SpawnActorfromClass "/Game/Game_Dev/Blueprints/IA/Generals/Spider/Blueprint/BP_SpiderSpit1.BP_SpiderSpit1_C" (Math|Transform|MakeTransform (Transformation|GetSocketLocation (Variables|Character|GetMesh) "l_mandible_skn") "0.000000,90.000000,0.000000" "0.100000,0.100000,0.100000") "AdjustIfPossibleButAlwaysSpawn" 0 0))
    (Variables|Default|SetBeginSpiderSplitPos (Transformation|GetActorLocation _returnvalue_2))
    (bind _movingz (Timeline|Timeline_1 PlayFromStart)
      (:Update
        (if (not (Variables|/Game/Game_Dev/Blueprints/IA/Generals/Spider/Blueprint/BP_SpiderSpit1.BP_SpiderSpit1_C|GetPlayerHit _returnvalue_2))
          (Transformation|SetActorLocationAndRotation _returnvalue_2 (Math|Vector|Lerp(Vector) (Variables|Default|GetBeginSpiderSplitPos) (Variables|Default|GetPosPlayer) _movingz) (Math|Rotator|MakeRotator (.roll (Transformation|GetActorRotation _returnvalue_2)) (.pitch (Transformation|GetActorRotation _returnvalue_2)) (- (.yaw (Math|Rotator|FindLookatRotation (Transformation|GetActorLocation _returnvalue_2) (Math|Vector|MakeVector (.x (Variables|Default|GetPosPlayer)) (.y (Variables|Default|GetPosPlayer)) 0.0))) 9e+01)) true)
          (Transformation|SetActorScale3D _returnvalue_2 "1.000000,1.000000,1.000000")))
      (:Finished
        (if (Variables|/Game/Game_Dev/Blueprints/IA/Generals/Spider/Blueprint/BP_SpiderSpit1.BP_SpiderSpit1_C|GetPlayerHit _returnvalue_2)
          _
          (else
            (bind _outhit (Collision|LineTraceByChannel (Variables|Default|GetPosPlayer) (+ (Variables|Default|GetPosPlayer) "0, 0,-500.000000") "TraceTypeQuery1" false 0 "ForDuration"))
            (Game|SpawnActorfromClass "/Game/Game_Dev/Blueprints/IA/Generals/Spider/Blueprint/Bp_SpiderWeb.Bp_SpiderWeb_C" (Math|Transform|MakeTransform (.location _outhit) "0, 0, 0" "2.000000,2.000000,2.000000") "AlwaysSpawn" 0 0)))
        (Variables|Default|SetFinishSpit true)
        (Variables|Default|SetSpiderSpit false)
        (Actor|DestroyActor _returnvalue_2)))))

(event Custom|SpiderBigAttack
  ;[1 1 1] BigAttack
  (if (Math|Boolean|ANDBoolean (not (Variables|Default|GetIsAttacking?)) (not (Variables|Default|GetDead?)) (not (Variables|Default|GetSecondAttack)))
    (Variables|Default|SetBigAttack true)
    (Class|INTAnimBpIA|BigAttackSpider(Message) (Components|SkeletalMesh|GetAnimInstance (Variables|Character|GetMesh)))
    (Utilities|FlowControl|Delay 1.5)
    (Components|Activation|SetActive (Variables|Default|GetNiagara) true false)
    (Game|Damage|ApplyRadialDamage 15.0 (+ (Transformation|GetActorLocation) "0.000000,50.000000, 0") 5e+01 0 0 0 0 false "ECC_Visibility")))

(event Custom|GetHit
  ;[1 1 1] Hit
  (if (not (Variables|Default|GetIsHit?))
    (Math|Integer|IncrementInt (Variables|Default|GetNumberOfHit)
      (:%20%20
        (if (>= (Variables|Default|GetNumberOfHit) (Math|Random|RandomIntegerinRange 5 9))
          (bind _output_get (Variables|Default|SetIsHit? true))
          (AI|Components|Blackboard|SetValueasBool (AI|GetBlackboard 0) (Utilities|Name|MakeLiteralName "IsHit") _output_get)
          (Class|INTAnimBpIA|HitSpider(Message) (Components|SkeletalMesh|GetAnimInstance (Variables|Character|GetMesh)))
          (Development|PrintString (Utilities|String|Append "SpawnTaniere" (Utilities|String|ToString(Boolean) (Variables|Default|GetSpawnTaniere))))
          (if (Variables|Default|GetSpawnTaniere)
            (if (>= (Variables|Default|GetNumberOfHit) 3)
              (Animation|Montage|PlayMontage (Variables|Character|GetMesh) "/Game/Game_Dev/Blueprints/IA/Generals/Spider/Animation/AnimMontage_SpiderFlee.AnimMontage_SpiderFlee"
                (:OnCompleted
                  _)
                (:OnBlendOut
                  _))
              (Variables|Default|SetNumberOfHit 0)
              (Variables|Default|SetSpawnTaniere false)
              (Rendering|SetVisibility (Variables|Character|GetMesh) false false))))))))

(event Custom|BeginSecondAttack
  ;[1 1 1] Attack
  (if (not (and (Variables|Default|GetIsAttacking?) (not (Variables|Default|GetSpawnTaniere))))
    (Variables|Default|SetSecondAttack true)
    (Animation|Montage|PlayMontage (Variables|Character|GetMesh) "/Game/Game_Dev/Blueprints/IA/Generals/Spider/Animation/AnimMontage_SpiderSecondAttack.AnimMontage_SpiderSecondAttack"
      (:OnCompleted
        _)
      (:OnInterrupted
        _))
    (Variables|Default|SetSecondAttack false)))

(event Custom|PoisonDamage
  (params (Degats :type Float%20%28single-precision%29) (Count :type Integer))
  ;[1 1 1] Poison
  (if (not (Variables|Default|GetDead?))
    (if (> Count 0)
      (bind _result (Math|Integer|DecrementInt Count)
        (:%20%20
          (Game|Damage|ApplyDamage self Degats 0 0)
          (if (<= (Variables|Default|GetCurrentHP) 0.0)
            (Class|Pawn|DetachfromControllerPendingDestroy)
            (Variables|Default|SetDead? true)
            (Class|INTAnimBpIA|Death(Message) (Components|SkeletalMesh|GetAnimInstance (Variables|Character|GetMesh)))
            (else
              (Utilities|FlowControl|Delay 1.0)
              (CallFunction|PoisonDamage Degats _result))))))))

(event Custom|BeginThirdAttack
  ;[1 1 1] Attack
  (if (Math|Boolean|ANDBoolean (not (Variables|Default|GetIsAttacking?)) (not (Variables|Default|GetSecondAttack)) (not (Variables|Default|GetSpawnTaniere)))
    (Variables|Default|SetThirdAttack true)
    (Animation|Montage|PlayMontage (Variables|Character|GetMesh) "/Game/Game_Dev/Blueprints/IA/Generals/Spider/Animation/AnimMontage_SpiderThirdAttack.AnimMontage_SpiderThirdAttack"
      (:OnCompleted
        _)
      (:OnBlendOut
        _))
    (Variables|Default|SetThirdAttack false)))

(event Custom|TakeDamage
  (params (Degats :type Float%20%28single-precision%29))
  ;[1 1 1] Hit
  (Development|PrintString "Hello")
  (Utilities|FlowControl|DoOnce false
    (:Completed
      (CallFunction|GetHit)
      (bind _output_get (Variables|Default|SetCurrentHP (- (Variables|Default|GetCurrentHP) Degats)))
      (if (<= _output_get 0.0)
        (bind _output_get_2 (Variables|Default|SetDead? true))
        (Class|INTAnimBpIA|DeathSpider(Message) (Components|SkeletalMesh|GetAnimInstance (Variables|Character|GetMesh)))
        (Development|PrintString (Utilities|String|ToString(Boolean) _output_get_2))
        (AI|Components|Blackboard|SetValueasBool (AI|GetBlackboard 0) (Utilities|Name|MakeLiteralName "Dead") _output_get_2)
        (bind _outactors (Actor|GetAllActorsOfClass "/Game/Game_Dev/Blueprints/GameplayScript/BP_BigDoorEndJail.BP_BigDoorEndJail_C"))
        (bind _output_get_3 (Variables|Default|SetBigDoorRef (Utilities|Array|Get(acopy) _outactors)))
        (Default|OpenDoor _output_get_3)
        (bind _returnvalue (Actor|GetActorOfClass "/Script/CinematicCamera.CineCameraActor"))
        (Game|Player|SetViewTargetwithBlend (Game|GetPlayerController 0) _returnvalue 1.0 "VTBlend_Linear" 0.0 false)
        (bind _returnvalue_2 (Sequencer|Player|CreateLevelSequencePlayer "/Game/Game_Dev/Sequence/SQ_EndSpiderBoss.SQ_EndSpiderBoss" (Utilities|Struct|MakeMovieSceneSequencePlaybackSettings false "(Value=0)" 1.0 0.0 false false false false false false false true)))
        (Sequencer|Player|Play _returnvalue_2 :!class /Script/MovieScene.MovieSceneSequencePlayer)
        (else
          (Utilities|FlowControl|Delay 0.7)
          (CallFunction|CanTakeDamage))))))

(event EventBeginPlay
  (bind _asia_controller_trashmob (Utilities|Casting|CastToIA_Controller_Trashmob (AI|GetAIController self)))
  (AI|RunBehaviorTree _asia_controller_trashmob "/Game/Game_Dev/Blueprints/IA/Generals/Spider/BT_BTTASK/BT_IA_Spider.BT_IA_Spider"))

(event Game|Damage|EventAnyDamage
  (params (Damage :type Float%20%28single-precision%29) (DamageType :type Damage%20Type%20Object%20Reference) (InstigatedBy :type Controller%20Object%20Reference) (DamageCauser :type Actor%20Object%20Reference))
  ;[1 1 1] Hit
  (if (Variables|Default|GetIsHit?)
    (CallFunction|TakeDamage Damage)))

(event EventTick
  (params (DeltaSeconds :type Float%20%28single-precision%29))
  (bind _asbp_player_test (CallFunction|CastPlayer))
  (bind _returnvalue (Transformation|GetActorLocation))
  (bind _returnvalue_2 (AI|GetBlackboard 0))
  (bind _asbp_player_test_2 (CallFunction|CastPlayer))
  (bind _returnvalue_3 (Transformation|GetActorLocation))
  (bind _maxhpspider (Variables|Default|GetMaxHPSpider))
  (bind _currenthp (Variables|Default|GetCurrentHP))
  (bind _maxhpspider_2 (Variables|Default|GetMaxHPSpider))
  (bind _currenthp_2 (Variables|Default|GetCurrentHP))
  (bind _maxhpspider_3 (Variables|Default|GetMaxHPSpider))
  (bind _currenthp_3 (Variables|Default|GetCurrentHP))
  (bind _returnvalue_4 (Transformation|GetActorLocation _asbp_player_test))
  (bind _returnvalue_5 (Transformation|GetActorLocation _asbp_player_test_2))
  (bind _returnvalue_6 (* _maxhpspider 0.25))
  (bind _returnvalue_7 (Math|Vector|Distance(Vector) (Math|Vector|MakeVector (.x _returnvalue_3) (.y _returnvalue_3) 0.0) (Math|Vector|MakeVector (.x _returnvalue_5) (.y _returnvalue_5) 0.0)))
  (bind _returnvalue_8 (Math|Vector|Distance(Vector) (Math|Vector|MakeVector (.x _returnvalue) (.y _returnvalue) 0.0) (Math|Vector|MakeVector (.x _returnvalue_4) (.y _returnvalue_4) 0.0)))
  (bind _returnvalue_9 (< _returnvalue_8 1.5e+03))
  ;[1 1 1] Set Near
  (Utilities|FlowControl|Sequence
    (:then_0
      (AI|Components|Blackboard|SetValueasBool (AI|GetBlackboard 0) (Utilities|Name|MakeLiteralName "Near") (< _returnvalue_8 5e+02))
      (AI|Components|Blackboard|SetValueasBool _returnvalue_2 (Utilities|Name|MakeLiteralName "CanSpiderSpit") (and (> _returnvalue_7 5e+02) (< _returnvalue_7 1.5e+03)))
      (if _returnvalue_9
        (Utilities|FlowControl|DoOnce false
          (:Completed
            (AI|Components|Blackboard|SetValueasBool (AI|GetBlackboard 0) (Utilities|Name|MakeLiteralName "CanSpawn") _returnvalue_9)))))
    (:then_1
      (if (and (<= _currenthp_2 (* _maxhpspider_2 0.75)) (>= _currenthp_2 (* _maxhpspider_2 0.7)))
        (Variables|Default|Set3QuartLife true)
        (else
          (Variables|Default|Set3QuartLife false)
          (if (and (<= _currenthp_3 (* _maxhpspider_3 0.5)) (>= _currenthp_3 (* _maxhpspider_3 0.45)))
            (Variables|Default|SetMidLife true)
            (else
              (Variables|Default|SetMidLife false)
              (if (and (<= _currenthp _returnvalue_6) (>= _currenthp (* _returnvalue_6 0.2)))
                (Variables|Default|SetQuartLife true)
                (else
                  (Variables|Default|SetQuartLife false))))))))
    (:then_2
      (bind _output_get (Variables|Default|SetVeryNear (< _returnvalue_8 285.0)))
      (AI|Components|Blackboard|SetValueasBool _returnvalue_2 (Utilities|Name|MakeLiteralName "VeryNear") _output_get))))

(fn ConstructionScript
  (Rendering|SetVisibility (Variables|Character|GetMesh) true false))