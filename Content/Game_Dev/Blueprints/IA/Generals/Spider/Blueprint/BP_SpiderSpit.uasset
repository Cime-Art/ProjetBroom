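; BP_SpiderSpit is the spider's spit actor, which turns into a web when it touches the player.
; The first Sphere overlap with BP_PlayerTest disables sphere and mesh collision and hides the skeletal mesh, guarded by a DoOnce.
; After a short delay it spawns a Bp_SpiderWeb at its own transform and calls Slow on it.
; The spit actor is only hidden, with no destroy call here.
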(event OnComponentBeginOverlap(Sphere)
  (params (OverlappedComponent :type Primitive%20Component%20Object%20Reference) (OtherActor :type Actor%20Object%20Reference) (OtherComp :type Primitive%20Component%20Object%20Reference) (OtherBodyIndex :type Integer) (bFromSweep :type Boolean) (SweepResult :type Hit%20Result%20Structure%20%28by%20ref%29))
  (bind _skeletalmesh (Variables|Default|GetSkeletalMesh))
  (Utilities|Casting|CastToBP_PlayerTest OtherActor)
  (Utilities|FlowControl|DoOnce false
    (:Completed
      (Collision|SetCollisionEnabled (Variables|Default|GetSphere) "NoCollision")
      (Rendering|SetVisibility _skeletalmesh false false)
      (Collision|SetCollisionEnabled _skeletalmesh "NoCollision")
      (Utilities|FlowControl|Delay 0.1)
      (bind _returnvalue (Game|SpawnActorfromClass "/Game/Game_Dev/Blueprints/IA/Generals/Spider/Blueprint/Bp_SpiderWeb.Bp_SpiderWeb_C" (Transformation|GetActorTransform) "AdjustIfPossibleButAlwaysSpawn" 0 0))
      (Default|Slow _returnvalue false))))

(event EventBeginPlay)

(fn ConstructionScript)