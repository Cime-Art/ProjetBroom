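; Spider enemy Blueprint, flagged as an AI general, that runs the BT_IA_Spider behavior tree on its trashmob AI controller and starts at max HP.
; JumpAttack, BigAttack and Apparition events send animation messages to the mesh's AnimInstance, each guarded by a boolean that this graph sets but never clears.
; An attached Niagara attack effect is present but disconnected, so it never plays.
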(event Custom|BigAttack
  (if (not (Variables|Default|GetIsBigAttacking?))
    (Class|INTAnimBpIA|BigAttack(Message) (Components|SkeletalMesh|GetAnimInstance (Variables|Character|GetMesh)))
    (Variables|Default|SetIsBigAttacking? true)))

(event Custom|JumpAttack
  (if (not (Variables|Default|GetIsAttacking?))
    (Class|INTAnimBpIA|AttackGeneral1(Message) (Components|SkeletalMesh|GetAnimInstance (Variables|Character|GetMesh)))
    (Variables|Default|SetIsAttacking? true)))

(event Custom|ApparitionSpider
  (if (not (Variables|Default|GetApparition))
    (Utilities|FlowControl|DoOnce false
      (:Completed
        (Class|INTAnimBpIA|Apparition(Message) (Components|SkeletalMesh|GetAnimInstance (Variables|Character|GetMesh)))
        (Variables|Default|SetApparition true)))))

(event EventBeginPlay
  (|CallParentFunction)
  (bind _asia_controller_trashmob (Utilities|Casting|CastToIA_Controller_Trashmob (AI|GetAIController self)))
  (AI|RunBehaviorTree _asia_controller_trashmob "/Game/Game_Dev/Blueprints/IA/Generals/Spider/Spider/BT_BTTASK/BT_IA_Spider.BT_IA_Spider")
  (Variables|Default|SetCurrentHp (Variables|Default|GetMaxHp))
  (Variables|Default|SetIsIAGeneral true))

(fn ConstructionScript
  (|CallParentFunction))