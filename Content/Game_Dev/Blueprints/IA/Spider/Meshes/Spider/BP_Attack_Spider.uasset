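; Anim notify state for the spider enemy's attack that damages the player during the animation's notify window.
; Each tick it sphere-traces on the Visibility channel between two body sockets on the mesh.
; It casts the first hit actor to the player, subtracts fixed HP through SetterHP, prints the health and returns.
; Nothing guards against repeat hits, so damage can recur every tick of the window.
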(fn ReceivedNotifyTick
  (params (MeshComp :type Skeletal%20Mesh%20Component%20Object%20Reference) (Animation :type Anim%20Sequence%20Base%20Object%20Reference) (FrameDeltaTime :type Float%20%28single-precision%29))
  (bind _outhits (Collision|MultiSphereTraceByChannel MeshComp (Transformation|GetSocketLocation MeshComp "BodySocket") (Transformation|GetSocketLocation MeshComp "BodySocket_0") 3e+01 "TraceTypeQuery1" false 0 "None"))
  (for _array_element _outhits
    (Default|SetterHP (CallFunction|CastPlayer (.HitActor (Collision|BreakHitResult _array_element))) (- (.HpPlayer (Utilities|Struct|BreakStruct_InfoPlayer (Variables|/Game/Game_Dev/Blueprints/Player/BP_PlayerTest.BP_PlayerTest_C|GetInfoPlayer (CallFunction|CastPlayer (.HitActor (Collision|BreakHitResult _array_element)))))) 15.0) false)
    (Development|PrintString 0 (Utilities|String|ToString(Float) (.HpPlayer (Utilities|Struct|BreakStruct_InfoPlayer (Variables|/Game/Game_Dev/Blueprints/Player/BP_PlayerTest.BP_PlayerTest_C|GetInfoPlayer (CallFunction|CastPlayer (.HitActor (Collision|BreakHitResult _array_element))))))))
    (return false)))