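; Spider enemy AI character Blueprint that plugs into the shared trash mob AI controller.
; On BeginPlay it casts its AI controller to IA_Controller_Trashmob and switches it to the spider behavior tree.
; Its JumpAttack event, skipped while the spider is hit, sets the attacking flag and spawns an attached Niagara attack effect offset from the mesh.
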(event Custom|JumpAttack
  (bind _mesh (Variables|Character|GetMesh))
  (bind _relativelocation (Variables|/Script/Engine.SceneComponent|GetRelativeLocation _mesh))
  (if (not (Variables|Default|GetIsHit?))
    (Variables|Default|SetIsAttacking? true)
    (Niagara|SpawnSystemAttached "/Game/Game_Dev/FX/NiagaraSystems/NS_Spider_Attack.NS_Spider_Attack" _mesh "None" (Math|Vector|MakeVector (+ (.x _relativelocation) 4e+01) (.y _relativelocation) (+ (.z _relativelocation) 1e+02)) "0, 0, 0" "KeepRelativeOffset" false)))

(event EventBeginPlay
  (|CallParentFunction)
  (bind _asia_controller_trashmob (Utilities|Casting|CastToIA_Controller_Trashmob (AI|GetAIController self)))
  (Default|ChangeBehaviorTree _asia_controller_trashmob "/Game/Game_Dev/Blueprints/IA/Trashmob/BehaviorTree_Blackboard/BT_IA_Spider.BT_IA_Spider"))

(fn ConstructionScript
  (|CallParentFunction))