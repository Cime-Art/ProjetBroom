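; Breakable prop actor that stands in for barrels, benches, bowls, buckets, stools, mugs and torture tools.
; The construction script uses an enum to pick both the destructible mesh and its matching Wwise break sound.
; DestroyMesh fires once, applying damage and an impulse along the given impact direction, posting the sound, then destroying the actor after a delay.
; An older per-type sound switch remains in the event graph but never runs.
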(event Custom|DestroyMesh
  (params (ImpactDirection :type Vector))
  (Utilities|FlowControl|DoOnce false
    (:Completed
      (Class|DestructibleComponent|ApplyDamage (Variables|Default|GetDestructible) 1e+02 (Transformation|GetWorldLocation (Variables|Default|GetDestructible)) ImpactDirection 2e+03)
      (Class|AkGameplayStatics|PostEvent (Variables|Default|GetAkEvent) self 0 0 0 true)
      (Utilities|FlowControl|Delay 8.0)
      (Actor|DestroyActor))))

(fn ConstructionScript
  (bind _enumdestructiblemesh (Variables|Default|GetEnumDestructibleMesh))
  (Class|DestructibleComponent|SetDestructibleMesh (Variables|Default|GetDestructible) (Utilities|Select :Index _enumdestructiblemesh :NewEnumerator0 "/Game/Game_Dev/DestructibleMesh/SM_Barrel_01_DM.SM_Barrel_01_DM" :NewEnumerator2 "/Game/Game_Dev/DestructibleMesh/SM_Barrel_02_DM.SM_Barrel_02_DM" :NewEnumerator8 "/Game/Game_Dev/DestructibleMesh/SM_Bench_01_DM.SM_Bench_01_DM" :NewEnumerator13 "/Game/Game_Dev/DestructibleMesh/SM_Bench_02_DM.SM_Bench_02_DM" :NewEnumerator15 "/Game/Game_Dev/DestructibleMesh/SM_Bench_03_DM.SM_Bench_03_DM" :NewEnumerator18 "/Game/Game_Dev/DestructibleMesh/SM_Bench_04_DM.SM_Bench_04_DM" :NewEnumerator21 "/Game/Game_Dev/DestructibleMesh/SM_Bench_06_DM.SM_Bench_06_DM" :NewEnumerator24 "/Game/Game_Dev/DestructibleMesh/SM_Bowl_01_DM.SM_Bowl_01_DM" :NewEnumerator27 "/Game/Game_Dev/DestructibleMesh/SM_Bowl_02_DM.SM_Bowl_02_DM" :NewEnumerator28 "/Game/Game_Dev/DestructibleMesh/SM_Bowl_03_DM.SM_Bowl_03_DM" :NewEnumerator29 "/Game/Game_Dev/DestructibleMesh/SM_Bowl_DM.SM_Bowl_DM" :NewEnumerator30 "/Game/Game_Dev/DestructibleMesh/SM_BowlV2_DM.SM_BowlV2_DM" :NewEnumerator31 "/Game/Game_Dev/DestructibleMesh/SM_BowlV3_DM.SM_BowlV3_DM" :NewEnumerator32 "/Game/Game_Dev/DestructibleMesh/SM_Bucket01_DM.SM_Bucket01_DM" :NewEnumerator33 "/Game/Game_Dev/DestructibleMesh/SM_Bucket02_DM.SM_Bucket02_DM" :NewEnumerator34 "/Game/Game_Dev/DestructibleMesh/SM_jail_Stool_01_DM.SM_jail_Stool_01_DM" :NewEnumerator35 "/Game/Game_Dev/DestructibleMesh/SM_jail_Stool_02_DM.SM_jail_Stool_02_DM" :NewEnumerator36 "/Game/Game_Dev/DestructibleMesh/SM_jail_Stool_03_DM.SM_jail_Stool_03_DM" :NewEnumerator37 "/Game/Game_Dev/DestructibleMesh/SM_Mug_01_DM.SM_Mug_01_DM" :NewEnumerator38 "/Game/Game_Dev/DestructibleMesh/SM_Mug_02_DM.SM_Mug_02_DM" :NewEnumerator39 "/Game/Game_Dev/DestructibleMesh/SM_Mug_03_DM.SM_Mug_03_DM" :NewEnumerator40 "/Game/Game_Dev/DestructibleMesh/SM_TortureTool_A_DM.SM_TortureTool_A_DM" :NewEnumerator41 "/Game/Game_Dev/DestructibleMesh/SM_TortureTool_B_DM.SM_TortureTool_B_DM" :NewEnumerator42 "/Game/Game_Dev/DestructibleMesh/SM_TortureTool_C_DM.SM_TortureTool_C_DM"))
  (Variables|Default|SetAkEvent (Utilities|Select :Index _enumdestructiblemesh :NewEnumerator0 "/Game/WwiseAudio/Events/Default_Work_Unit/Props/Play_BreakBucket.Play_BreakBucket" :NewEnumerator2 "/Game/WwiseAudio/Events/Default_Work_Unit/Props/Play_BreakBucket.Play_BreakBucket" :NewEnumerator8 "/Game/WwiseAudio/Events/Default_Work_Unit/Props/Play_BreakBench.Play_BreakBench" :NewEnumerator13 "/Game/WwiseAudio/Events/Default_Work_Unit/Props/Play_BreakBench.Play_BreakBench" :NewEnumerator15 "/Game/WwiseAudio/Events/Default_Work_Unit/Props/Play_BreakBench.Play_BreakBench" :NewEnumerator18 "/Game/WwiseAudio/Events/Default_Work_Unit/Props/Play_BreakBench.Play_BreakBench" :NewEnumerator21 "/Game/WwiseAudio/Events/Default_Work_Unit/Props/Play_BreakBench.Play_BreakBench" :NewEnumerator24 "/Game/WwiseAudio/Events/Default_Work_Unit/Props/Event_BreakMugBowl.Event_BreakMugBowl" :NewEnumerator27 "/Game/WwiseAudio/Events/Default_Work_Unit/Props/Event_BreakMugBowl.Event_BreakMugBowl" :NewEnumerator28 "/Game/WwiseAudio/Events/Default_Work_Unit/Props/Event_BreakMugBowl.Event_BreakMugBowl" :NewEnumerator29 "/Game/WwiseAudio/Events/Default_Work_Unit/Props/Event_BreakMugBowl.Event_BreakMugBowl" :NewEnumerator30 "/Game/WwiseAudio/Events/Default_Work_Unit/Props/Event_BreakMugBowl.Event_BreakMugBowl" :NewEnumerator31 "/Game/WwiseAudio/Events/Default_Work_Unit/Props/Event_BreakMugBowl.Event_BreakMugBowl" :NewEnumerator32 "/Game/WwiseAudio/Events/Default_Work_Unit/Props/Play_BreakBucket.Play_BreakBucket" :NewEnumerator33 "/Game/WwiseAudio/Events/Default_Work_Unit/Props/Play_BreakBucket.Play_BreakBucket" :NewEnumerator34 "/Game/WwiseAudio/Events/Default_Work_Unit/Props/Play_BreakBench.Play_BreakBench" :NewEnumerator35 "/Game/WwiseAudio/Events/Default_Work_Unit/Props/Play_BreakBench.Play_BreakBench" :NewEnumerator36 "/Game/WwiseAudio/Events/Default_Work_Unit/Props/Play_BreakBench.Play_BreakBench" :NewEnumerator37 "/Game/WwiseAudio/Events/Default_Work_Unit/Props/Event_BreakMugBowl.Event_BreakMugBowl" :NewEnumerator38 "/Game/WwiseAudio/Events/Default_Work_Unit/Props/Event_BreakMugBowl.Event_BreakMugBowl" :NewEnumerator39 "/Game/WwiseAudio/Events/Default_Work_Unit/Props/Event_BreakMugBowl.Event_BreakMugBowl" :NewEnumerator40 "/Game/WwiseAudio/Events/Default_Work_Unit/Level/Tuto/Kitchen/Event_PigChain_GetHit.Event_PigChain_GetHit" :NewEnumerator41 "/Game/WwiseAudio/Events/Default_Work_Unit/Level/Tuto/Kitchen/Event_PigChain_GetHit.Event_PigChain_GetHit" :NewEnumerator42 "/Game/WwiseAudio/Events/Default_Work_Unit/Level/Tuto/Kitchen/Event_PigChain_GetHit.Event_PigChain_GetHit")))